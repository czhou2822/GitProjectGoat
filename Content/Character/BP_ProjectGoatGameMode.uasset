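; Game mode that manages game phases and an air strike system, plus a 5x fast-forward while the player holds T in one phase.
; Targets queue up to the available strike count, then fire from registered towers paired by index.
; Strike state lives in the Bulkhead game and player states, with a counter-based recharge function.
; Initialization and the recharge timer setup are unwired, and phase changes are broadcast through CallOnPhaseChangeBP.
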(event EventBeginPlay)

(event EventTick
  (params (DeltaSeconds :type Float%20%28single-precision%29))
  (bind _gamephase (Variables|Default|GetGamePhase))
  (bind _asbp_player_character (Utilities|Casting|CastToBP_PlayerCharacter (Game|GetPlayerCharacter 0)))
  (if (Variables|/Game/Character/PlayerCharacter/BP_PlayerCharacter.BP_PlayerCharacter_C|GetIsTdown _asbp_player_character)
    (if (Utilities|Enum|Equal(Enum) _gamephase "NewEnumerator0")
      (Utilities|Time|SetGlobalTimeDilation 5.0)
      (else
        (Utilities|Time|SetGlobalTimeDilation 1.0 :!label _label)))
    (elif (Utilities|Enum|Equal(Enum) _gamephase "NewEnumerator0")
      (goto _label))))

(fn ConstructionScript)

(fn AddtoStrikeList
  (params (NewTarget :type BP%20Enemy%20Base%20Object%20Reference))
  (if (<= (+ (Utilities|Set|Length (Variables|/Game/Character/BP_BulkheadGameStates.BP_BulkheadGameStates_C|GetAirStrikeTargetsList (Variables|Default|GetBulkheadGameState_0))) 1) (Variables|/Game/Character/BP_BulkheadPlayerState.BP_BulkheadPlayerState_C|GetAirStrikeCount (Variables|Default|GetBulkheadPlayerState_0)))
    (Utilities|Set|Add (Variables|/Game/Character/BP_BulkheadGameStates.BP_BulkheadGameStates_C|GetAirStrikeTargetsList (Variables|Default|GetBulkheadGameState_0)) NewTarget)))

(fn RemovefromStrikeList
  (params (NewTarget :type BP%20Enemy%20Base%20Object%20Reference))
  (bind _returnvalue (Utilities|Set|Remove (Variables|/Game/Character/BP_BulkheadGameStates.BP_BulkheadGameStates_C|GetAirStrikeTargetsList (Variables|Default|GetBulkheadGameState_0)) NewTarget))
  (return _returnvalue))

(fn AirStrike
  (bind _bulkheadgamestate_0 (Variables|Default|GetBulkheadGameState_0))
  (bind _airstriketargetslist (Variables|/Game/Character/BP_BulkheadGameStates.BP_BulkheadGameStates_C|GetAirStrikeTargetsList _bulkheadgamestate_0))
  (bind _returnvalue (Utilities|Set|Length _airstriketargetslist))
  (Development|PrintString (Utilities|String|Append "strike target length: " (Utilities|String|ToString(Integer) _returnvalue) " strike tower length: " (Utilities|String|ToString(Integer) (Utilities|Set|Length (Variables|/Game/Character/BP_BulkheadGameStates.BP_BulkheadGameStates_C|GetAirStrikeTowerList (Variables|Default|GetBulkheadGameState_0))))))
  (if (>= _returnvalue 1)
    (bind _result (Utilities|Set|ToArray _airstriketargetslist))
    (for (_array_element _array_index) _result
      (Development|PrintString (Utilities|String|Append "Current index: " (Utilities|String|ToString(Integer) _array_index)))
      (bind _result_2 (Utilities|Set|ToArray (Variables|/Game/Character/BP_BulkheadGameStates.BP_BulkheadGameStates_C|GetAirStrikeTowerList (Variables|Default|GetBulkheadGameState_0))))
      (Default|ResetMark _array_element)
      (Utilities|IsValid (Utilities|Array|Get(acopy) _result_2 _array_index)
        (:Is%20Valid
          (Utilities|IsValid _array_element
            (:Is%20Valid
              (Default|AirStrike (Utilities|Array|Get(acopy) _result_2 _array_index) _array_element)
              (Math|Integer|DecrementInt (Variables|/Game/Character/BP_BulkheadPlayerState.BP_BulkheadPlayerState_C|GetAirStrikeCount (Variables|Default|GetBulkheadPlayerState_0))))))
        (:Is%20Not%20Valid
          (Development|PrintString (Utilities|String|Append "tower index: " (Utilities|String|ToString(Integer) _array_index) " not valid")))))
    (Utilities|Set|Clear (Variables|/Game/Character/BP_BulkheadGameStates.BP_BulkheadGameStates_C|GetAirStrikeTargetsList (Variables|Default|GetBulkheadGameState_0)))
    (else
      (Development|PrintString "Air strike not firing"))))

(fn AddAirStrikeTower
  (params (NewAirStrikeTower :type BP%20Air%20Strike%20Tower%20Object%20Reference))
  (Utilities|Set|Add (Variables|/Game/Character/BP_BulkheadGameStates.BP_BulkheadGameStates_C|GetAirStrikeTowerList (Variables|Default|GetBulkheadGameState_0)) NewAirStrikeTower)
  (Math|Integer|IncrementInt (Variables|/Game/Character/BP_BulkheadPlayerState.BP_BulkheadPlayerState_C|GetMaxAirStrikeCount (Variables|Default|GetBulkheadPlayerState_0))))

(fn AirStrikeTimerTick
  (bind _bulkheadplayerstate_0 (Variables|Default|GetBulkheadPlayerState_0))
  (if (< (Variables|/Game/Character/BP_BulkheadPlayerState.BP_BulkheadPlayerState_C|GetAirStrikeCount _bulkheadplayerstate_0) (Variables|/Game/Character/BP_BulkheadPlayerState.BP_BulkheadPlayerState_C|GetMaxAirStrikeCount _bulkheadplayerstate_0))
    (bind _result (Math|Integer|IncrementInt (Variables|AirStrike|GetAirStrikeCounter))
      (:%20%20
        (if (>= _result (Variables|AirStrike|GetMaxAirStrikeCounter))
          (Default|RechargeAirStrike (Variables|Default|GetBulkheadPlayerState_0))
          (Variables|AirStrike|SetAirStrikeCounter 0)
          (return)
          (else
            (return)))))
    (else
      (return))))

(fn InitBP
  (bind _asbp_bulkhead_player_state (Utilities|Casting|CastToBP_BulkheadPlayerState (Variables|/Script/Engine.Controller|GetPlayerState (Game|GetPlayerController 0))))
  (Variables|Default|SetBulkheadPlayerState_0 _asbp_bulkhead_player_state)
  (bind _asbp_bulkhead_game_states (Utilities|Casting|CastToBP_BulkheadGameStates (Game|GetGameState)))
  (Variables|Default|SetBulkheadGameState_0 _asbp_bulkhead_game_states))

(fn SetGamePhaseBP
  (params (NewGamePhase :type ENUM_GamePhase%20Enum :default "NewEnumerator0"))
  (bind _output_get (Variables|Default|SetGamePhase NewGamePhase))
  (Development|PrintString (Utilities|String|Append "CurrentPhase: " (Utilities|String|EnumtoString _output_get)))
  (Default|CallOnPhaseChangeBP _output_get))