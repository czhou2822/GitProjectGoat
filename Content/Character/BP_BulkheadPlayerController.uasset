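; BP_BulkheadPlayerController is a player controller that shows a bulkhead radial selection menu while Left Shift is held.
; Pressing creates UMG_BulkhedRadialMenu if needed, adds it to the viewport and switches to Game and UI input focused on it.
; Releasing removes and clears the widget, then restores game-only input.
; GetJoystickDirection returns the chosen stick's axes as a 2D vector, inverting Y for the left stick only.
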(event Input|KeyboardEvents|LeftShift
  (params (Key :type Key%20Structure :default "None"))
  (:Pressed
    (Variables|Default|GetSelectionWheel
      (:then
        _)
      (:else
        (bind _returnvalue (Game|ConstructObjectfromClass "/Game/UI/UMG_BulkhedRadialMenu.UMG_BulkhedRadialMenu_C" self))
        (Variables|Default|SetSelectionWheel _returnvalue)))
    (UserInterface|Viewport|AddtoViewport (Variables|Default|GetSelectionWheel) 0)
    (Input|SetInputModeGameandUI (Game|GetPlayerController 0) (Variables|Default|GetSelectionWheel) "DoNotLock" true))
  (:Released
    (bind _selectionwheel (Variables|Default|GetSelectionWheel)
      (:then
        (Widget|RemovefromParent _selectionwheel)
        (Variables|Default|SetSelectionWheel 0)
        (Input|SetInputModeGameOnly (Game|GetPlayerController 0)))
      (:else))))

(fn ConstructionScript)

(fn GetJoystickDirection
  (params (Stick :type EJoystickTypes%20Enum :default "NewEnumerator0"))
  (switch Utilities|FlowControl|Switch|SwitchonEJoystickTypes Stick
    (:NewEnumerator0
      (return (Math|Vector2D|MakeVector2D (Class|Actor|GetInputAxisKeyValue) (* (Class|Actor|GetInputAxisKeyValue) -1.0))))
    (:NewEnumerator1
      (return (Math|Vector2D|MakeVector2D (Class|Actor|GetInputAxisKeyValue) (Class|Actor|GetInputAxisKeyValue))))))