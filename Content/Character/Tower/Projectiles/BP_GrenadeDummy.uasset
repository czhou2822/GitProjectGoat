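; BP_GrenadeDummy is a tower projectile stand-in that delivers a delayed grenade strike from high above a target enemy.
; SetActorAndLocation stores the enemy and a snapshot of its position.
; After a short delay from BeginPlay, it spawns BP_GrenadeTest overhead at the enemy's current position, falling back to the snapshot if the enemy is invalid.
; It passes instigator and damage to the grenade, then destroys itself.
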(event EventBeginPlay
  (Utilities|FlowControl|Delay 2.0)
  (CallFunction|SpawnGrenade)
  (Actor|DestroyActor))

(event Collision|EventActorBeginOverlap
  (params (OtherActor :type Actor%20Object%20Reference)))

(event EventTick
  (params (DeltaSeconds :type Float%20%28single-precision%29)))

(fn ConstructionScript)

(fn SpawnGrenade
  (bind _targetenemy (Variables|Default|GetTargetEnemy)
    (:then
      (LocalVariables|SetSpawnLocation (+ (Transformation|GetActorLocation _targetenemy) "0, 0,5000.000000")))
    (:else
      (LocalVariables|SetSpawnLocation (+ (Variables|Default|GetTargetLocation) "0, 0,5000.000000"))))
  (bind _returnvalue (Game|SpawnActorfromClass "/Game/Character/Tower/Projectiles/BP_GrenadeTest.BP_GrenadeTest_C" (Math|Transform|MakeTransform (LocalVariables|GetSpawnLocation) "-90.000000,0.000000, 0" "1,1,1") "Undefined" 0 0))
  (Variables|/Script/Engine.Actor|SetInstigator _returnvalue (Game|GetInstigator))
  (Variables|/Game/Character/Tower/Projectiles/BP_ProjectileBase.BP_ProjectileBase_C|SetProjectileDamage _returnvalue (Variables|Default|GetProjectileDamage)))

(fn SetActorandLocation
  (params (InEnemy :type Enemy%20Base%20Object%20Reference))
  (bind _output_get (Variables|Default|SetTargetEnemy InEnemy))
  (Variables|Default|SetTargetLocation (Transformation|GetActorLocation _output_get)))