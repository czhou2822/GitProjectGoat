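; Tower grenade projectile that flies an arc toward an enemy and explodes with radial damage.
; A three-point spline with a raised midpoint is built from the target's position at that moment, and a timeline moves the mesh along it.
; It explodes at timeline end or shortly after an enemy enters the trigger sphere, drawing a debug sphere.
; Trigger range input is unwired, and stored delay values are unused here.
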(event OnComponentBeginOverlap(TriggerRadius)
  (params (OverlappedComponent :type Primitive%20Component%20Object%20Reference) (OtherActor :type Actor%20Object%20Reference) (OtherComp :type Primitive%20Component%20Object%20Reference) (OtherBodyIndex :type Integer) (bFromSweep :type Boolean) (SweepResult :type Hit%20Result%20Structure%20%28by%20ref%29))
  (Utilities|FlowControl|Delay 0.2)
  (Utilities|Casting|CastToBP_EnemyBase OtherActor)
  (CallFunction|Explode))

(event EventBeginPlay
  (|CallParentFunction)
  (bind _newtrack_0 (Timeline|Timeline_0 PlayFromStart)
    (:Update
      (Transformation|SetWorldLocation (Variables|Character|GetMesh) (Spline|GetLocationatDistanceAlongSpline (Variables|Default|GetSpline) (* (Spline|GetSplineLength (Variables|Default|GetSpline)) _newtrack_0) "World") false false))
    (:Finished
      (CallFunction|Explode))))

(event Collision|EventActorBeginOverlap
  (params (OtherActor :type Actor%20Object%20Reference))
  (|CallParentFunction OtherActor) ; This node is disabled and will not be called.\nDrag off pins to build functionality.
)

(event EventTick
  (params (DeltaSeconds :type Float%20%28single-precision%29))
  (|CallParentFunction DeltaSeconds))

(fn ConstructionScript
  (|CallParentFunction))

(fn Explode
  (Game|Damage|ApplyRadialDamage (Variables|Default|GetGrenadeDamage) (Transformation|GetWorldLocation (Variables|Character|GetMesh)) (Variables|Default|GetExplosiveRange) 0 0 0 0 false "ECC_Visibility")
  (Rendering|Debug|DrawDebugSphere (Transformation|GetWorldLocation (Variables|Character|GetMesh)) (Variables|Default|GetExplosiveRange) 12 "(R=1.000000,G=1.000000,B=1.000000,A=1.000000)" 2.0 3.0)
  (Actor|DestroyActor))

(fn SetDamageParameter
  (params (InDamage :type Float%20%28single-precision%29) (InTriggerRange :type Float%20%28single-precision%29) (InExplosiveRange :type Float%20%28single-precision%29) (InExplosionDelay :type Float%20%28single-precision%29) (InTriggerDelay :type Float%20%28single-precision%29))
  (Utilities|FlowControl|Sequence
    (:then_0
      (Variables|Default|SetGrenadeDamage InDamage))
    (:then_2
      (Variables|Default|SetExplosiveRange InExplosiveRange))
    (:then_3
      (Variables|Default|SetExplosionDelay InExplosionDelay))
    (:then_4
      (Variables|Default|SetTriggerDelay InTriggerDelay))))

(fn SetTargetSplineLinePoints
  (params (TargetEnemy :type BP%20Enemy%20Base%20Object%20Reference) (InZOffset :type Float%20%28single-precision%29))
  (LocalVariables|SetZOffset InZOffset)
  (LocalVariables|SetTargetLocation (Transformation|GetActorLocation TargetEnemy))
  (Spline|ClearSplinePoints (Variables|Default|GetSpline) true)
  (Spline|AddSplinePoint (Variables|Default|GetSpline) (Transformation|GetActorLocation) "World" true)
  (Spline|AddSplinePoint (Variables|Default|GetSpline) (Math|Vector|MakeVector (.x (/ (+ (Transformation|GetActorLocation) (LocalVariables|GetTargetLocation)) 2.0)) (.y (/ (+ (Transformation|GetActorLocation) (LocalVariables|GetTargetLocation)) 2.0)) (+ (.z (/ (+ (Transformation|GetActorLocation) (LocalVariables|GetTargetLocation)) 2.0)) (LocalVariables|GetZOffset))) "World" true)
  (Spline|AddSplinePoint (Variables|Default|GetSpline) (LocalVariables|GetTargetLocation) "World" true))