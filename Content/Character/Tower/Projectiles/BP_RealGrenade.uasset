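; Tower grenade projectile that explodes when its mesh hits something or an actor overlaps its trigger radius.
; Both events attach an explosion Niagara effect and call Explode, which applies radial damage attributed to the instigator and plays a sound.
; The construction script takes the damage range from the ExplosiveRadius sphere.
; The actor destroys itself when its own Niagara component finishes; debug range drawing is switched off.
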(event OnComponentHit(Mesh)
  (params (HitComponent :type Primitive%20Component%20Object%20Reference) (OtherActor :type Actor%20Object%20Reference) (OtherComp :type Primitive%20Component%20Object%20Reference) (NormalImpulse :type Vector :default "0, 0, 0") (Hit :type Hit%20Result%20Structure%20%28by%20ref%29))
  (Development|PrintString "Mesh Hit")
  (Development|PrintString (Utilities|GetObjectName (stale OnComponentBeginOverlap(TriggerRadius) OtherActor)) false false)
  (Niagara|SpawnSystemAttached "/Game/VFX/NS_Explosion.NS_Explosion" (Variables|Default|GetNiagara) "None" (Transformation|GetWorldLocation (Variables|Character|GetMesh)) "0, 0, 0" "KeepWorldPosition" false)
  (CallFunction|Explode))

(event OnComponentBeginOverlap(TriggerRadius)
  (params (OverlappedComponent :type Primitive%20Component%20Object%20Reference) (OtherActor :type Actor%20Object%20Reference) (OtherComp :type Primitive%20Component%20Object%20Reference) (OtherBodyIndex :type Integer) (bFromSweep :type Boolean) (SweepResult :type Hit%20Result%20Structure%20%28by%20ref%29))
  (Development|PrintString "TriggerHid")
  (Development|PrintString (Utilities|GetObjectName OtherActor) false false)
  (Niagara|SpawnSystemAttached "/Game/VFX/NS_Explosion.NS_Explosion" (Variables|Default|GetNiagara) "None" (Transformation|GetWorldLocation (Variables|Character|GetMesh)) "0, 0, 0" "KeepWorldPosition" false)
  (CallFunction|Explode))

(event OnSystemFinished(Niagara)
  (params (PSystem :type Niagara%20Component%20Object%20Reference))
  (Actor|DestroyActor))

(event EventBeginPlay
  (|CallParentFunction) ; This node is disabled and will not be called.\nDrag off pins to build functionality.
)

(event Collision|EventActorBeginOverlap
  (params (OtherActor :type Actor%20Object%20Reference))
  (|CallParentFunction OtherActor) ; This node is disabled and will not be called.\nDrag off pins to build functionality.
)

(event EventTick
  (params (DeltaSeconds :type Float%20%28single-precision%29))
  (|CallParentFunction DeltaSeconds) ; This node is disabled and will not be called.\nDrag off pins to build functionality.
)

(fn ConstructionScript
  (|CallParentFunction)
  (Variables|Default|SetExplosiveRange (Variables|/Script/Engine.SphereComponent|GetSphereRadius (Variables|Default|GetExplosiveRadius))))

(fn SetTarget
  (params (NewParam :type BP%20Enemy%20Base%20Object%20Reference))
  (Variables|Default|SetTarget NewParam))

(fn Explode
  (bind _returnvalue (Game|GetInstigator))
  (Development|PrintString (Utilities|String|Append "grenade test instigator: " (Utilities|GetDisplayName _returnvalue)))
  (Game|Damage|ApplyRadialDamage (Variables|Default|GetProjectileDamage) (Transformation|GetWorldLocation (Variables|Character|GetMesh)) (Variables|Default|GetExplosiveRange) 0 0 _returnvalue 0 false "ECC_Visibility")
  (Audio|SpawnSoundatLocation "/Game/Sound/Explosion_Cue.Explosion_Cue" (Transformation|GetActorLocation) "0, 0, 0" 1.0 1.0 0.0 "/Game/Character/MasterSoundAttenuation.MasterSoundAttenuation" 0)
  (CallFunction|DrawDebugRange false))

(fn DrawDebugRange
  (params (IsShown :type Boolean))
  (if IsShown
    (Rendering|Debug|DrawDebugSphere (Transformation|GetActorLocation) (Variables|Default|GetExplosiveRange) 12 "(R=1.000000,G=0.000000,B=0.045011,A=1.000000)" 0.5 3.0)
    (else
      (return))))