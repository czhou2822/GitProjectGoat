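; BP_HoloTower is the holographic placement preview for the player's selected Tesla, Gatling or Mortar tower.
; Construction picks the preview mesh, gear cost and data-driven range scale, then creates dynamic materials.
; Overlaps track tagged construction areas and nearby towers, while a player-state event updates gears only when gold rises.
; CheckCanBeBuilt requires an area, no overlapping towers and enough gears, tinting preview and range green or red.
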(event OnComponentBeginOverlap(SenseTower)
  (params (OverlappedComponent :type Primitive%20Component%20Object%20Reference) (OtherActor :type Actor%20Object%20Reference) (OtherComp :type Primitive%20Component%20Object%20Reference) (OtherBodyIndex :type Integer) (bFromSweep :type Boolean) (SweepResult :type Hit%20Result%20Structure%20%28by%20ref%29))
  (bind _overlappedtower (Variables|Default|GetOverlappedTower))
  ;[1 1 1] Sense tower begin overlap
  (if (== "/Script/Engine.CapsuleComponent" (Utilities|GetClass OtherComp))
    (bind _asbp_tower_base (Utilities|Casting|CastToBP_TowerBase OtherActor)
      (:then
        (Utilities|Casting|CastToBP_HoloTower _asbp_tower_base
          (:CastFailed
            (Utilities|Set|Add _overlappedtower _asbp_tower_base))))
      (:CastFailed
        (bind _asbp_mortar_tower (Utilities|Casting|CastToBP_MortarTower OtherActor))
        (Utilities|Set|Add _overlappedtower _asbp_mortar_tower)))
    (CallFunction|CheckCanbeBuilt)))

(event OnComponentEndOverlap(SenseTower)
  (params (OverlappedComponent :type Primitive%20Component%20Object%20Reference) (OtherActor :type Actor%20Object%20Reference) (OtherComp :type Primitive%20Component%20Object%20Reference) (OtherBodyIndex :type Integer))
  (bind _overlappedtower (Variables|Default|GetOverlappedTower))
  ;[1 1 1] Sense tower end overlap
  (if (== "/Script/Engine.CapsuleComponent" (Utilities|GetClass OtherComp))
    (bind _astower_base (Utilities|Casting|CastToTowerBase OtherActor)
      (:then
        (Utilities|Casting|CastToBP_HoloTower _astower_base
          (:CastFailed
            (Utilities|Set|Remove _overlappedtower _astower_base))))
      (:CastFailed
        (bind _asbp_mortar_tower (Utilities|Casting|CastToBP_MortarTower OtherActor))
        (Utilities|Set|Remove _overlappedtower _asbp_mortar_tower)))
    (CallFunction|CheckCanbeBuilt)))

(event OnComponentBeginOverlap(CapsuleComponent)
  (params (OverlappedComponent :type Primitive%20Component%20Object%20Reference) (OtherActor :type Actor%20Object%20Reference) (OtherComp :type Primitive%20Component%20Object%20Reference) (OtherBodyIndex :type Integer) (bFromSweep :type Boolean) (SweepResult :type Hit%20Result%20Structure%20%28by%20ref%29))
  ;[1 1 1] Capsule begin overlap
  (if (Actor|ActorHasTag OtherActor "ConstructionArea")
    (Variables|Default|SetIsInBuildingArea true)
    (Math|Integer|IncrementInt (Variables|Default|GetBuildingAreas)
      (:%20%20
        (CallFunction|CheckCanbeBuilt)))))

(event OnComponentEndOverlap(CapsuleComponent)
  (params (OverlappedComponent :type Primitive%20Component%20Object%20Reference) (OtherActor :type Actor%20Object%20Reference) (OtherComp :type Primitive%20Component%20Object%20Reference) (OtherBodyIndex :type Integer))
  ;[1 1 1] Capsule end overlap
  (if (Actor|ActorHasTag OtherActor "ConstructionArea") ; only matters if the other actor was a construction area
    (bind _result (Math|Integer|DecrementInt (Variables|Default|GetBuildingAreas))
      (:%20%20
        (if (< _result 0)
          (Development|PrintString "Error Tower Building Areas Went Negative" true true "(R=1.000000,G=0.000000,B=0.000000,A=1.000000)")
          (Variables|Default|SetBuildingAreas 0))
        (if (not (Math|Conversions|ToBoolean(Integer) (Variables|Default|GetBuildingAreas)))
          (Variables|Default|SetIsInBuildingArea false)
          (Development|PrintString "no contrcution area" false false "(R=0.485000,G=0.000000,B=0.013618,A=1.000000)")
          (CallFunction|CheckCanbeBuilt))))))

(event Custom|OnGoldChanged
  (params (CurrentGold :type Integer))
  (if (> CurrentGold (Variables|Default|GetCurrentGears))
    (Variables|Default|SetCurrentGears CurrentGold)
    (CallFunction|CheckCanbeBuilt)))

(event EventBeginPlay
  (bind _asbp_bulkhead_player_state (Utilities|Casting|CastToBP_BulkheadPlayerState (Utilities|Array|Get(acopy) (Variables|/Script/Engine.GameStateBase|GetPlayerArray (Game|GetGameState)))))
  (EventDispatchers|BindEventtoOnGoldChanged _asbp_bulkhead_player_state (delegate Custom|OnGoldChanged))
  (bind _returnvalue (Class|BulkheadPlayerState|GetGold _asbp_bulkhead_player_state))
  (Variables|Default|SetCurrentGears _returnvalue)
  (CallFunction|CheckCanbeBuilt))

(fn ConstructionScript
  (|CallParentFunction)
  (Utilities|FlowControl|Sequence
    (:then_0
      ;[1 1 1] Set gameplay vars
      (bind _asbp_bulkhead_player_state (Utilities|Casting|CastToBP_BulkheadPlayerState (Utilities|Array|Get(acopy) (Variables|/Script/Engine.GameStateBase|GetPlayerArray (Game|GetGameState)))))
      (bind _output_get (LocalVariables|SetSelectedTower (Variables|/Script/ProjectGoat.BulkheadPlayerState|GetSelectedTower _asbp_bulkhead_player_state)))
      (CallFunction|SetTowerPreview _output_get)
      (CallFunction|SetRangeScale _output_get)
      (switch Utilities|FlowControl|Switch|SwitchonETowerType _output_get
        (:TESLA
          (Variables|Default|SetReqiredGears 10))
        (:GATLING
          (Variables|Default|SetReqiredGears 5))
        (:MORTAR
          (Variables|Default|SetReqiredGears 30))))
    (:then_1
      ;[1 1 1] Create dynamic materials
      (bind _returnvalue (Rendering|Material|CreateDynamicMaterialInstance (Variables|Default|GetRangeMeshC) 0 0 "None" :!class /Script/Engine.PrimitiveComponent))
      (Variables|Default|SetRangeMaterial _returnvalue)
      (bind _returnvalue_2 (Rendering|Material|CreateDynamicMaterialInstance (Variables|Default|GetPreviewMesh) 0 0 "None" :!class /Script/Engine.PrimitiveComponent))
      (Variables|Default|SetTowerMaterial _returnvalue_2)
      ;[1 1 1] Mortar range material
      (if (Utilities|Enum|Equal(Enum) (LocalVariables|GetSelectedTower) "MORTAR")
        (Rendering|Material|SetScalarParameterValue (Variables|Default|GetRangeMaterial) "Height" 1.5e+03 :!class /Script/Engine.MaterialInstanceDynamic)))))

(fn SetTowerPreview
  (params (NewParam :type ETowerType%20Enum :default "TESLA"))
  (switch Utilities|FlowControl|Switch|SwitchonETowerType NewParam
    (:TESLA
      (Components|StaticMesh|SetStaticMesh (Variables|Default|GetPreviewMesh) (Variables|Default|GetTeslaPreviewMesh)))
    (:GATLING
      (Components|StaticMesh|SetStaticMesh (Variables|Default|GetPreviewMesh) (Variables|Default|GetGatlingPreviewMesh)))
    (:MORTAR
      (Components|StaticMesh|SetStaticMesh (Variables|Default|GetPreviewMesh) (Variables|Default|GetMortarPreviewMesh)))))

(fn SetRangeScale
  (params (NewParam :type ETowerType%20Enum :default "TESLA"))
  (switch Utilities|FlowControl|Switch|SwitchonETowerType NewParam
    (:TESLA
      (LocalVariables|SetTowerID 0))
    (:GATLING
      (LocalVariables|SetTowerID 2))
    (:MORTAR
      (LocalVariables|SetTowerID 1)))
  (bind _asbp_bulkhead_game_states (Utilities|Casting|CastToBP_BulkheadGameStates (Game|GetGameState)))
  (bind _returnvalue (Class|BulkheadGameState|GetTowerDatabyID _asbp_bulkhead_game_states (LocalVariables|GetTowerID)))
  (Transformation|SetWorldScale3D (Variables|Default|GetRangeMeshC) (Math|Vector|MakeVector (/ (.range _returnvalue) (Variables|Default|GetRangeRatio)) (/ (.range _returnvalue) (Variables|Default|GetRangeRatio)) (/ (.range _returnvalue) (Variables|Default|GetRangeRatio)))))

(fn CheckCanbeBuilt
  (CallFunction|UpdateMaterial (Math|Boolean|ANDBoolean (== (Utilities|Set|Length (Variables|Default|GetOverlappedTower)) 0) (Variables|Default|GetIsInBuildingArea) (>= (Variables|Default|GetCurrentGears) (Variables|Default|GetReqiredGears)))))

(fn UpdateMaterial
  (params (InCanBeBuild :type Boolean))
  (bind _rangematerial (Variables|Default|GetRangeMaterial))
  (bind _towermaterial (Variables|Default|GetTowerMaterial))
  (bind _output_get (Variables|Default|SetbCanBeBuilt InCanBeBuild))
  (if _output_get
    (Rendering|Material|SetVectorParameterValue _rangematerial "Color" "(R=0.009862,G=0.485000,B=0.125235,A=1.000000)" :!class /Script/Engine.MaterialInstanceDynamic)
    (Rendering|Material|SetVectorParameterValue _towermaterial "Color" "(R=0.009862,G=0.485000,B=0.125235,A=1.000000)" :!class /Script/Engine.MaterialInstanceDynamic)
    (else
      (Rendering|Material|SetVectorParameterValue _rangematerial "Color" "(R=0.485000,G=0.000000,B=0.013618,A=1.000000)" :!class /Script/Engine.MaterialInstanceDynamic)
      (Rendering|Material|SetVectorParameterValue _towermaterial "Color" "(R=0.485000,G=0.000000,B=0.013618,A=1.000000)" :!class /Script/Engine.MaterialInstanceDynamic))))