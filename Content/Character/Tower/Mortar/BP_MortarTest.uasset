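; Mortar tower character that lobs grenades at enemies, apparently a test variant.
; Placement starts construction in the anim instance; completion caches the AI controller and sizes the range sphere, whose overlaps maintain an enemy list.
; Each tick copies the AI's target; TurnTo is an empty stub.
; Firing plays a montage, while separate handlers spawn grenades on a suggested high-arc velocity using the tower's attack as damage.
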(event OnComponentBeginOverlap(RangeBP)
  (params (OverlappedComponent :type Primitive%20Component%20Object%20Reference) (OtherActor :type Actor%20Object%20Reference) (OtherComp :type Primitive%20Component%20Object%20Reference) (OtherBodyIndex :type Integer) (bFromSweep :type Boolean) (SweepResult :type Hit%20Result%20Structure%20%28by%20ref%29))
  ;[1 1 1] Enemy overlap
  (bind _asenemy_base (Utilities|Casting|CastToEnemyBase OtherActor))
  (Utilities|Set|Add (Variables|Default|GetEnemyList) _asenemy_base))

(event OnComponentEndOverlap(RangeBP)
  (params (OverlappedComponent :type Primitive%20Component%20Object%20Reference) (OtherActor :type Actor%20Object%20Reference) (OtherComp :type Primitive%20Component%20Object%20Reference) (OtherBodyIndex :type Integer))
  ;[1 1 1] Enemy overlap
  (bind _asenemy_base (Utilities|Casting|CastToEnemyBase OtherActor))
  (Utilities|Set|Remove (Variables|Default|GetEnemyList) _asenemy_base))

(event Custom|OnTowerDead
  (bind _self self)
  (bind _returnvalue (Transformation|GetActorLocation _self))
  ;[1 1 1] TowerDead
  (bind _swtowerdestruction (Variables|Default|GetSWTowerDestruction)
    (:then
      (Audio|PlaySoundatLocation _swtowerdestruction _returnvalue "0, 0, 0" 1.0 1.0 0.0 "/Game/Character/MasterSoundAttenuation.MasterSoundAttenuation" 0 0)
      (Niagara|SpawnSystematLocation "/Game/VFX/Niagara/Damage/NS_Damage_Burst.NS_Damage_Burst" _returnvalue))
    (:else)))

(event Custom|HandleABPOnConstructionComplete
  (bind _towerrange (Variables|Default|GetTowerRange))
  ;[1 1 1] Construction complete
  (Class|TowerBase|HandleonConstructionComplete)
  (bind _asai_tower_base (Utilities|Casting|CastToAI_TowerBase (Pawn|GetController)))
  (Variables|Default|SetTowerAI _asai_tower_base)
  (Development|PrintString (Utilities|String|Append "TowerRange: " (Utilities|String|ToString(Float) _towerrange)) false false)
  (Components|Sphere|SetSphereRadius (Variables|Default|GetRangeBP) _towerrange true)
  (Transformation|SetWorldScale3D (Variables|Default|GetRangeMeshC) (Math|Conversions|ToVector(Float) (/ 0.0 5e+01))))

(event Custom|HandleInternalTowerPlaced
  ;[1 1 1] Tower placed
  (Utilities|IsValid (Variables|Default|GetAnimBase)
    (:Is%20Valid
      (EventDispatchers|BindEventtoOnConstructionComplete (Variables|Default|GetAnimBase) (delegate Custom|HandleABPOnConstructionComplete))
      (Variables|/Script/ProjectGoat.AnimTowerBase|SetbIsPlaced (Variables|Default|GetAnimBase) true)
      (EventDispatchers|BindEventtoOnBulkheadCharacterDead (delegate Custom|OnTowerDead)))))

(event EventFireBullet
  (CallFunction|FireGrenade)
  (Class|TowerBase|PlayFireSound))

(event EventBeginPlay
  ;[1 1 1] Begin play
  (|CallParentFunction)
  (bind _asanim_tower_base (Utilities|Casting|CastToAnimTowerBase (Components|SkeletalMesh|GetAnimInstance (Variables|Character|GetMesh))))
  (Variables|Default|SetAnimBase _asanim_tower_base)
  (EventDispatchers|AssignInternalTowerPlaced (delegate Custom|HandleInternalTowerPlaced)))

(event EventTick
  (params (DeltaSeconds :type Float%20%28single-precision%29))
  (|CallParentFunction DeltaSeconds)
  (CallFunction|SetTargetActor)
  (Utilities|IsValid (Variables|Default|GetTargetEnemy)
    (:Is%20Valid
      (CallFunction|Turnto DeltaSeconds))))

(event EventTowerFire
  (Animation|Montage|PlayMontage (Variables|Character|GetMesh) "/Game/Character/Tower/Mortar/Animations/AM_Montar_Shooting.AM_Montar_Shooting" 1.0 0.0 "Default"))

(fn ConstructionScript
  (|CallParentFunction))

(fn FireGrenade
  (bind (_tossvelocity _returnvalue) (Class|GameplayStatics|BlueprintSuggestProjectileVelocity (Transformation|GetSocketLocation (Variables|Character|GetMesh) "FirePoint") (Transformation|GetActorLocation (Variables|Default|GetTargetEnemy)) (Variables|Default|GetFiringVelocity) 0.0 "DoNotTrace" 0.0 true false))
  (if _returnvalue
    (bind _returnvalue_2 (Game|SpawnActorfromClass "/Game/Character/Tower/Mortar/BP_RealGrenade.BP_RealGrenade_C" (Transformation|GetSocketTransform (Variables|Character|GetMesh) "FirePoint" "RTS_World") "Undefined" 0 _tossvelocity 0))
    (bind _returnvalue_3 (Class|BulkheadCharacterBase|GetCharacterData))
    (Variables|/Game/Character/Tower/Projectiles/BP_ProjectileBase.BP_ProjectileBase_C|SetProjectileDamage _returnvalue_2 (.attack _returnvalue_3))))

(fn Turnto
  (params (DeltaTime :type Float%20%28single-precision%29)))

(fn HandleTowerFireEvent
  (CallFunction|FireGrenade)
  (Class|TowerBase|PlayFireSound))

(fn SetTargetActor
  (bind _towerai (Variables|Default|GetTowerAI))
  (bind _targetactor (Variables|/Game/Character/Tower/TowerBase/AI_TowerBase.AI_TowerBase_C|GetTargetActor _towerai))
  (Utilities|IsValid _towerai
    (:Is%20Valid
      (Utilities|IsValid _targetactor
        (:Is%20Valid
          (bind _output_get (Variables|Default|SetTargetEnemy _targetactor))
          (Variables|Default|SetTargetLocation (Transformation|GetActorLocation _output_get)))
        (:Is%20Not%20Valid
          (Variables|Default|SetTargetEnemy 0))))))