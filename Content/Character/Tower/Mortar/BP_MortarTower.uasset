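; Mortar tower Blueprint that lobs grenades in a high arc at the target chosen by its AI controller.
; Placement clears instanced foliage beneath it; construction completion caches the AI and sizes the range sphere, whose overlaps maintain an enemy list.
; TowerFire plays the shooting montage, whose FireBullet event solves the toss velocity, aims the anim dome and spawns a randomly scattered shell carrying the tower's attack damage.
; Construction and death trigger sound, with a burst effect on death.
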(event OnComponentBeginOverlap(RangeBP)
  (params (OverlappedComponent :type Primitive%20Component%20Object%20Reference) (OtherActor :type Actor%20Object%20Reference) (OtherComp :type Primitive%20Component%20Object%20Reference) (OtherBodyIndex :type Integer) (bFromSweep :type Boolean) (SweepResult :type Hit%20Result%20Structure%20%28by%20ref%29))
  ;[1 1 1] Enemy overlap
  (bind _asenemy_base (Utilities|Casting|CastToEnemyBase OtherActor))
  (Utilities|Set|Add (Variables|Default|GetEnemyList) _asenemy_base))

(event OnComponentEndOverlap(RangeBP)
  (params (OverlappedComponent :type Primitive%20Component%20Object%20Reference) (OtherActor :type Actor%20Object%20Reference) (OtherComp :type Primitive%20Component%20Object%20Reference) (OtherBodyIndex :type Integer))
  ;[1 1 1] Enemy overlap
  (bind _asenemy_base (Utilities|Casting|CastToEnemyBase OtherActor))
  (Utilities|Set|Remove (Variables|Default|GetEnemyList) _asenemy_base))

(event Custom|OnTowerDead
  (bind _self self)
  (bind _returnvalue (Transformation|GetActorLocation _self))
  ;[1 1 1] TowerDead
  (bind _swtowerdestruction (Variables|Default|GetSWTowerDestruction)
    (:then
      (Audio|PlaySoundatLocation _swtowerdestruction _returnvalue "0, 0, 0" 1.0 1.0 0.0 "/Game/Audio/Attenuation/MasterSoundAttenuation.MasterSoundAttenuation" 0 0)
      (Niagara|SpawnSystematLocation "/Game/VFX/Niagara/Damage/NS_Damage_Burst.NS_Damage_Burst" _returnvalue))
    (:else)))

(event Custom|HandleABPOnConstructionComplete
  (bind _towerrange (Variables|Default|GetTowerRange))
  ;[1 1 1] Construction complete
  (Class|TowerBase|HandleonConstructionComplete)
  (bind _asai_tower_base (Utilities|Casting|CastToAI_TowerBase (Pawn|GetController)))
  (Variables|Default|SetTowerAI _asai_tower_base)
  (Development|PrintString (Utilities|String|Append "TowerRange: " (Utilities|String|ToString(Float) _towerrange)) false false)
  (Components|Sphere|SetSphereRadius (Variables|Default|GetRangeBP) _towerrange true)
  (Transformation|SetWorldScale3D (Variables|Default|GetRangeMeshC) (Math|Conversions|ToVector(Float) (/ 0.0 5e+01))))

(event Custom|HandleInternalTowerPlaced
  ;[1 1 1] Tower placed
  (CallFunction|DestroyPossibleFoliage)
  (Utilities|IsValid (Variables|Default|GetAnimBase)
    (:Is%20Valid
      (EventDispatchers|BindEventtoOnConstructionComplete (Variables|Default|GetAnimBase) (delegate Custom|HandleABPOnConstructionComplete))
      (Variables|/Script/ProjectGoat.AnimTowerBase|SetbIsPlaced (Variables|Default|GetAnimBase) true)
      (EventDispatchers|BindEventtoOnBulkheadCharacterDead (delegate Custom|OnTowerDead)))))

(event EventFireBullet
  ;[1 1 1] Animation trigger shell spawn event
  (CallFunction|FireGrenade)
  (Audio|Components|Audio|Play (Variables|Default|GetAudio) 0.0))

(event EventConstructionStarts
  ;[1 1 1] Construction Sound
  (Audio|PlaySoundatLocation "/Game/Audio/SFX/Towers/Construction/SFX_Mortar_Construction.SFX_Mortar_Construction" (Transformation|GetActorLocation self) "0, 0, 0" 1.0 1.0 0.0 "/Game/Audio/Attenuation/MasterSoundAttenuation.MasterSoundAttenuation" 0 0))

(event EventBeginPlay
  ;[1 1 1] Begin play
  (|CallParentFunction)
  (bind _asanim_tower_base (Utilities|Casting|CastToAnimTowerBase (Components|SkeletalMesh|GetAnimInstance (Variables|Character|GetMesh))))
  (Variables|Default|SetAnimBase _asanim_tower_base)
  (EventDispatchers|AssignInternalTowerPlaced (delegate Custom|HandleInternalTowerPlaced)))

(event EventTick
  (params (DeltaSeconds :type Float%20%28single-precision%29))
  ;[1 1 1] Tick
  (|CallParentFunction DeltaSeconds)
  (CallFunction|SetTargetActor)
  (Utilities|IsValid (Variables|Default|GetTargetEnemy)
    (:Is%20Valid
      (CallFunction|Turnto DeltaSeconds)
      (Class|TowerBase|TurnFirePointtotheEnemy))))

(event EventTowerFire
  ;[1 1 1] CPP Trigger fire event
  (Development|PrintString "Fire" false false)
  (Animation|Montage|PlayMontage (Variables|Character|GetMesh) "/Game/Character/Tower/Mortar/Animations/AM_Montar_Shooting.AM_Montar_Shooting" 1.0 0.0 "Default"))

(fn ConstructionScript
  (|CallParentFunction))

(fn FireGrenade
  (bind _toss_vector (Variables|Default|GetToss_Vector))
  (bind _animbase (Variables|Default|GetAnimBase))
  (bind _targetenemy (Variables|Default|GetTargetEnemy)
    (:then
      (bind (_tossvelocity _returnvalue) (Class|GameplayStatics|BlueprintSuggestProjectileVelocity (Transformation|GetSocketLocation (Variables|Character|GetMesh) "FirePoint") (Transformation|GetActorLocation _targetenemy) (Variables|Default|GetFiringVelocity) 0.0 "DoNotTrace" 45.0 true false))
      ;[1 1 1] Use Toss Vector to set Arrow World Rotation then use Relative Rotation as Doom Rotation
      (Transformation|SetWorldRotation _toss_vector (Math|Conversions|RotationFromXVector _tossvelocity) false false)
      (Variables|/Script/ProjectGoat.AnimTowerBase|SetDoomRotation _animbase (Variables|/Script/Engine.SceneComponent|GetRelativeRotation _toss_vector))
      (Variables|/Script/ProjectGoat.AnimTowerBase|SetBarrelRotation _animbase "0, 0, 0")
      (Development|PrintString (Utilities|String|Append "Yaw: " (Utilities|String|ToString(Float) (.Yaw (Math|Vector|GetYawPitchfromVector _tossvelocity))) " Pitch: " (Utilities|String|ToString(Float) (.Pitch (Math|Vector|GetYawPitchfromVector _tossvelocity))) " degree: " (Utilities|String|ToString(Float) (Class|KismetMathLibrary|DegAcos (Math|Vector|DotProduct (Math|Vector|Normalize _tossvelocity) "0.000000,0.000000,1.000000"))) " tossVelocity: " (Utilities|String|ToString(Vector) _tossvelocity)) false false)
      (if _returnvalue
        (bind _returnvalue_2 (Game|SpawnActorfromClass "/Game/Character/Tower/Mortar/BP_RealGrenade.BP_RealGrenade_C" (Math|Transform|MakeTransform (.location (Transformation|GetSocketTransform (Variables|Character|GetMesh) "FirePoint" "RTS_World")) (Math|Rotator|MakeRotator 0.0 (.Pitch (Math|Vector|GetYawPitchfromVector _tossvelocity)) (.Yaw (Math|Vector|GetYawPitchfromVector _tossvelocity))) "1,1,1") "Undefined" 0 (+ (* _tossvelocity 1.025) (* (Math|Random|RandomUnitVector) (Variables|Default|GetTrajectoryRandomization))) (Variables|Default|GetFiringVelocity) 0))
        (bind _returnvalue_3 (Class|BulkheadCharacterBase|GetCharacterData))
        (Variables|/Game/Character/Tower/Projectiles/BP_ProjectileBase.BP_ProjectileBase_C|SetProjectileDamage _returnvalue_2 (.attack _returnvalue_3))))
    (:else)))

(fn Turnto
  (params (DeltaTime :type Float%20%28single-precision%29)))

(fn SetTargetActor
  (bind _towerai (Variables|Default|GetTowerAI))
  (bind _targetactor (Variables|/Game/Character/Tower/TowerBase/AI_TowerBase.AI_TowerBase_C|GetTargetActor _towerai))
  (Utilities|IsValid _towerai
    (:Is%20Valid
      (Utilities|IsValid _targetactor
        (:Is%20Valid
          (bind _output_get (Variables|Default|SetTargetEnemy _targetactor))
          (Variables|Default|SetTargetLocation (Transformation|GetActorLocation _output_get)))
        (:Is%20Not%20Valid
          (Variables|Default|SetTargetEnemy 0))))))

(fn DestroyPossibleFoliage
  (bind _returnvalue (Transformation|GetActorLocation))
  (bind _outhits (Collision|MultiSphereTraceByChannel (Transformation|GetActorLocation) (Math|Vector|MakeVector (.x _returnvalue) (.y _returnvalue) (- (.z _returnvalue) 1e+02)) (Variables|/Script/Engine.CapsuleComponent|GetCapsuleRadius (Variables|Default|GetCapsuleComponent)) "TraceTypeQuery5" false 0 "None"))
  (for _array_element _outhits
    (Development|PrintString (Utilities|String|Append "component:  " (Utilities|GetDisplayName (.HitComponent (Collision|BreakHitResult _array_element))) " hit item: " (Utilities|String|ToString(Integer) (.HitItem (Collision|BreakHitResult _array_element)))) false false)
    (bind _asinstanced_static_mesh_component (Utilities|Casting|CastToInstancedStaticMeshComponent (.HitComponent (Collision|BreakHitResult _array_element))))
    (Class|InstancedStaticMeshComponent|RemoveInstance _asinstanced_static_mesh_component (.HitItem (Collision|BreakHitResult _array_element)))))