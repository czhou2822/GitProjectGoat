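; BP_RealGrenade is the mortar tower's grenade, which deals radial damage when something enters its trigger or two seconds after spawning.
; Trigger overlap, guarded by HasExplode, spawns Niagara explosion and camera shake before calling Explode; the timer calls Explode directly, without those effects or the guard.
; Explode sets the flag, damages within the ExplosiveRadius sphere's radius with the instigator as causer, and plays the sound.
; The actor is never destroyed here.
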(event OnComponentBeginOverlap(TriggerRadius)
  (params (OverlappedComponent :type Primitive%20Component%20Object%20Reference) (OtherActor :type Actor%20Object%20Reference) (OtherComp :type Primitive%20Component%20Object%20Reference) (OtherBodyIndex :type Integer) (bFromSweep :type Boolean) (SweepResult :type Hit%20Result%20Structure%20%28by%20ref%29))
  (Development|PrintString "TriggerHid" false)
  (if (not (Variables|Default|GetHasExplode))
    (Development|PrintString (Utilities|String|Append "other actor: " (Utilities|GetObjectName OtherActor) " other comp: " (Utilities|GetObjectName OtherComp) " overlapped component: " (Utilities|GetObjectName OverlappedComponent)) false)
    (Niagara|SpawnSystemAttached "/Game/VFX/Niagara/Mortar/NS_Explosion.NS_Explosion" (Variables|Default|GetExplosion) "None" (Transformation|GetWorldLocation (Variables|Character|GetMesh)) "0, 0, 0" "KeepWorldPosition" false)
    ;[1 1 1] Apply Camera Shake
    (Camera|PlayWorldCameraShake "/Game/VFX/Blueprints/BP_CameraShake_Explosion.BP_CameraShake_Explosion_C" (Transformation|GetWorldLocation (Variables|Character|GetMesh)) 0.0 1.5e+03)
    (CallFunction|Explode)))

(event EventBeginPlay
  (|CallParentFunction)
  (Utilities|FlowControl|Delay 2.0)
  (CallFunction|Explode))

(event Collision|EventActorBeginOverlap
  (params (OtherActor :type Actor%20Object%20Reference))
  (|CallParentFunction OtherActor) ; This node is disabled and will not be called.\nDrag off pins to build functionality.
)

(event EventTick
  (params (DeltaSeconds :type Float%20%28single-precision%29))
  (|CallParentFunction DeltaSeconds) ; This node is disabled and will not be called.\nDrag off pins to build functionality.
)

(fn ConstructionScript
  (|CallParentFunction)
  (Variables|Default|SetExplosiveRange (Variables|/Script/Engine.SphereComponent|GetSphereRadius (Variables|Default|GetExplosiveRadius))))

(fn SetTarget
  (params (NewParam :type BP%20Enemy%20Base%20Object%20Reference))
  (Variables|Default|SetTarget NewParam))

(fn Explode
  (bind _returnvalue (Game|GetInstigator))
  (Variables|Default|SetHasExplode true)
  (Development|PrintString (Utilities|String|Append "grenade test instigator: " (Utilities|GetDisplayName _returnvalue)) false)
  (Game|Damage|ApplyRadialDamage (Variables|Default|GetProjectileDamage) (Transformation|GetWorldLocation (Variables|Character|GetMesh)) (Variables|Default|GetExplosiveRange) 0 0 _returnvalue 0 false "ECC_Visibility")
  (Audio|SpawnSoundatLocation "/Game/Sound/Explosion_Cue.Explosion_Cue" (Transformation|GetActorLocation) "0, 0, 0" 1.0 1.0 0.0 "/Game/Character/MasterSoundAttenuation.MasterSoundAttenuation" 0)
  (CallFunction|DrawDebugRange false))

(fn DrawDebugRange
  (params (IsShown :type Boolean))
  (if IsShown
    (Rendering|Debug|DrawDebugSphere (Transformation|GetActorLocation) (Variables|Default|GetExplosiveRange) 12 "(R=1.000000,G=0.000000,B=0.045011,A=1.000000)" 0.5 3.0)
    (else
      (return))))