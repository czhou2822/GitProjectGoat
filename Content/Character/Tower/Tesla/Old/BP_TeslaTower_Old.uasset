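; Tesla tower that fires chain lightning, jumping between nearby living enemies with damage scaled by 0.7 per jump.
; TowerFire starts a looping LightingTick timer that hits one enemy per tick, then sphere-overlaps for the next, skipping those already hit.
; BeginPlay pre-spawns a pool of hidden beam emitters, repositioned and shown for each jump.
; A recursive LightingStrike variant, uncalled here, and a G-key beam test are also present.
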(event EventBeginPlay
  (|CallParentFunction)
  (for _index (range 0 (- (Variables|Default|GetTowerStrikeTimesDefault) 1))
    (bind _returnvalue (Effects|SpawnEmitteratLocation "/Game/Character/Tower/Tesla/Particles/P_Lighting.P_Lighting" "0, 0, 0" "0, 0, 0" "1.000000,1.000000,1.000000" false))
    (Rendering|SetVisibility _returnvalue false false)
    (Utilities|Array|Add (Variables|Default|GetLightingBeams) _returnvalue)))

(event Collision|EventActorBeginOverlap
  (params (OtherActor :type Actor%20Object%20Reference))
  (|CallParentFunction OtherActor) ; This node is disabled and will not be called.\nDrag off pins to build functionality.
)

(event EventTick
  (params (DeltaSeconds :type Float%20%28single-precision%29))
  (|CallParentFunction DeltaSeconds))

(event EventTowerFire
  (bind _targetenemy (Variables|Default|GetTargetEnemy))
  (Development|PrintString "Tesla Fire")
  (Utilities|IsValid _targetenemy
    (:Is%20Valid
      (Variables|Default|SetNextEnemy _targetenemy)
      (Variables|Default|SetLastLightingLocation (Transformation|GetSocketLocation (Variables|Character|GetMesh) "FirePoint"))
      (Variables|Default|SetTowerStrikeTimes 0)
      (bind _returnvalue (Utilities|Time|SetTimerbyFunctionName 0 "LightingTick" 0.1 true))
      (Variables|Default|SetLightingHandle _returnvalue)
      (Utilities|Time|SetTimerbyFunctionName 0 "LightingEffectTick" 0.1 true)
      (Class|TowerBase|PlayFireSound))))

(event Input|KeyboardEvents|G
  (params (Key :type Key%20Structure))
  (bind _returnvalue (Game|GetPlayerCharacter 0))
  (bind _mesh (Variables|Character|GetMesh))
  (bind _lightingbeams (Variables|Default|GetLightingBeams))
  (bind _returnvalue_2 (Transformation|GetActorLocation _returnvalue))
  (bind _returnvalue_3 (Transformation|GetSocketLocation _mesh "FirePoint"))
  (bind _output (Utilities|Array|Get(acopy) _lightingbeams))
  (:Pressed
    (Development|PrintString "tesla ")
    (Rendering|SetVisibility (Utilities|Array|Get(acopy) (Variables|Default|GetLightingBeams)) true false)
    (Rendering|Debug|DrawDebugLine _returnvalue_3 _returnvalue_2 "(R=0.000000,G=0.000000,B=0.000000,A=1.000000)" 2.0 5.0)
    (Class|ParticleSystemComponent|SetBeamSourcePoint _output 0 _returnvalue_3)
    (Class|ParticleSystemComponent|SetBeamTargetPoint _output 0 _returnvalue_2)))

(fn ConstructionScript
  (|CallParentFunction))

(fn LightingStrike
  (params (InRemaningStrike :type Integer) (InTargetEnemy :type Enemy%20Base%20Object%20Reference) (InSplashRadius :type Float%20%28single-precision%29))
  (bind _lightingignorelist (Variables|Default|GetLightingIgnoreList))
  (bind _lightingignorelist_2 (Variables|Default|GetLightingIgnoreList))
  (bind _returnvalue (Utilities|Array|Length _lightingignorelist_2))
  (bind _returnvalue_2 (- _returnvalue 1))
  (bind _output (Utilities|Array|Get(acopy) _lightingignorelist _returnvalue_2))
  (Utilities|FlowControl|Sequence
    (:then_0
      (if (== InRemaningStrike 0)
        (Utilities|Array|Clear (Variables|Default|GetLightingIgnoreList))
        (return)))
    (:then_1
      (LocalVariables|SetRemaningStrike InRemaningStrike))
    (:then_2
      (LocalVariables|SetThisEnemy InTargetEnemy))
    (:then_3
      (LocalVariables|SetSplashRadius InSplashRadius)
      (if (== (Utilities|Array|Length (Variables|Default|GetLightingIgnoreList)) 0)
        (Rendering|Debug|DrawDebugLine (Variables|Default|GetFirePoint) (Variables|Default|GetTargetLocation) "(R=1.000000,G=0.078098,B=0.000000,A=1.000000)" 0.4 3.0)
        (else
          (Utilities|IsValid _output
            (:Is%20Valid
              (Rendering|Debug|DrawDebugLine (Transformation|GetActorLocation _output) (Transformation|GetActorLocation (LocalVariables|GetThisEnemy)) "(R=1.000000,G=0.074510,B=0.000000,A=1.000000)" 0.5 3.0))
            (:Is%20Not%20Valid
              (Utilities|Array|Clear (Variables|Default|GetLightingIgnoreList))
              (return)))))
      ;[1 1 1] Damage
      (Development|PrintString (Utilities|String|ToString(Float) (* (Variables|Default|GetTowerDamage) (Math|Float|Power 0.7 (Math|Conversions|ToFloat(Integer) (- (Variables|Default|GetTowerStrikeTimes) (LocalVariables|GetRemaningStrike)))))) false false)
      (Class|BulkheadCharacterBase|Attack self (LocalVariables|GetThisEnemy) (* (Variables|Default|GetTowerDamage) (Math|Float|Power 0.7 (Math|Conversions|ToFloat(Integer) (- (Variables|Default|GetTowerStrikeTimes) (LocalVariables|GetRemaningStrike))))))
      (Utilities|IsValid (LocalVariables|GetThisEnemy)
        (:Is%20Valid
          (Utilities|Array|Add (Variables|Default|GetLightingIgnoreList) (LocalVariables|GetThisEnemy))
          (bind (_outactors _returnvalue_3) (Collision|SphereOverlapActors (Transformation|GetActorLocation (LocalVariables|GetThisEnemy)) (LocalVariables|GetSplashRadius) (LocalVariables|GetNewLocalVar_0) "/Game/Character/Enemy/EnemyBase/BP_EnemyBase.BP_EnemyBase_C" (Variables|Default|GetLightingIgnoreList)))
          (if _returnvalue_3
            (bind _array_element (Utilities|Array|ForEachLoopwithBreak _outactors)
              (:LoopBody
                (Utilities|IsValid _array_element
                  (:Is%20Valid
                    (bind _asbp_enemy_base (Utilities|Casting|CastToBP_EnemyBase _array_element))
                    (if (== (LocalVariables|GetRemaningStrike) 0)
                      (return)
                      (else
                        (CallFunction|LightingStrike (- (LocalVariables|GetRemaningStrike) 1) _asbp_enemy_base (LocalVariables|GetSplashRadius))
                        (return))))))
              (:Completed
                (Utilities|Array|Clear (Variables|Default|GetLightingIgnoreList))
                (return)))
            (else
              (Utilities|Array|Clear (Variables|Default|GetLightingIgnoreList))
              (return))))))))

(fn LightingTick
  (if (== (Variables|Default|GetTowerStrikeTimes) (Variables|Default|GetTowerStrikeTimesDefault))
    (CallFunction|StopLightingAttack)
    (return)
    (else
      (bind _nextenemy (Variables|Default|GetNextEnemy)
        (:then
          (Utilities|Array|Add (Variables|Default|GetLightingIgnoreList) _nextenemy)
          (CallFunction|PlayLightingEffect (Variables|Default|GetLastLightingLocation) (Transformation|GetActorLocation _nextenemy))
          (Variables|Default|SetLastLightingLocation (Transformation|GetActorLocation _nextenemy))
          (bind (_outactors _returnvalue) (Collision|SphereOverlapActors (Transformation|GetActorLocation _nextenemy) (Variables|Default|GetLIghtingStrikeRadius) (LocalVariables|GetNewLocalVar_2) "/Game/Character/Enemy/EnemyBase/BP_EnemyBase.BP_EnemyBase_C" (Variables|Default|GetLightingIgnoreList)))
          (CallFunction|LightingAttack)
          (if _returnvalue
            (bind _array_element (Utilities|Array|ForEachLoopwithBreak _outactors)
              (:LoopBody
                (Utilities|IsValid _array_element
                  (:Is%20Valid
                    (bind _asbp_enemy_base (Utilities|Casting|CastToBP_EnemyBase _array_element))
                    (bind _returnvalue_2 (Class|BulkheadCharacterBase|GetCharacterData _asbp_enemy_base))
                    (if (> (.health _returnvalue_2) 0.0)
                      (Variables|Default|SetNextEnemy _asbp_enemy_base)
                      (Math|Integer|IncrementInt (Variables|Default|GetTowerStrikeTimes)
                        (:%20%20
                          (return)))))))
              (:Completed
                (CallFunction|StopLightingAttack)
                (return)))
            (else
              (CallFunction|StopLightingAttack)
              (return))))
        (:else
          (return))))))

(fn LightingAttack
  (bind _nextenemy (Variables|Default|GetNextEnemy))
  (Utilities|IsValid _nextenemy
    (:Is%20Valid
      (Class|BulkheadCharacterBase|Attack self _nextenemy (* (Variables|Default|GetTowerDamage) (Math|Float|Power 0.7 (Math|Conversions|ToFloat(Integer) (Variables|Default|GetTowerStrikeTimes))))))))

(fn StopLightingAttack
  (Utilities|Time|ClearandInvalidateTimerbyHandle (Variables|Default|GetLightingHandle))
  (Utilities|Array|Clear (Variables|Default|GetLightingIgnoreList)))

(fn PlayLightingEffect
  (params (Start :type Vector) (End :type Vector))
  (bind _lightingbeams (Variables|Default|GetLightingBeams))
  (bind _towerstriketimes (Variables|Default|GetTowerStrikeTimes))
  (bind _output (Utilities|Array|Get(acopy) _lightingbeams _towerstriketimes))
  (Class|ParticleSystemComponent|SetBeamSourcePoint _output 0 Start)
  (Class|ParticleSystemComponent|SetBeamTargetPoint _output 0 End)
  (Rendering|SetVisibility _output true false))

(fn StopLightingEffect
  (for _array_element (Variables|Default|GetLightingBeams)
    (Rendering|SetVisibility _array_element false false))
  (return))