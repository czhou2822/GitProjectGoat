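; Gatling tower Blueprint, a child tower that attacks a target enemy with direct damage.
; Each tick runs the parent logic and then calls TurnTo.
; The TowerFire event passes the target and tower damage to Attack, draws a brief blue debug line from fire point to target location as the shot visual, and plays the fire sound.
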(event EventTick
  (params (DeltaSeconds :type Float%20%28single-precision%29))
  (|CallParentFunction DeltaSeconds)
  (Utilities|FlowControl|Sequence
    (:then_0
      (CallFunction|Turnto 0.0))))

(event EventTowerFire
  (Class|BulkheadCharacterBase|Attack self (Variables|Default|GetTargetEnemy) (Variables|Default|GetTowerDamage))
  (Rendering|Debug|DrawDebugLine (Variables|Default|GetFirePoint) (Variables|Default|GetTargetLocation) "(R=0.000000,G=0.132017,B=1.000000,A=1.000000)" 0.05 3.0)
  (CallFunction|PlayFireSound))

(fn ConstructionScript
  (|CallParentFunction))