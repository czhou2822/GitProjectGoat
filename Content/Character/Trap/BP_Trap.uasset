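; BP_Trap is the defended objective that loses health when enemies reach it, ending the game as a loss at zero.
; Box overlap applies damage tiered by enemy character ID, up to instant destruction, and kills the enemy without scrap drops.
; Each health change notifies the game state, writes a health ratio to a Material Parameter Collection for UI, and plays a rumble that grows louder and deeper as health falls.
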(event OnComponentBeginOverlap(BoxComponent)
  (params (OverlappedComponent :type Primitive%20Component%20Object%20Reference) (OtherActor :type Actor%20Object%20Reference) (OtherComp :type Primitive%20Component%20Object%20Reference) (OtherBodyIndex :type Integer) (bFromSweep :type Boolean) (SweepResult :type Hit%20Result%20Structure%20%28by%20ref%29))
  ;[1 1 1] Detect Enemy & take damage
  (bind _asbp_enemy_base (Utilities|Casting|CastToBP_EnemyBase OtherActor))
  (bind _returnvalue (Class|BulkheadCharacterBase|GetCharacterData _asbp_enemy_base))
  (if (<= (.id _returnvalue) 5)
    (bind _result (Math|Integer|DecrementInt (Variables|Default|GetBaseHP))
      (:%20%20
        (Class|Trap|SetBaseHealth _result)))
    (elif (<= (.id _returnvalue) 10)
      (bind _output_get (Variables|Default|SetBaseHP (- (Variables|Default|GetBaseHP) 2)))
      (Class|Trap|SetBaseHealth _output_get)
      (else
        (bind _output_get_2 (Variables|Default|SetBaseHP 0))
        (Class|Trap|SetBaseHealth _output_get_2))))
  (Variables|/Script/ProjectGoat.EnemyBase|SetbSpawnScraps _asbp_enemy_base false)
  (Class|BulkheadCharacterBase|MarkforDead _asbp_enemy_base)
  (Audio|PlaySoundatLocation "/Game/Audio/SFX/Trap/C_Trap_Damage.C_Trap_Damage" (Transformation|GetActorLocation) "0, 0, 0" 1.0 1.0 0.0 0 0 0))

(event EventUpdateHealthUI
  ;[1 1 1] Update Health UI
  (Rendering|Material|SetScalarParameterValue "/Game/Materials/MPC_Global_Parameters.MPC_Global_Parameters" "TrapHealth" (/ (Math|Conversions|ToFloat(Integer) (Variables|Default|GetBaseHP)) (Math|Conversions|ToFloat(Integer) (Variables|Default|GetBaseHPDefault))) :!class /Script/Engine.KismetMaterialLibrary))

(event EventSetBaseHealth
  (params (InHealth :type Integer))
  ;[1 1 1] Set health
  (bind _output_get (Variables|Default|SetBaseHP InHealth))
  (Development|PrintString (Utilities|String|ToString(Integer) _output_get))
  (bind _asbp_bulkhead_game_states (Utilities|Casting|CastToBP_BulkheadGameStates (Game|GetGameState)))
  (Default|CallOnTrapDamaged _asbp_bulkhead_game_states _output_get)
  (Class|Trap|UpdateHealthUI)
  (CallFunction|PlayRumble)
  (if (<= _output_get 0)
    (Audio|PlaySoundatLocation (Variables|Audio|GetTrapDestruction) (Transformation|GetActorLocation) "0, 0, 0" 1.0 1.0 0.0 0 0 0)
    (Default|CallBaseExploded)
    (bind _asbp_project_goat_game_mode (Utilities|Casting|CastToBP_ProjectGoatGameMode (Game|GetGameMode)))
    (Class|ProjectGoatGameMode|EndGame _asbp_project_goat_game_mode false)))

(fn ConstructionScript)

(fn PlayRumble
  (bind _basehp (Variables|Default|GetBaseHP))
  (bind _returnvalue (Math|Conversions|ToFloat(Integer) _basehp))
  (Audio|PlaySound2D "/Game/Audio/SFX/Trap/A_Rumble_Cue.A_Rumble_Cue" (Math|Float|MapRangeClamped _returnvalue 6.0 1.0 0.5 2.0) (Math|Float|MapRangeClamped _returnvalue 6.0 1.0 1.0 0.9) 0.0 0 0 false))