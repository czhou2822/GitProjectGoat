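; BP_Reaver is an enemy character that shoots at towers, steering its AI through blackboard keys.
; The SenseTower overlap records the target tower, while EnterAttack applies a random chance before flagging attack and starting a looping timer at the character's attack rate.
; Each tick fires a BP_EnemyBullet from FirePoint, or returns to patrol once the tower is invalid.
; Grunt brittle-state logic is left disconnected.
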(event OnComponentBeginOverlap(SenseGrunt)
  (params (OverlappedComponent :type Primitive%20Component%20Object%20Reference) (OtherActor :type Actor%20Object%20Reference) (OtherComp :type Primitive%20Component%20Object%20Reference) (OtherBodyIndex :type Integer) (bFromSweep :type Boolean) (SweepResult :type Hit%20Result%20Structure%20%28by%20ref%29)))

(event OnComponentBeginOverlap(SenseTower)
  (params (OverlappedComponent :type Primitive%20Component%20Object%20Reference) (OtherActor :type Actor%20Object%20Reference) (OtherComp :type Primitive%20Component%20Object%20Reference) (OtherBodyIndex :type Integer) (bFromSweep :type Boolean) (SweepResult :type Hit%20Result%20Structure%20%28by%20ref%29))
  (bind _asbp_tower_base (Utilities|Casting|CastToBP_TowerBase OtherActor))
  (bind _output_get (Variables|Default|SetTargetTower _asbp_tower_base))
  (CallFunction|SetBlackBoardTarget _output_get))

(event OnComponentEndOverlap(SenseGrunt)
  (params (OverlappedComponent :type Primitive%20Component%20Object%20Reference) (OtherActor :type Actor%20Object%20Reference) (OtherComp :type Primitive%20Component%20Object%20Reference) (OtherBodyIndex :type Integer)))

(event EventBeginPlay
  (|CallParentFunction))

(fn ConstructionScript)

(fn SetBlackBoardAttack
  (params (InIsAttack :type Boolean))
  (AI|Components|Blackboard|SetValueasBool (AI|GetBlackboard (AI|GetAIController self)) (Utilities|Name|MakeLiteralName "IsTowerInRange") InIsAttack))

(fn EnterAttack
  (params (RateOfAttack :type Float%20%28single-precision%29) (TargetTower :type BP%20Tower%20Base%20Object%20Reference))
  (if (< (Math|Random|RandomFloat) RateOfAttack)
    (CallFunction|SetBlackBoardAttack true)
    (CallFunction|SetBlackBoardTarget TargetTower)
    (CallFunction|StartAttackTower TargetTower)))

(fn SetBlackBoardTarget
  (params (TargetTower :type BP%20Tower%20Base%20Object%20Reference))
  (AI|Components|Blackboard|SetValueasObject (AI|GetBlackboard (AI|GetAIController self)) (Utilities|Name|MakeLiteralName "TargetTower") TargetTower))

(fn StartAttackTower
  (params (TargetTower :type BP%20Tower%20Base%20Object%20Reference))
  (Variables|Default|SetTargetTower TargetTower)
  (bind _returnvalue (Class|BulkheadCharacterBase|GetCharacterData))
  (bind _returnvalue_2 (Utilities|Time|SetTimerbyFunctionName 0 "AttackTick" (.attackrate _returnvalue) true))
  (Variables|Default|SetAttackTimer _returnvalue_2))

(fn AttackTick
  (bind _firepoint (Variables|Default|GetFirePoint))
  (bind _returnvalue (Transformation|GetWorldLocation _firepoint))
  (Utilities|IsValid (Variables|Default|GetTargetTower)
    (:Is%20Valid
      (bind _returnvalue_2 (Game|SpawnActorfromClass "/Game/Character/Tower/Projectiles/BP_EnemyBullet.BP_EnemyBullet_C" (Math|Transform|MakeTransform _returnvalue (Math|Rotator|FindLookatRotation _returnvalue (Transformation|GetActorLocation (Variables|Default|GetTargetTower))) "1,1,1") "AdjustIfPossibleButAlwaysSpawn" 0 0))
      (bind _returnvalue_3 (Class|BulkheadCharacterBase|GetCharacterData))
      (Default|SetProjectileParams _returnvalue_2 (.attack _returnvalue_3)))
    (:Is%20Not%20Valid
      (CallFunction|ReturntoPatrol))))

(fn ReturntoPatrol
  (Utilities|Time|ClearandInvalidateTimerbyHandle (Variables|Default|GetAttackTimer))
  (CallFunction|SetBlackBoardAttack false))