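; BP_Grunt is the Blueprint for the Grunt enemy character, adding audible footsteps.
; Its Footstep event plays the enemy footstep sound at the mesh's world location at reduced volume.
; The event's parameter only feeds a PrintText call with screen and log output switched off.
; BeginPlay, overlap and Tick are disabled stubs, and the construction script only calls its parent.
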(event EventBeginPlay
  (|CallParentFunction) ; This node is disabled and will not be called.\nDrag off pins to build functionality.
)

(event Collision|EventActorBeginOverlap
  (params (OtherActor :type Actor%20Object%20Reference)))

(event EventTick
  (params (DeltaSeconds :type Float%20%28single-precision%29))
  (|CallParentFunction DeltaSeconds) ; This node is disabled and will not be called.\nDrag off pins to build functionality.
)

(event EventFootstep
  (params (NewParam :type String))
  (Development|PrintText (Utilities|Text|ToText(String) NewParam) false false)
  (Audio|PlaySoundatLocation (Variables|Default|GetSWEnemyFootStep) (Transformation|GetWorldLocation (Variables|Character|GetMesh)) "0, 0, 0" 0.2 1.0 0.0 0 0 0))

(fn ConstructionScript
  (|CallParentFunction))