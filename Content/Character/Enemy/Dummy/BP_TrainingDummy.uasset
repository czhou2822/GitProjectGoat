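; BP_TrainingDummy is an enemy training dummy that reacts to activation, damage and death with skeletal mesh animations.
; It overrides parent events to play one-shot activate, hit and defeat animations directly on the mesh.
; The hit animation plays only while health remains above zero.
; On death it plays the defeat animation and waits briefly before handing off to the parent's dying logic.
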(event Custom|Activate
  (Components|Animation|PlayAnimation (Variables|Character|GetMesh) "/Game/Character/Enemy/Dummy/Animations/A_Dummy_Activate.A_Dummy_Activate" false))

(event EventOnReceivedDamage
  (params (ReceivedDamage :type Float%20%28single-precision%29) (RemainingHealthPercentage :type Float%20%28single-precision%29))
  (if (not (<= RemainingHealthPercentage 0.0))
    (Components|Animation|PlayAnimation (Variables|Character|GetMesh) "/Game/Character/Enemy/Dummy/Animations/A_Dummy_Hit.A_Dummy_Hit" false)))

(event EventOnCharacterDying
  (Components|Animation|PlayAnimation (Variables|Character|GetMesh) "/Game/Character/Enemy/Dummy/Animations/A_Dummy_Defeat.A_Dummy_Defeat" false)
  (Utilities|FlowControl|Delay 1.0)
  (|CallParentFunction))

(fn ConstructionScript
  (|CallParentFunction))