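; Base enemy character that attacks towers, reacts to freezing, and can drop gold-valued scrap on death.
; Attack helpers set blackboard and anim-instance state, then fire projectiles or apply direct damage to the target tower.
; Freeze amount drives a material parameter and a fully-frozen flag, while state events swap voice audio.
; Dying unpossesses the AI and plays sound, montage, emissive fade and Niagara-linked dissolve, delaying parent death handling by montage length.
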(event Custom|Enter%20Run
  ;[1 1 1] Voice audio for state changes
  (Audio|Components|Audio|SetSound (Variables|Default|GetVoiceAudio) (Variables|Default|GetRunningSound))
  (Audio|Components|Audio|Play (Variables|Default|GetVoiceAudio) 0.0))

(event Custom|HandleOnBulkheadCharacterDead
  (bind _dropgold (Variables|Default|GetDropGold))
  ;[1 1 1] Spawn gears on death
  (if (Variables|Default|GetbSpawnScraps)
    (bind _returnvalue (Game|SpawnActorfromClass (Variables|Default|GetScrapClass) (Math|Transform|MakeTransform (Transformation|GetActorLocation) (Math|Rotator|MakeRotator 0.0 0.0 (Math|Random|RandomFloatinRange 0.0 359.0)) "1,1,1") "AdjustIfPossibleButAlwaysSpawn" 0 0))
    (if (>= _dropgold 0)
      (Variables|/Game/Character/Gears/BP_GearBase.BP_GearBase_C|SetCoinValue _returnvalue _dropgold))))

(event Custom|Enter%20Idle
  ;[1 1 1] Voice audio for state changes
  (Audio|Components|Audio|SetSound (Variables|Default|GetVoiceAudio) (Variables|Default|GetIdleSound))
  (Audio|Components|Audio|Play (Variables|Default|GetVoiceAudio) 0.0))

(event Custom|Event_EnterAttack
  ;[1 1 1] Voice audio for state changes
  (Audio|Components|Audio|SetSound (Variables|Default|GetVoiceAudio) (Variables|Default|GetAttackSound))
  (Audio|Components|Audio|Play (Variables|Default|GetVoiceAudio) 0.0))

(event EventBeginPlay
  ;[1 1 1] Begin play
  (EventDispatchers|BindEventtoOnBulkheadCharacterDead (delegate Custom|HandleOnBulkheadCharacterDead))
  (Class|NiagaraComponent|SetVariableObject (Variables|Default|GetDissolveFX) "BPCallback" self))

(event EventOnCharacterDying
  (bind _voiceaudio (Variables|Default|GetVoiceAudio))
  (bind _deathanimmontage (Variables|Default|GetDeathAnimMontage))
  ;[1 1 1] Dying
  (if (not (Variables|Default|GetDying))
    (Variables|Default|SetDying true)
    (Pawn|UnPossess (AI|GetAIController self))
    (Utilities|FlowControl|Sequence ; 1. Play audio 2. Play particle effects and set death delay 3. delay then call parent death function
      (:then_0
        (Audio|Components|Audio|SetSound _voiceaudio (Variables|Default|GetDeathSound))
        (Audio|Components|Audio|Play _voiceaudio 0.0))
      (:then_1
        ;;[1 1 1] Fade Emissive
        (Audio|Components|Audio|Play (Variables|Default|GetTimeline_Emissive_Death_Fade))
        ;;[1 1 1] Works here but enemy needs to stay dead to play later
        (Audio|Components|Audio|Play (Variables|Default|GetTimeline_Dissolve))
        (Components|Activation|Activate (Variables|Default|GetDissolveFX) false)
        (Animation|Montage|PlayMontage (Variables|Character|GetMesh) _deathanimmontage (Variables|Default|GetDeathPlayRate)
          (:then
            (bind _returnvalue (Animation|GetPlayLength _deathanimmontage))
            (Variables|Default|SetDeathDelay (* (/ _returnvalue (Variables|Default|GetDeathPlayRate)) 0.8)))))
      (:then_2
        (Utilities|FlowControl|Delay (Variables|Default|GetDeathDelay))
        (Class|BulkheadCharacterBase|MarkforDead)
        (|CallParentFunction)))))

(event EventOnSlowStart
  ;[1 1 1] OnSlow
  (Utilities|FlowControl|Sequence
    (:then_0
      (Components|Timeline|PlayfromStart (Variables|Default|GetTimeline_Frozen)))))

(event EventOnSlowEnd
  ;[1 1 1] OnSlow
  (Utilities|FlowControl|Sequence
    (:then_0
      (Audio|Components|Audio|Stop (Variables|Default|GetTimeline_Frozen))
      (CallFunction|SetFrozenEffect 0.0)
      (Variables|Default|SetIsFrozen false))
    (:then_1
      (Class|EnemyBase|EndBrittle))))

(event EventFootstep
  (params (NewParam :type String))
  ;[1 1 1] FootStep
  (Development|PrintText (Utilities|Text|ToText(String) NewParam) false false)
  (Audio|PlaySoundatLocation (Variables|Default|GetFootstepSound) (Transformation|GetWorldLocation (Variables|Character|GetMesh)) "0, 0, 0" 1.0 1.0 0.0 0 0 0))

(event EventParticleData
  (params (Data :type Array%20of%20Basic%20Particle%20Data%20Structures) (NiagaraSystem :type Niagara%20System%20Object%20Reference))
  ;[1 1 1] Particle Data Debug
)

(event EventOnFrozen
  (params (FrozenAmount :type Float%20%28single-precision%29))
  ;[1 1 1] Frozen
  (Development|PrintString (Utilities|String|ToString(Float) FrozenAmount))
  (CallFunction|SetFrozenEffect FrozenAmount)
  (CallFunction|DetermainIsFrozen FrozenAmount))

(fn ConstructionScript
  ;[1 1 1] Death animation speed
  (Components|Timeline|SetPlayRate (Variables|Default|GetTimeline_Emissive_Death_Fade) (Variables|Default|GetDeathPlayRate))
  (Components|Timeline|SetPlayRate (Variables|Default|GetTimeline_Dissolve) (Variables|Default|GetDeathPlayRate)))

(fn SetFrozenEffect
  (params (FreezeAmount :type Float%20%28single-precision%29))
  (Rendering|Material|SetScalarParameterValueonMaterials (Variables|Character|GetMesh) "FreezeAmount" FreezeAmount))

(fn SetBlackBoardFrozen
  (params (NewParam :type Boolean))
  (AI|Components|Blackboard|SetValueasBool (AI|GetBlackboard self) (Utilities|Name|MakeLiteralName "IsFrozen") NewParam))

(fn SetAnimAttackBase
  (params (InIsAttacking :type Boolean))
  (bind _asanim_enemy_base (Utilities|Casting|CastToAnimEnemyBase (Components|SkeletalMesh|GetAnimInstance (Variables|Character|GetMesh))))
  (Variables|/Script/ProjectGoat.AnimEnemyBase|SetbIsAttacking _asanim_enemy_base InIsAttacking))

(fn ReturntoPatrolBase
  (CallFunction|SetBlackBoardAttackBase false))

(fn SetBlackBoardAttackBase
  (params (InIsAttack :type Boolean))
  (AI|Components|Blackboard|SetValueasBool (AI|GetBlackboard (AI|GetAIController self)) (Utilities|Name|MakeLiteralName "IsTowerInRange") InIsAttack))

(fn SpawnBulletBase
  (Utilities|IsValid (Variables|Default|GetTargetTowerBase)
    (:Is%20Valid
      (bind _firelocation (CallFunction|GetFireLocation))
      (bind _returnvalue (Game|SpawnActorfromClass (Variables|Default|GetBulletClass) (Math|Transform|MakeTransform _firelocation (Math|Rotator|FindLookatRotation _firelocation (Transformation|GetActorLocation (Variables|Default|GetTargetTowerBase))) "1,1,1") "AdjustIfPossibleButAlwaysSpawn" 0 0))
      (Utilities|IsValid _returnvalue
        (:Is%20Valid
          (Variables|/Script/Engine.Actor|SetInstigator _returnvalue self)
          (bind _returnvalue_2 (Class|BulkheadCharacterBase|GetCharacterData))
          (Default|SetProjectileParams _returnvalue (.attack _returnvalue_2)))))
    (:Is%20Not%20Valid
      (CallFunction|ReturntoPatrolBase)
      (CallFunction|SetAnimAttackBase false))))

(fn EnterAttackBase
  (params (InTower :type BP%20Tower%20Base%20Object%20Reference))
  (CallFunction|SetBlackBoardAttackBase true)
  (CallFunction|SetBlackBoardTargetBase InTower)
  (CallFunction|SetAnimAttackBase true))

(fn SetBlackBoardTargetBase
  (params (InTower :type BP%20Tower%20Base%20Object%20Reference))
  (AI|Components|Blackboard|SetValueasObject (AI|GetBlackboard (AI|GetAIController self)) (Utilities|Name|MakeLiteralName "TargetTower") InTower))

(fn GetFireLocation
  (return "0, 0, 0"))

(fn DetermainIsFrozen
  (params (InFrozenProgress :type Float%20%28single-precision%29))
  ;[1 1 1] If true, enemy is frozen completely, if false, check if set free completely
  (if (>= InFrozenProgress 1.0)
    ;[1 1 1] If the enemy has not been completely frozen before, set it to frozen and call event
    (if (Variables|Default|GetIsFrozen)
      (return)
      (else
        (Utilities|FlowControl|Sequence ; 1. Set bool 2. stop breathing audio
          (:then_0
            (Variables|Default|SetIsFrozen true)
            (Default|CallOnFrozenCompletely))
          (:then_1
            (Audio|Components|Audio|Stop (Variables|Default|GetVoiceAudio))))))
    (else
      ;[1 1 1] If set free completly, check if it been frozen completly before, if so, reset flag.
      (if (<= InFrozenProgress 0.0)
        (if (Variables|Default|GetIsFrozen)
          (Utilities|FlowControl|Sequence ; 1. Set bool 2. play breathing audio
            (:then_0
              (Variables|Default|SetIsFrozen false))
            (:then_1
              (Audio|Components|Audio|Play (Variables|Default|GetVoiceAudio) 0.0)))
          (else
            (return)))
        (else
          (return))))))

(fn DamageTower
  (Utilities|IsValid (Variables|Default|GetTargetTowerBase)
    (:Is%20Valid
      (Game|Damage|ApplyDamage (Variables|Default|GetTargetTowerBase) 2e+01 0 self))
    (:Is%20Not%20Valid
      (CallFunction|ReturntoPatrolBase)
      (CallFunction|SetAnimAttackBase false))))