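; BP_EnemyRouteSegment is one segment of an enemy route: a NavSplinePoints spline visualized by a Niagara effect that can fade.
; Construction passes spline length and initial opacity to Niagara and sets the timeline's start time from InitVisible.
; ToggleVFX plays or reverses the GlobalOpacity timeline based on its stored Direction, ignoring its Enable input.
; CreateSplineMesh builds shadowless spline meshes between points but is never called here.
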(event EventBeginPlay)

(event Collision|EventActorBeginOverlap
  (params (OtherActor :type Actor%20Object%20Reference)))

(event EventTick
  (params (DeltaSeconds :type Float%20%28single-precision%29)))

(fn ConstructionScript
  (bind _initvisible_ (Variables|Default|GetInitVisible?))
  (bind _returnvalue (Math|Conversions|ToFloat(Boolean) _initvisible_))
  ;[1 1 1] Send spline length to VFX
  (Niagara|SetNiagaraVariable(Float) (Variables|Default|GetNiagara) "SplineLength" (Spline|GetSplineLength (Variables|Default|GetNavSplinePoints)))
  ;[1 1 1] Init VFX opacity & timeline
  (Niagara|SetNiagaraVariable(Float) (Variables|Default|GetNiagara) "GlobalOpacity" _returnvalue)
  (Components|Timeline|SetNewTime (Variables|Default|GetVFX_Timeline) _returnvalue)
  (if (Variables|Default|GetInitVisible?)
    (Variables|Default|SetDirection "Forward")))

(fn CreateSplineMesh
  (bind _navsplinepoints (Variables|Default|GetNavSplinePoints))
  (Development|PrintString "CreateSplineMesh")
  (for _index (range 0 (- (Spline|GetNumberOfSplinePoints _navsplinepoints) 2))
    (bind _returnvalue (AddComponent|AddSplineMeshComponent true))
    (Rendering|SetCastShadow _returnvalue false)
    (Utilities|Array|Add (Variables|Default|GetSplineMeshes) _returnvalue)
    (SplineMesh|SetStartandEnd _returnvalue (.Location (Spline|GetLocationandTangentatSplinePoint _navsplinepoints _index "World")) (.Tangent (Spline|GetLocationandTangentatSplinePoint _navsplinepoints _index "World")) (.Location (Spline|GetLocationandTangentatSplinePoint _navsplinepoints (+ _index 1) "World")) (.Tangent (Spline|GetLocationandTangentatSplinePoint _navsplinepoints (+ _index 1) "World")) true :!class /Script/Engine.SplineMeshComponent)))

(fn ToggleVFX
  (params (Enable :type Boolean))
  (bind _vfx_timeline (Variables|Default|GetVFX_Timeline))
  (switch Utilities|FlowControl|Switch|SwitchonETimelineDirection (Variables|Default|GetDirection)
    (:Forward
      (Utilities|String|Reverse _vfx_timeline))
    (:Backward
      (Audio|Components|Audio|Play _vfx_timeline))))