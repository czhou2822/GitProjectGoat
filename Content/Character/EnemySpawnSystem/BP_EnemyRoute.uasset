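; BP_EnemyRoute is an enemy route actor in the spawn system, with spline, Niagara and segment-based visuals.
; An interface event toggles VFX on each BP_EnemyRouteSegment in RouteSegments.
; BeginPlay registers the actor as the Niagara export callback, whose received particle sizes are only printed.
; CreateSplineMesh builds shadowless spline meshes between NavSplinePoints and calls RouteSplineToArray, but its construction script call is disconnected.
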(event EventBeginPlay
  (Class|NiagaraComponent|SetVariableObject (Variables|Default|GetNS_Route) "BPCallback" self))

(event Collision|EventActorBeginOverlap
  (params (OtherActor :type Actor%20Object%20Reference)))

(event EventTick
  (params (DeltaSeconds :type Float%20%28single-precision%29)))

(event EventParticleData
  (params (Data :type Array%20of%20Basic%20Particle%20Data%20Structures) (NiagaraSystem :type Niagara%20System%20Object%20Reference))
  (bind _array_element (Utilities|Array|ForEachLoopwithBreak Data)
    (:LoopBody
      (Development|PrintString (Utilities|String|ToString(Float) (.Size (Utilities|Struct|BreakBasicParticleData _array_element)))))))

(event EventToggleRouteSegmentVFXInterface
  (params (InEnable :type Boolean))
  (for _array_element (Variables|Default|GetRouteSegments)
    (bind _asbp_enemy_route_segment (Utilities|Casting|CastToBP_EnemyRouteSegment _array_element))
    (Default|ToggleVFX _asbp_enemy_route_segment InEnable)))

(fn ConstructionScript)

(fn CreateSplineMesh
  (bind _navsplinepoints (Variables|Default|GetNavSplinePoints))
  (Development|PrintString "CreateSplineMesh")
  (for _index (range 0 (- (Spline|GetNumberOfSplinePoints _navsplinepoints) 2))
    (bind _returnvalue (AddComponent|AddSplineMeshComponent true))
    (Rendering|SetCastShadow _returnvalue false)
    (Utilities|Array|Add (Variables|Default|GetSplineMeshes) _returnvalue)
    (SplineMesh|SetStartandEnd _returnvalue (.Location (Spline|GetLocationandTangentatSplinePoint _navsplinepoints _index "World")) (.Tangent (Spline|GetLocationandTangentatSplinePoint _navsplinepoints _index "World")) (.Location (Spline|GetLocationandTangentatSplinePoint _navsplinepoints (+ _index 1) "World")) (.Tangent (Spline|GetLocationandTangentatSplinePoint _navsplinepoints (+ _index 1) "World")) true :!class /Script/Engine.SplineMeshComponent))
  (Class|EnemyRoute|RouteSplinetoArray))