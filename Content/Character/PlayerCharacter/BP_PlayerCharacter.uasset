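; Player character for a tower-defense game, handling snow and gold collection, tower spawning, air-strike aiming, pausing and footsteps.
; Input drives the child Frost Cannon's suction and toggles sphere components for scrap pickup and air strikes, which the game mode fires.
; Snow hits paint a render target through a dynamic material; towers spawn via screen-center trace, with timelines pulling out the build camera.
; Debug time-dilation and much disconnected placement and missile logic remain.
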(event OnComponentBeginOverlap(NearPlayerSphere)
  (params (OverlappedComponent :type Primitive%20Component%20Object%20Reference) (OtherActor :type Actor%20Object%20Reference) (OtherComp :type Primitive%20Component%20Object%20Reference) (OtherBodyIndex :type Integer) (bFromSweep :type Boolean) (SweepResult :type Hit%20Result%20Structure%20%28by%20ref%29))
  ;[1 1 1] AirStrikeCheckBox
)

(event OnComponentEndOverlap(NearPlayerSphere)
  (params (OverlappedComponent :type Primitive%20Component%20Object%20Reference) (OtherActor :type Actor%20Object%20Reference) (OtherComp :type Primitive%20Component%20Object%20Reference) (OtherBodyIndex :type Integer))
  ;[1 1 1] AirStrikeCheckBox
)

(event OnComponentBeginOverlap(GoldCollectingSphere)
  (params (OverlappedComponent :type Primitive%20Component%20Object%20Reference) (OtherActor :type Actor%20Object%20Reference) (OtherComp :type Primitive%20Component%20Object%20Reference) (OtherBodyIndex :type Integer) (bFromSweep :type Boolean) (SweepResult :type Hit%20Result%20Structure%20%28by%20ref%29))
  ;[1 1 1] GoldSucking
  (bind _asbp_scrap_base (Utilities|Casting|CastToBP_ScrapBase OtherActor))
  (Default|FlytoPlayerEvent _asbp_scrap_base))

(event Custom|WhichTower
  ;[1 1 1] Spawn Different Towers
  (bind _hitpoint (CallFunction|GetScreentoWorldLocation))
  (switch Utilities|FlowControl|Switch|SwitchonTower_Type (Variables|Default|GetTower)
    (:NewEnumerator1
      (Variables|Default|SetSpawnTowerID 0))
    (:NewEnumerator0
      (Variables|Default|SetSpawnTowerID 1))
    (:NewEnumerator2
      (Variables|Default|SetSpawnTowerID 2)))
  (bind _asbp_project_goat_game_mode (Utilities|Casting|CastToBP_ProjectGoatGameMode (Game|GetGameMode)))
  (bind _returnvalue (Class|ProjectGoatGameMode|SpawnTower _asbp_project_goat_game_mode (Variables|Default|GetSpawnTowerID) (.Location (Math|Transform|BreakTransform (Math|Conversions|ToTransform(Vector) (.Location (Collision|BreakHitResult _hitpoint))))) (.Rotation (Math|Transform|BreakTransform (Math|Conversions|ToTransform(Vector) (.Location (Collision|BreakHitResult _hitpoint)))))))
  (bind _asbp_tower_base (Utilities|Casting|CastToBP_TowerBase _returnvalue))
  (Variables|Default|SetSpawnedTower _asbp_tower_base))

(event Custom|OnCollectSnow_1
  (params (location :type Vector))
  (bind _hitsonwmaterial (Variables|Default|GetHitSonwMaterial))
  ;[1 1 1] collecting snow RTT
  (Rendering|Material|SetVectorParameterValue _hitsonwmaterial "HitLocationW" (Math|Conversions|ToLinearColor(Vector) location) :!class /Script/Engine.MaterialInstanceDynamic)
  (Rendering|DrawMaterialtoRenderTarget "/Game/Materials/Snow/SnowDeformation/Snow_Scene_Capture_RTT2.Snow_Scene_Capture_RTT2" _hitsonwmaterial)
  (Audio|PlaySoundatLocation (Variables|Sound|GetOnSnowCollectSound_0) location "0, 0, 0" 0.2 1.0 0.0 0 0 0))

(event EventTick
  (params (DeltaSeconds :type Float%20%28single-precision%29)))

(event EventPulloutBuildingCamera
  ;[1 1 1] Press Button
  (|PulloutBuildingCamera))

(event EventBeginPlay
  (Utilities|FlowControl|Sequence
    (:then_0
      (BuildingCamera|LockPitchLimit))
    (:then_1
      ;[1 1 1] set up hit snow material
      (bind _returnvalue (Rendering|Material|CreateDynamicMaterialInstance "/Game/Materials/Snow/SnowDeformation/HitOnSnow.HitOnSnow" "None" :!class /Script/Engine.KismetMaterialLibrary))
      (Variables|Default|SetHitSonwMaterial _returnvalue))
    (:then_2
      ;[1 1 1] Setup Variables
      (CallFunction|SetupVariablesBP))))

(event EventResetBuildingCamera
  ;[1 1 1] Press Button
  (|ResetBuildingCamera))

(event EventFootstep
  (params (NewParam :type String))
  (Development|PrintText (Utilities|Text|ToText(String) NewParam) false false)
  (Audio|PlaySoundatLocation (Variables|Default|GetSWCharacterFootStep) (Transformation|GetWorldLocation (Variables|Character|GetMesh)) "0, 0, 0" 0.2 1.0 0.0 0 0 0))

(event Input|ActionEvents|InputActionDestroyTower
  (params (Key :type Key%20Structure :default "None"))
  ;[1 1 1] Press Button
)

(event Input|ActionEvents|InputActionBuild
  (params (Key :type Key%20Structure :default "None"))
  ;[1 1 1] Press Button
)

(event Input|ActionEvents|InputActionCollect
  (params (Key :type Key%20Structure :default "None"))
  ;[1 1 1] CollectSnow
  (:Pressed
    (if (Variables|Default|GetbAiming)
      (bind _asbp_frost_cannon (Utilities|Casting|CastToBP_FrostCannon (Variables|/Script/Engine.ChildActorComponent|GetChildActor (Variables|Default|GetWeaponSlot))))
      (Default|StartSnowSucking _asbp_frost_cannon)))
  (:Released
    (bind _asbp_frost_cannon_2 (Utilities|Casting|CastToBP_FrostCannon (Variables|/Script/Engine.ChildActorComponent|GetChildActor (Variables|Default|GetWeaponSlot))))
    (Default|StopSnowSucking _asbp_frost_cannon_2)))

(event Input|ActionEvents|InputActionBuild
  (params (Key :type Key%20Structure :default "None"))
  ;[1 1 1] TowerSeedThrowing
)

(event Input|ActionEvents|InputActionOpenMenu
  (params (Key :type Key%20Structure :default "None"))
  (bind _returnvalue (Game|GetPlayerController 0))
  ;[1 1 1] Press Button
  (:Pressed
    (Game|SetGamePaused true)
    (bind _returnvalue_2 (UserInterface|CreateWidget "/Game/UI/UMG_Pause.UMG_Pause_C" _returnvalue))
    (UserInterface|Viewport|AddtoViewport _returnvalue_2 0)
    (Input|SetInputModeUIOnly _returnvalue _returnvalue_2 "DoNotLock")
    (Variables|/Script/Engine.PlayerController|SetbShowMouseCursor _returnvalue true)))

(event Input|ActionEvents|InputActionSelectTower
  (params (Key :type Key%20Structure :default "None"))
  ;[1 1 1] Press Button
)

(event Input|ActionEvents|InputActionCollectGold
  (params (Key :type Key%20Structure :default "None"))
  ;[1 1 1] GoldSucking
  (:Pressed
    (CollectingGold|EnableGoldSucking))
  (:Released
    (CollectingGold|DisableGoldSucking)))

(event Input|ActionEvents|InputActionAirStrike
  (params (Key :type Key%20Structure :default "None"))
  ;[1 1 1] AirStrike
)

(event Input|ActionEvents|InputActionAirStrike
  (params (Key :type Key%20Structure :default "None"))
  (:Pressed
    (AirStrike|OnAirStrikeAimUp))
  (:Released
    (AirStrike|OnAirStrikeAimDown)))

(event Input|ActionEvents|InputActionCancel
  (params (Key :type Key%20Structure :default "None")))

(event Input|ActionEvents|InputActionFastForward
  (params (Key :type Key%20Structure :default "None"))
  ;[1 1 1] Speed up
  (:Pressed
    (Variables|Default|SetIsTdown true))
  (:Released
    (Variables|Default|SetIsTdown false)))

(event Input|KeyboardEvents|Z
  (params (Key :type Key%20Structure :default "None")))

(event Input|KeyboardEvents|T
  (params (Key :type Key%20Structure :default "None"))
  (:Pressed
    (Utilities|Time|SetGlobalTimeDilation 5.0)
    (Development|PrintString "fast worward"))
  (:Released
    (Utilities|Time|SetGlobalTimeDilation 1.0)
    (Development|PrintString "back to normal")))

(event Input|KeyboardEvents|G
  (params (Key :type Key%20Structure :default "None")))

(fn ConstructionScript)

(fn GetScreentoWorldLocation
  (bind _returnvalue (Game|GetPlayerController 0))
  (bind _returnvalue_2 (Viewport|GetViewportSize))
  (bind _returnvalue_3 (/ _returnvalue_2 2.0))
  (bind (_worldposition _worlddirection) (Class|GameplayStatics|DeprojectScreentoWorld _returnvalue _returnvalue_3))
  (bind _outhit (Collision|LineTraceForObjects _worldposition (+ _worldposition (* _worlddirection 5000)) (Variables|Default|GetTowerTraceObjectArray) false 0 "ForDuration" true "(R=1.000000,G=0.000000,B=0.000000,A=1.000000)" "(R=0.000000,G=1.000000,B=0.000000,A=1.000000)" 0.2))
  (return _outhit))

(fn SetupVariablesBP
  (Variables|Default|SetTower "NewEnumerator0")
  (Variables|BuildingCamera|SetDefaultFOV (Variables|/Script/Engine.CameraComponent|GetFieldOfView (Variables|Default|GetCamera)))
  (Variables|BuildingCamera|SetDefaultCamaraTransform (Transformation|GetRelativeTransform (Variables|Default|GetCamera)))
  (Variables|BuildingCamera|SetDefaultCameraArmLength (Variables|/Script/Engine.SpringArmComponent|GetTargetArmLength (Variables|Default|GetSpringArm))))

(fn HandleStrikeAim
  (bind _result (Utilities|Set|ToArray (Variables|Default|GetEnemiesAroundPlayer)))
  (for _array_element _result
    (if (.ReturnValue (Class|PlayerController|ProjectWorldLocationtoScreen (Game|GetPlayerController 0) (Transformation|GetActorLocation _array_element) false))
      (Development|PrintString (Utilities|String|Append "Screen location: " (Utilities|String|ToString(Vector2d) (.ScreenLocation (Class|PlayerController|ProjectWorldLocationtoScreen (Game|GetPlayerController 0) (Transformation|GetActorLocation _array_element) false)))) false true "(R=0.000000,G=0.660000,B=1.000000,A=1.000000)" 0.0)
      (Utilities|Array|Add (LocalVariables|GetEnemiesBeingAimed) _array_element)
      (Default|StartMarking _array_element 1.0))))

(fn OnAirStrikeAimUp
  (bind _nearplayersphere (Variables|Default|GetNearPlayerSphere))
  (Rendering|SetVisibility _nearplayersphere true false)
  (Collision|SetCollisionResponsetoChannel _nearplayersphere "ECC_GameTraceChannel9" "ECR_Overlap"))

(fn OnAirStrikeAimDown
  (bind _nearplayersphere (Variables|Default|GetNearPlayerSphere))
  (Rendering|SetVisibility _nearplayersphere false false)
  (Collision|SetCollisionResponsetoChannel _nearplayersphere "ECC_GameTraceChannel9" "ECR_Ignore")
  (bind _asbp_project_goat_game_mode (Utilities|Casting|CastToBP_ProjectGoatGameMode (Game|GetGameMode)))
  (Default|AirStrike _asbp_project_goat_game_mode))

(fn HandleonAirStrikeReady
  (params (ReadyedTower :type BP%20Air%20Strike%20Tower%20Object%20Reference))
  (Development|PrintString (Utilities|String|Append (Utilities|GetDisplayName ReadyedTower) " is ready"))
  (Utilities|Set|Add (Variables|Default|GetAirStrikeTowerSet) ReadyedTower)
  (Math|Integer|IncrementInt (Variables|Default|GetMissileCount)))

(fn AirStrike
  (bind _asbp_frost_cannon (Utilities|Casting|CastToBP_FrostCannon (Variables|/Script/Engine.ChildActorComponent|GetChildActor (Variables|Default|GetWeaponSlot))))
  (bind _output_get (LocalVariables|SetAirStrikeList (Variables|/Game/Character/Weapon/BP_FrostCannon.BP_FrostCannon_C|GetAirStrikeList _asbp_frost_cannon)))
  (if (and (> (Utilities|Set|Length _output_get) 0) (> (Utilities|Set|Length (Variables|Default|GetAirStrikeTowerSet)) 0))
    (bind _result (Utilities|Set|ToArray (Variables|Default|GetAirStrikeTowerSet)))
    (for _array_element _result
      (Utilities|FlowControl|Sequence
        (:then_0
          (bind _result_2 (Utilities|Set|ToArray (LocalVariables|GetAirStrikeList)))
          (Utilities|IsValid (Utilities|Array|Get(acopy) _result_2)
            (:Is%20Valid
              (bind _output_get_2 (LocalVariables|SetSingleEnemy (Utilities|Array|Get(acopy) _result_2)))
              (Default|AirStrike _array_element _output_get_2)
              (bind _returnvalue (Utilities|Set|Remove (LocalVariables|GetAirStrikeList) _output_get_2))
              (if _returnvalue
                (Math|Integer|DecrementInt (Variables|Default|GetMissileCount))))
            (:Is%20Not%20Valid
              (Utilities|Set|Remove (LocalVariables|GetAirStrikeList) (Utilities|Array|Get(acopy) _result_2)))))))
    (Utilities|Set|Clear (Variables|Default|GetAirStrikeTowerSet))))

(fn LockPitchLimit
  (bind _returnvalue (Game|GetPlayerCameraManager 0))
  ;[1 1 1] limiting the camera pitch
  (Variables|/Script/Engine.PlayerCameraManager|SetViewPitchMin _returnvalue -8e+01)
  (Variables|/Script/Engine.PlayerCameraManager|SetViewPitchMax _returnvalue 1e+01))

(fn UnlockPitchLimit
  (bind _returnvalue (Game|GetPlayerCameraManager 0))
  ;[1 1 1] limiting the camera pitch
  (Variables|/Script/Engine.PlayerCameraManager|SetViewPitchMin _returnvalue -1e+01)
  (Variables|/Script/Engine.PlayerCameraManager|SetViewPitchMax _returnvalue 6e+01))

(fn IsinMonitor
  (params (InLocation :type Vector%202D%20Structure) (ComparingArea :type Vector%202D%20Structure))
  (if (<= (.x InLocation) (.x ComparingArea))
    (if (<= (.y InLocation) (.y ComparingArea))
      (return true)
      (else
        (return false)))
    (else
      (return false))))

(fn EnableGoldSucking
  (Rendering|SetVisibility (Variables|Default|GetGoldCollectingSphere) true false)
  (bind _result (Utilities|Set|ToArray (Variables|Default|GetCoinList)))
  (for _array_element _result
    (Default|FlytoPlayerEvent _array_element))
  (Utilities|Set|Clear (Variables|Default|GetCoinList)))

(fn DisableGoldSucking
  (Rendering|SetVisibility (Variables|Default|GetGoldCollectingSphere) false false))