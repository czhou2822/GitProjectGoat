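; BP_BulkheadPlayerState is a player state that tracks the player's gold and air strike charges.
; CollectGold adds to the gold total, and ConsumeGold deducts a cost only when affordable, returning whether it succeeded.
; RechargeAirStrike adds one charge until the maximum count is reached.
; The event graph and construction script hold no logic.
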(event EventBeginPlay)

(event EventTick
  (params (DeltaSeconds :type Float%20%28single-precision%29)))

(fn ConstructionScript)

(fn RechargeAirStrike
  (if (>= (Variables|Default|GetAirStrikeCount) (Variables|Default|GetMaxAirStrikeCount))
    (return)
    (else
      (Math|Integer|IncrementInt (Variables|Default|GetAirStrikeCount)))))

(fn ConsumeGold
  (params (Cost :type Integer))
  (if (>= (- (Variables|Gold|GetGold) Cost) 0)
    (Variables|Gold|SetGold (- (Variables|Gold|GetGold) Cost))
    (return true)
    (else
      (return false))))

(fn CollectGold
  (params (InGold :type Integer))
  (Variables|Gold|SetGold (+ InGold (Variables|Gold|GetGold))))