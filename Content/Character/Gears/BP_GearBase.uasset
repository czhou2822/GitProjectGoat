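; BP_GearBase is a gear pickup that flies to the player and adds its coin value when collected.
; FlyToPlayer_Event waits a second, builds a two-point spline to player 0, then a timeline moves the skeletal mesh along it.
; Tick keeps the spline's end on the moving player.
; When the timeline finishes, ConsumeSelf credits BP_BulkheadPlayerState, plays the pickup sound and destroys the actor.
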(event Custom|FlyToPlayer_Event
  (bind _spline (Variables|Default|GetSpline))
  (Utilities|FlowControl|Delay 1.0)
  (if (not (Variables|Default|GetIsMoving))
    (CallFunction|SetSplinePointstoPlayer)
    (Variables|Default|SetIsMoving true)
    (bind _newtrack_0 (Timeline|Timeline_0 PlayFromStart)
      (:Update
        (Transformation|SetRelativeLocation (Variables|Default|GetSkeletalMesh) (Spline|GetLocationatDistanceAlongSpline _spline (* _newtrack_0 (Spline|GetSplineLength _spline)) "Local") false false))
      (:Finished
        (CallFunction|ConsumeSelf)))))

(event EventBeginPlay
  (Audio|Components|Audio|SetSound (Variables|Default|GetScrapAudioComp) (Variables|Audio|GetScrapLoop))
  (Audio|Components|Audio|Play (Variables|Default|GetScrapAudioComp) 0.0))

(event Collision|EventActorBeginOverlap
  (params (OtherActor :type Actor%20Object%20Reference)))

(event EventTick
  (params (DeltaSeconds :type Float%20%28single-precision%29))
  (if (Variables|Default|GetIsMoving)
    (Spline|SetLocationatSplinePoint (Variables|Default|GetSpline) (- (Spline|GetNumberOfSplinePoints (Variables|Default|GetSpline)) 1) (Transformation|GetActorLocation (Game|GetPlayerCharacter 0)) "World" true)))

(fn ConstructionScript)

(fn SetSplinePointstoPlayer
  (Spline|ClearSplinePoints (Variables|Default|GetSpline) true)
  (Spline|AddSplinePoint (Variables|Default|GetSpline) (Transformation|GetActorLocation) "World" true)
  (Spline|AddSplinePoint (Variables|Default|GetSpline) (Transformation|GetActorLocation (Game|GetPlayerCharacter 0)) "World" true)
  (Development|PrintString (Utilities|String|Append "numer of spline now: " (Utilities|String|ToString(Integer) (Spline|GetNumberOfSplinePoints (Variables|Default|GetSpline)))) false false))

(fn ConsumeSelf
  (Utilities|IsValid self
    (:Is%20Valid
      (bind _asbp_bulkhead_player_state (Utilities|Casting|CastToBP_BulkheadPlayerState (Variables|/Script/Engine.Controller|GetPlayerState (Game|GetPlayerController 0))))
      (Class|BulkheadPlayerState|AddCointoPlayer _asbp_bulkhead_player_state (Variables|Default|GetCoinValue))
      (Audio|PlaySoundatLocation (Variables|Audio|GetScrapPickup) (Transformation|GetActorLocation) "0, 0, 0" 1.0 1.0 0.0 0 0 0)
      (Actor|DestroyActor))))