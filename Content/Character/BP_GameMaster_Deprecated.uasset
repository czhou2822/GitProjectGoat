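; Deprecated game master that runs the wave loop: Building, Building to Combat, Combat and Post Combat.
; It reacts to game mode phase changes, using looping countdown timers to request the next phase.
; Each wave's DataTable row configures the spawn points, whose completion callbacks trigger Post Combat.
; After the enemy check passes, it starts building again or wins if no row remains; base explosion loads the fail level.
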(event BaseExploded(BaseObject)
  (CallFunction|EndGameFailed))

(event Custom|OnWaveComplete_Event_0
  ;[1 1 1] DataBinding
  (CallFunction|HandleonWaveCompleteBP))

(event Custom|BindOnBulkChanged
  (params (CurrentBulkCount :type Integer))
  (CallFunction|HandleonBulkChanged CurrentBulkCount))

(event Custom|OnPhaseChange_Event_0
  (params (NewParam :type ENUM_GamePhase%20Enum :default "NewEnumerator0"))
  ;[1 1 1] DataBinding
  (CallFunction|HandleonPhaseChange NewParam))

(event EventBeginPlay
  (Utilities|FlowControl|Sequence
    (:then_0
      (bind _result (Utilities|Set|ToArray (Variables|Spawn|GetSpawnPointsArray)))
      ;[1 1 1] DataBinding
      (for _array_element _result
        (Utilities|IsValid _array_element
          (:Is%20Valid
            (EventDispatchers|AssignOnWaveCompleteBP _array_element (delegate Custom|OnWaveComplete_Event_0))
            (Variables|/Game/Character/Misc/BP_EnemySpawn.BP_EnemySpawn_C|SetBaseLocation _array_element (Transformation|GetActorLocation (Variables|Gameplay|GetBaseObject)))
            (bind _asbp_project_goat_game_mode (Utilities|Casting|CastToBP_ProjectGoatGameMode (Game|GetGameMode)))
            (EventDispatchers|AssignOnPhaseChangeBP _asbp_project_goat_game_mode (delegate Custom|OnPhaseChange_Event_0))))))
    (:then_2
      (if (Variables|Spawn|GetIsSpawning)
        (BuildingPhase|StartBuildingPhaseBP (Variables|BuildingPhase|GetBuildingPhaseWaitTime))))))

(fn ConstructionScript)

(fn HandleonWaveCompleteBP
  (bind _result (Math|Integer|DecrementInt (Variables|Default|GetSpawnPointNumbers))
    (:%20%20
      (if (== _result 0)
        (Development|PrintString "WaveComplete")
        (bind _asbp_project_goat_game_mode (Utilities|Casting|CastToBP_ProjectGoatGameMode (Game|GetGameMode)))
        (Default|SetGamePhaseBP _asbp_project_goat_game_mode "NewEnumerator3")))))

(fn HandleonCollectingPhaseComplete
  (bind _asbp_project_goat_game_mode (Utilities|Casting|CastToBP_ProjectGoatGameMode (Game|GetGameMode)))
  (Default|SetGamePhaseBP _asbp_project_goat_game_mode "NewEnumerator1"))

(fn HandleonBulkChanged
  (params (InBulkCount :type Integer))
  (Variables|Gameplay|SetBulkCountString (Utilities|String|Append "BulkCount: " (Utilities|String|ToString(Integer) InBulkCount) "/" (Utilities|String|ToString(Integer) (Variables|Gameplay|GetBulkTarget))))
  (if (>= InBulkCount (Variables|Gameplay|GetBulkTarget))
    (CallFunction|EndGameSuccess)))

(fn EndGameSuccess
  (Development|PrintString "Thanks for playing" true true "(R=1.000000,G=0.000000,B=0.008526,A=1.000000)" 3e+01)
  (Game|OpenLevel(byName) "EndGameLevel"))

(fn StartBuildingtoCombatPhaseBP
  (params (WaveNumber :type Integer))
  (Variables|Default|SetSpawnPointNumbers (Utilities|Set|Length (Variables|Spawn|GetSpawnPointsArray)))
  (bind _output (BuildingtoCombat|GetandSetWaveStatBP (Utilities|String|StringToName (Utilities|String|ToString(Integer) WaveNumber))))
  (CallFunction|StruttoString _output false)
  (BuildingToCombat|ParseandSetActiveSpawnPoints _output)
  (BuildingtoCombat|StartBuildingtoCombatTimer (Variables|BuildingToCombat|GetBuildingToCombatWaitTime)))

(fn StartBuildingtoCombatTimer
  (params (WaitTime :type Float%20%28single-precision%29))
  (Variables|BuildingToCombat|SetBuildingToCombatTickCount (/ WaitTime (Variables|BuildingToCombat|GetBuildingToCombatTickInterval)))
  (bind _returnvalue (Utilities|Time|SetTimerbyFunctionName 0 "BuildingToCombatTick" (Variables|BuildingToCombat|GetBuildingToCombatTickInterval) true))
  (Variables|BuildingtoCombat|SetBuildingToCombatTimerHandler _returnvalue))

(fn BuildingtoCombatTickBP
  (if (> (Variables|BuildingToCombat|GetBuildingToCombatTickCount) 0.0)
    (Math|Float|DecrementFloat (Variables|BuildingToCombat|GetBuildingToCombatTickCount))
    (else
      (Utilities|Time|ClearandInvalidateTimerbyHandle (Variables|BuildingtoCombat|GetBuildingToCombatTimerHandler))
      (bind _asbp_project_goat_game_mode (Utilities|Casting|CastToBP_ProjectGoatGameMode (Game|GetGameMode)))
      (Default|SetGamePhaseBP _asbp_project_goat_game_mode "NewEnumerator2"))))

(fn GetandSetWaveStatBP
  (params (InWaveNumber :type Name))
  (bind _returnvalue (Utilities|String|ToString(Name) InWaveNumber))
  (bind _returnvalue_2 (Utilities|String|Append "WaveNumber: " _returnvalue))
  (Development|PrintString _returnvalue_2)
  (bind _returnvalue_3 (Utilities|GetDataTableRow "/Game/DataTable/DataTable_WaveStructProto.DataTable_WaveStructProto" InWaveNumber)
    (:then
      (bind _output_get (Variables|Default|SetSpawnWaveDetails _returnvalue_3))
      (return _output_get))
    (:RowNotFound
      (Development|PrintString (Utilities|String|Append _returnvalue_2 " not found. ")))))

(fn IsGameEnded
  (Variables|Gameplay|SetisGameEnd (== (Variables|/Script/ProjectGoat.InventoryComponent|GetBulkCount (Actor|GetComponentbyClass (Variables|Gameplay|GetPlayerCharacter) "/Script/ProjectGoat.InventoryComponent")) (Variables|Gameplay|GetBulkTarget)))
  (return))

(fn StruttoString
  (params (InStruct :type Spawn%20Wave%20Detail%20BPPPPP%20Structure) (PrintString :type Boolean))
  (bind (_wavenumber _spawnpoints) (Utilities|Struct|BreakSpawnWaveDetailBPPPPP InStruct))
  (if PrintString
    (Development|PrintString (Utilities|String|Append (Utilities|String|Append "Number: " (Utilities|String|ToString(Integer) _wavenumber)) (Utilities|String|Append " ActiveSpawnPointNumbers: " (Utilities|String|ToString(Integer) (Utilities|Array|Length _spawnpoints)))))
    (for _array_element _spawnpoints
      (for _array_element_2 (.miniwavenumbers _array_element)
        (Development|PrintString (Utilities|String|Append "MiniWave: " (Utilities|String|ToString(Integer) (.miniwavenumbers _array_element_2)) " route number: " (.route _array_element_2) " GruntID: " (Utilities|String|ToString(Integer) (.gruntsid _array_element_2)) " Grunt Number: " (Utilities|String|ToString(Integer) (.gruntsnumber _array_element_2))))
        (return)))))

(fn StartBuildingPhaseBP
  (params (WaitTime :type Float%20%28single-precision%29))
  (Variables|BuildingPhase|SetBuildingPhaseTickCount (/ WaitTime (Variables|BuildingPhase|GetBuildingPhaseTickInterval)))
  (bind _returnvalue (Utilities|Time|SetTimerbyFunctionName 0 "BuildingPhaseTick" (Variables|BuildingPhase|GetBuildingPhaseTickInterval) true))
  (Variables|BuildingPhase|SetBuildingPhaseTimerHandler _returnvalue)
  (bind _asbp_bulkhead_game_states (Utilities|Casting|CastToBP_BulkheadGameStates (Game|GetGameState)))
  (Default|ClearActiveEnemyListBP _asbp_bulkhead_game_states))

(fn BuildingPhaseTickBP
  (if (> (Variables|BuildingPhase|GetBuildingPhaseTickCount) 0.0)
    (Math|Float|DecrementFloat (Variables|BuildingPhase|GetBuildingPhaseTickCount))
    (else
      (Utilities|Time|ClearandInvalidateTimerbyHandle (Variables|BuildingPhase|GetBuildingPhaseTimerHandler))
      (bind _asbp_project_goat_game_mode (Utilities|Casting|CastToBP_ProjectGoatGameMode (Game|GetGameMode)))
      (Default|SetGamePhaseBP _asbp_project_goat_game_mode "NewEnumerator1"))))

(fn EndGameFailed
  (Game|OpenLevel(byName) "FailLevel"))

(fn ParseandSetActiveSpawnPoints
  (params (InWave :type Spawn%20Wave%20Detail%20BPPPPP%20Structure))
  (bind (_wavenumber _spawnpoints) (Utilities|Struct|BreakSpawnWaveDetailBPPPPP InWave))
  (bind _spawnpointsarray (Variables|Spawn|GetSpawnPointsArray))
  (bind _returnvalue (Utilities|Array|Length _spawnpoints))
  (bind _returnvalue_2 (Utilities|Set|Length _spawnpointsarray))
  (if (> _returnvalue _returnvalue_2)
    (Development|PrintString (Utilities|String|Append "Wave " (Utilities|String|ToString(Integer) _wavenumber) " number invalid. " "SpawnPoints in table: " (Utilities|String|ToString(Integer) _returnvalue) "SpawnPoints in world: " (Utilities|String|ToString(Integer) _returnvalue_2)))
    (return)
    (else
      (for _array_element _spawnpoints
        (bind _result (Utilities|Set|ToArray (Variables|Spawn|GetSpawnPointsArray)))
        (Variables|/Game/Character/Misc/BP_EnemySpawn.BP_EnemySpawn_C|SetCurrentWaveStat (Utilities|Array|Get(acopy) _result (.spawnpointindex _array_element)) (.miniwavenumbers _array_element))
        (Variables|/Game/Character/Misc/BP_EnemySpawn.BP_EnemySpawn_C|SetSpawnInterval_0 (Utilities|Array|Get(acopy) _result (.spawnpointindex _array_element)) (.spawninterval _array_element)))
      (return))))

(fn SetActiveWaveSpawnPoint
  (params (SpawnPointIndex :type Integer))
  (bind _result (Utilities|Set|ToArray (Variables|Spawn|GetSpawnPointsArray)))
  (return (Utilities|Array|Get(acopy) _result SpawnPointIndex)))

(fn HandleonPhaseChange
  (params (InPhase :type ENUM_GamePhase%20Enum :default "NewEnumerator0"))
  (switch Utilities|FlowControl|Switch|SwitchonENUM_GamePhase InPhase
    (:NewEnumerator0
      (BuildingPhase|StartBuildingPhaseBP (Variables|BuildingPhase|GetBuildingPhaseWaitTime)))
    (:NewEnumerator1
      (bind _result (Math|Integer|IncrementInt (Variables|Spawn|GetWaveCounter))
        (:%20%20
          (BuildingtoCombat|StartBuildingtoCombatPhaseBP _result)
          (Utilities|Time|SetGlobalTimeDilation 1.0))))
    (:NewEnumerator2
      (Default|CallOnStartWaveGMBP))
    (:NewEnumerator3
      (PostCombat|StartPostCombatTimer (Variables|PostCombat|GetPostCombatWaitTime)))))

(fn StartPostCombatTimer
  (params (WaitTime :type Float%20%28single-precision%29))
  (bind _postcombattickinterval (Variables|PostCombat|GetPostCombatTickInterval))
  (Variables|PostCombat|SetPostCombatTick (Math|Float|Truncate (/ WaitTime _postcombattickinterval)))
  (bind _returnvalue (Utilities|Time|SetTimerbyFunctionName 0 "PostCombatTickFunction" _postcombattickinterval true))
  (Variables|PostCombat|SetPostCombatHandler _returnvalue))

(fn PostCombatTickFunction
  (bind _result (Math|Integer|DecrementInt (Variables|PostCombat|GetPostCombatTick))
    (:%20%20
      (bind _asbp_bulkhead_game_states (Utilities|Casting|CastToBP_BulkheadGameStates (Game|GetGameState)))
      (bind _isallclear (Default|CheckAllActiveEnemyBP _asbp_bulkhead_game_states))
      (if (and (<= _result 0) _isallclear)
        (Utilities|GetDataTableRow "/Game/DataTable/DataTable_WaveStructProto.DataTable_WaveStructProto" (Utilities|String|StringToName (Utilities|String|ToString(Integer) (+ (Variables|Spawn|GetWaveCounter) 1)))
          (:then
            (Utilities|Time|ClearandInvalidateTimerbyHandle (Variables|PostCombat|GetPostCombatHandler))
            (bind _asbp_project_goat_game_mode (Utilities|Casting|CastToBP_ProjectGoatGameMode (Game|GetGameMode)))
            (Default|SetGamePhaseBP _asbp_project_goat_game_mode "NewEnumerator0"))
          (:RowNotFound
            (CallFunction|EndGameSuccess)))))))