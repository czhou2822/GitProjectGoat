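; BP_Constructor is a tossed physics object that turns into a tower after it lands.
; It launches its mesh with TossVelocity on BeginPlay and stops simulating physics on hitting WorldStatic or a custom channel.
; Drop sound and Niagara effect play at the HoloTower's XY and its own height.
; After a delay, it shakes the camera, has BP_PlayerCharacter build the tower from HoloTower and TowerType, then destroys itself.
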(event OnComponentHit(StaticMesh)
  (params (HitComponent :type Primitive%20Component%20Object%20Reference) (OtherActor :type Actor%20Object%20Reference) (OtherComp :type Primitive%20Component%20Object%20Reference) (NormalImpulse :type Vector :default "0, 0, 0") (Hit :type Hit%20Result%20Structure%20%28by%20ref%29))
  (bind _returnvalue (Collision|GetCollisionObjectType OtherComp))
  (bind _holotower (Variables|Default|GetHoloTower))
  (bind _returnvalue_2 (Transformation|GetActorLocation _holotower))
  (if (or (Utilities|Enum|Equal(Enum) _returnvalue "ECC_WorldStatic") (Utilities|Enum|Equal(Enum) _returnvalue "ECC_GameTraceChannel5"))
    (Development|PrintString "Hit" false false)
    (Physics|SetSimulatePhysics (Variables|Default|GetStaticMesh) false)
    ;[1 1 1] Build FX Location from Input XY and Actor Z
    (bind _output_get (Variables|Default|SetFXLocation (Math|Vector|MakeVector (.x _returnvalue_2) (.y _returnvalue_2) (.z (Transformation|GetActorLocation)))))
    (Audio|PlaySoundatLocation "/Game/Audio/SFX/Constructor/SC_Tower_Drop.SC_Tower_Drop" _output_get "0, 0, 0" 1.0 1.0 0.0 "/Game/Audio/Attenuation/SA_Tower_Drop.SA_Tower_Drop" 0 0)
    (Niagara|SpawnSystematLocation "/Game/VFX/Constructor/NS_Tower_Drop.NS_Tower_Drop" (Variables|Default|GetFXLocation))
    (Utilities|FlowControl|Delay 2.5)
    (Camera|PlayWorldCameraShake "/Game/VFX/Blueprints/BP_CameraShake_Explosion.BP_CameraShake_Explosion_C" (Variables|Default|GetFXLocation) 0.0 2e+03 1.0 true)
    (bind _asbp_player_character (Utilities|Casting|CastToBP_PlayerCharacter (Game|GetPlayerCharacter 0)))
    (Class|TPSCharacterQ|TurnConstructorIntoTower _asbp_player_character (Variables|Default|GetHoloTower) (Variables|Default|GetTowerType))
    (Actor|DestroyActor)))

(event EventBeginPlay
  (Physics|SetPhysicsLinearVelocity (Variables|Default|GetStaticMesh) (Variables|Default|GetTossVelocity) false "None"))

(event Collision|EventActorBeginOverlap
  (params (OtherActor :type Actor%20Object%20Reference)))

(event EventTick
  (params (DeltaSeconds :type Float%20%28single-precision%29)))

(fn ConstructionScript)