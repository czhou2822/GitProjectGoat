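; Enemy spawner that runs waves of mini-waves when BP_GameMaster signals wave start.
; Looping timers spawn each mini-wave's enemies through BulkheadGameState and count down the delay before the next.
; Grunts and Revers alternate by countdown parity with bosses last, each enemy receiving spline-based nav points from Routes.
; Wave completion fires after the last mini-wave delay; a separate event-triggered wait fires it once spawned enemies are gone or time runs out.
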(event Custom|OnWaitForWaveToComplete_Event
  (Variables|WaitforWave|SetWaitForWaveToCompleteTickCount (Variables|WaitforWave|GetWaitForWaveToCompleteTickCountDefault))
  (bind _returnvalue (Utilities|Time|SetTimerbyFunctionName 0 "WaitForWaveToCompleteTick" (Variables|WaitForWave|GetWaitForWaveToCompleteTickInterval) true))
  (Variables|WaitforWave|SetWaitForWaveToCompleteTimer _returnvalue))

(event Custom|OnStartWaveGM_Event_0
  (Development|PrintString (Utilities|String|Append (Utilities|GetObjectName self) " starts wave"))
  (CallFunction|SpawnNextWave (Variables|Default|GetCurrentWaveStat)))

(event Custom|OnMiniWaveComplete_Event
  (CallFunction|HandleonMiniWaveComplete))

(event EventBeginPlay
  (bind _outactors (Actor|GetAllActorsOfClass "/Game/Character/BP_GameMaster.BP_GameMaster_C"))
  (EventDispatchers|AssignOnStartWaveGM (Utilities|Array|Get(acopy) _outactors) (delegate Custom|OnStartWaveGM_Event_0))
  (EventDispatchers|BindEventtoOnWaitforWavetoComplete (delegate Custom|OnWaitForWaveToComplete_Event))
  (Variables|WaitforWave|SetWaitForWaveToCompleteTickCountDefault (Math|Float|Truncate (/ (Variables|WaitforWave|GetWaitForWaveToCompleteInSecond) (Variables|WaitForWave|GetWaitForWaveToCompleteTickInterval))))
  (EventDispatchers|BindEventtoOnMiniWaveComplete (delegate Custom|OnMiniWaveComplete_Event)))

(fn ConstructionScript)

(fn SpawnSingleEnemy
  (bind _arrow (Variables|Default|GetArrow))
  (bind _returnvalue (Transformation|GetWorldTransform _arrow))
  (bind (_location _rotation) (Math|Transform|BreakTransform _returnvalue))
  (if (> (Variables|Default|GetEnemyToBeSpawn) 0)
    (bind _asbulkhead_game_state (Utilities|Casting|CastToBulkheadGameState (Game|GetGameState)))
    (bind _output (CallFunction|GetNextMonsterID))
    (bind _returnvalue_2 (Class|BulkheadGameState|SpawnMonster _asbulkhead_game_state _output 0 _location _rotation))
    (Utilities|Set|Add (Variables|Default|GetEnemyArray) _returnvalue_2)
    (bind _asbp_enemy_base (Utilities|Casting|CastToBP_EnemyBase _returnvalue_2))
    (Variables|/Game/Character/Enemy/EnemyBase/BP_EnemyBase.BP_EnemyBase_C|SetBaseLocation _asbp_enemy_base (Variables|Default|GetBaseLocation))
    (bind _navpoints (CallFunction|GetNavPoints (Math|Integer|%(Integer) (Variables|Default|GetEnemyToBeSpawn) (Utilities|Array|Length (Variables|Default|GetCurrentRoutes)))))
    (Variables|/Game/Character/Enemy/EnemyBase/BP_EnemyBase.BP_EnemyBase_C|SetNavPoints _asbp_enemy_base _navpoints)
    (Math|Integer|DecrementInt (Variables|Default|GetEnemyToBeSpawn)
      (:%20%20
        (return)))
    (else
      ;[1 1 1] Spawn complete, wait for wave to be complete
      (Default|CallOnMiniWaveComplete)
      (Utilities|Time|ClearandInvalidateTimerbyHandle (Variables|Default|GetSpawnWaveTimer))
      (return))))

(fn SpawnNextWave
  (params (WaveStat :type Array%20of%20Mini%20Wave%20Detail%20Structures))
  (if (>= (Variables|Default|GetCurrentMiniWaveIndex) (Utilities|Array|Length WaveStat))
    (Default|CallOnWaveComplete)
    (elif (> (Utilities|Array|Length WaveStat) 0)
      (CallFunction|SpawnMiniWave (Utilities|Array|Get(acopy) WaveStat (Variables|Default|GetCurrentMiniWaveIndex)))
      (else
        (Development|PrintString (Utilities|String|Append (Utilities|GetObjectName self) " wave stat invalid"))))))

(fn SpawnMiniWave
  (params (ThisMiniWave :type Mini%20Wave%20Detail%20Structure))
  (bind _output_get (Variables|Default|SetCurrentMiniWaveStat ThisMiniWave))
  (CallFunction|ParseRouteNumber (.route _output_get))
  (Variables|Default|SetEnemyToBeSpawn (+ (.gruntsnumber _output_get) (.reversnumber _output_get) (.bossnumber _output_get)))
  (bind _returnvalue (Utilities|Time|SetTimerbyFunctionName 0 "SpawnSingleEnemy" (Variables|Default|GetSpawnInterval) true))
  (Variables|Default|SetSpawnWaveTimer _returnvalue))

(fn WaitforWavetoCompleteTick
  (bind _result (Utilities|Set|ToArray (Variables|Default|GetEnemyArray)))
  (for _array_element _result
    (Utilities|IsValid _array_element
      (:Is%20Not%20Valid
        (Utilities|Set|Remove (Variables|Default|GetEnemyArray) _array_element))))
  (if (== (Utilities|Set|Length (Variables|Default|GetEnemyArray)) 0)
    (Default|CallOnWaveComplete)
    (Utilities|Time|ClearandInvalidateTimerbyHandle (Variables|WaitforWave|GetWaitForWaveToCompleteTimer))
    (elif (> (Variables|WaitforWave|GetWaitForWaveToCompleteTickCount) 0)
      (Math|Integer|DecrementInt (Variables|WaitforWave|GetWaitForWaveToCompleteTickCount))
      (else
        (Default|CallOnWaveComplete)
        (Utilities|Time|ClearandInvalidateTimerbyHandle (Variables|WaitforWave|GetWaitForWaveToCompleteTimer))))))

(fn WaitforMiniWaveTick
  (bind _currentwavestat (Variables|Default|GetCurrentWaveStat))
  (if (>= (Variables|WaitfornextMiniWave|GetWaitForNextMiniWaveToCompleteTickCount) (Variables|WaitfornextMiniWave|GetWaitForNextMiniWaveToCompleteTickCountDefault))
    (bind _result (Math|Integer|IncrementInt (Variables|Default|GetCurrentMiniWaveIndex))
      (:%20%20
        (if (>= _result (Utilities|Array|Length _currentwavestat))
          (Default|CallOnWaveComplete)
          (Utilities|Time|ClearandInvalidateTimerbyHandle (Variables|WaitfornextMiniWave|GetWaitForNextMiniWaveTimer))
          (else
            (CallFunction|SpawnNextWave _currentwavestat)))))
    (else
      (Math|Integer|IncrementInt (Variables|WaitfornextMiniWave|GetWaitForNextMiniWaveToCompleteTickCount)))))

(fn RouteSplinetoArray
  (params (InRoute :type BP%20Enemy%20Route%20Object%20Reference))
  (Utilities|Array|Clear (LocalVariables|GetOutArray))
  (if (Utilities|IsValid InRoute)
    (for _index (range 0 (- (Spline|GetNumberOfSplinePoints (Variables|/Script/ProjectGoat.EnemyRoute|GetNavSplinePoints InRoute)) 1))
      (Utilities|Array|Add (LocalVariables|GetOutArray) (Spline|GetLocationatSplinePoint (Variables|/Script/ProjectGoat.EnemyRoute|GetNavSplinePoints InRoute) _index "World")))
    (return (LocalVariables|GetOutArray))
    (else
      (Development|PrintString "Route not valid")
      (return (LocalVariables|GetOutArray)))))

(fn DestroyWaveActor
  (bind _result (Utilities|Set|ToArray (Variables|Default|GetEnemyArray)))
  (for _array_element _result
    (Actor|DestroyActor _array_element)))

(fn GetNavPoints
  (params (NewParam :type Integer))
  (bind _newparam (CallFunction|RouteSplinetoArray (Utilities|Array|Get(acopy) (Variables|Default|GetRoutes) NewParam)))
  (return _newparam))

(fn ParseRouteNumber
  (params (NewParam :type String))
  (Utilities|Array|Clear (Variables|Default|GetCurrentRoutes))
  (for _array_element (Utilities|String|ParseIntoArray NewParam ",")
    (Utilities|Array|Add (Variables|Default|GetCurrentRoutes) (Math|Conversions|ToInteger(Byte) _array_element)))
  (return))

(fn HandleonMiniWaveComplete
  ;[1 1 1] start wait for mini wave
  (Variables|WaitfornextMiniWave|SetWaitForNextMiniWaveToCompleteTickCount 0)
  (Variables|WaitfornextMiniWave|SetWaitForNextMiniWaveToCompleteTickCountDefault (Math|Float|Truncate (/ (.delaytonextwave (Utilities|Array|Get(acopy) (Variables|Default|GetCurrentWaveStat) (Variables|Default|GetCurrentMiniWaveIndex))) (Variables|WaitForWave|GetWaitForWaveToCompleteTickInterval))))
  (bind _returnvalue (Utilities|Time|SetTimerbyFunctionName 0 "WaitForMiniWaveTick" (Variables|WaitForWave|GetWaitForWaveToCompleteTickInterval) true))
  (Variables|WaitfornextMiniWave|SetWaitForNextMiniWaveTimer _returnvalue))

(fn GetNextMonsterID
  (bind _currentminiwavestat (Variables|Default|GetCurrentMiniWaveStat))
  (LocalVariables|SetMiniWaveStat (Variables|Default|GetCurrentMiniWaveStat))
  (if (or (Math|Conversions|ToBoolean(Integer) (.reversnumber _currentminiwavestat)) (Math|Conversions|ToBoolean(Integer) (.bossnumber _currentminiwavestat)))
    (if (<= (Variables|Default|GetEnemyToBeSpawn) (.bossnumber (LocalVariables|GetMiniWaveStat)))
      (return (.bossid (LocalVariables|GetMiniWaveStat)))
      (else
        (switch int (Math|Integer|%(Integer) (Variables|Default|GetEnemyToBeSpawn) 2)
          (:0
            (return (.gruntsid (LocalVariables|GetMiniWaveStat))))
          (:1
            (return (.reversid (LocalVariables|GetMiniWaveStat)))))))
    (else
      (return (.gruntsid _currentminiwavestat)))))