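; BP_EnemyRoute is an actor holding the NavSplinePoints spline, which by its name defines an enemy route.
; On BeginPlay, CreateSplineMesh adds one manually attached spline mesh component per spline segment and stores it in SplineMeshes.
; Each mesh is bent between neighboring points using their world-space locations and tangents, so the route's mesh is built at runtime rather than in the construction script.
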(event EventBeginPlay
  (CallFunction|CreateSplineMesh))

(event Collision|EventActorBeginOverlap
  (params (OtherActor :type Actor%20Object%20Reference)))

(event EventTick
  (params (DeltaSeconds :type Float%20%28single-precision%29)))

(fn ConstructionScript)

(fn CreateSplineMesh
  (bind _navsplinepoints (Variables|Default|GetNavSplinePoints))
  (for _index (range 0 (- (Spline|GetNumberOfSplinePoints _navsplinepoints) 2))
    (bind _returnvalue (AddComponent|AddSplineMeshComponent true))
    (Utilities|Array|Add (Variables|Default|GetsplineMeshes) _returnvalue)
    (SplineMesh|SetStartandEnd _returnvalue (.Location (Spline|GetLocationandTangentatSplinePoint _navsplinepoints _index "World")) (.Tangent (Spline|GetLocationandTangentatSplinePoint _navsplinepoints _index "World")) (.Location (Spline|GetLocationandTangentatSplinePoint _navsplinepoints (+ _index 1) "World")) (.Tangent (Spline|GetLocationandTangentatSplinePoint _navsplinepoints (+ _index 1) "World")) true :!class /Script/Engine.SplineMeshComponent)))