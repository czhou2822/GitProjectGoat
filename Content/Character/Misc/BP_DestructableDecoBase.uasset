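; BP_DestructableDecoBase is a decoration actor, named as a base class, that is destroyed when a tower overlaps it.
; Its StaticMesh begin-overlap event prints the overlapping component's name on screen, then casts the other actor to Gatling, Mortar or Tesla tower.
; Any match calls DestroyDeco, which spawns a destruction particle system and plays a sound at the actor's bounds center, then destroys the actor.
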(event OnComponentBeginOverlap(StaticMesh)
  (params (OverlappedComponent :type Primitive%20Component%20Object%20Reference) (OtherActor :type Actor%20Object%20Reference) (OtherComp :type Primitive%20Component%20Object%20Reference) (OtherBodyIndex :type Integer) (bFromSweep :type Boolean) (SweepResult :type Hit%20Result%20Structure%20%28by%20ref%29))
  (Development|PrintString (Utilities|GetDisplayName OtherComp) true false "(R=5.000000,G=0.108700,B=0.050000,A=1.000000)" 3.0)
  (Utilities|Casting|CastToBP_GatlingTower OtherActor
    (:then
      _)
    (:CastFailed
      (Utilities|Casting|CastToBP_MortarTower OtherActor
        (:then
          _)
        (:CastFailed
          (Utilities|Casting|CastToBP_TeslaTower OtherActor)))))
  (CallFunction|DestroyDeco))

(event EventBeginPlay)

(event Collision|EventActorBeginOverlap
  (params (OtherActor :type Actor%20Object%20Reference)))

(event EventTick
  (params (DeltaSeconds :type Float%20%28single-precision%29)))

(fn ConstructionScript)

(fn DestroyDeco
  (bind _origin (Collision|GetActorBounds false false))
  ;[1 1 1] Spawn particle FX at actors bounds center
  (Niagara|SpawnSystematLocation "/Game/VFX/NS_Environment_Destruction.NS_Environment_Destruction" _origin)
  (Audio|PlaySoundatLocation "/Game/Audio/SFX/Destruction/A_Haystand_Cue.A_Haystand_Cue" _origin "0, 0, 0" 1.0 1.0 0.1 0 0 0)
  (Actor|DestroyActor))