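; Game state Blueprint, by its name, that keeps registries of active enemies and prioritized enemies.
; Helper functions add, remove and clear active enemies, and prune invalid references, with the all-enemy check returning true only when no valid enemy remains.
; The prioritized list is cleared at construction and accepts only valid enemies for adding or removal.
; BeginPlay and Tick are empty, and a debug print of a prioritized list count is left disconnected.
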(event EventBeginPlay)

(event EventTick
  (params (DeltaSeconds :type Float%20%28single-precision%29)))

(fn ConstructionScript
  (Utilities|Set|Clear (Variables|Default|GetPrioritizedEnemyListBP)))

(fn AddActiveEnemyBP
  (params (InEnemy :type BP%20Enemy%20Base%20Object%20Reference))
  (Utilities|Set|Add (Variables|Default|GetActiveEnemies) InEnemy))

(fn CheckActiveEnemyBP
  (params (NewParam :type BP%20Enemy%20Base%20Object%20Reference))
  (Utilities|IsValid NewParam
    (:Is%20Not%20Valid
      (CallFunction|DeleteActiveEnemyBP NewParam))))

(fn DeleteActiveEnemyBP
  (params (NewParam :type BP%20Enemy%20Base%20Object%20Reference))
  (Utilities|Set|Remove (Variables|Default|GetActiveEnemies) NewParam))

(fn CheckAllActiveEnemyBP
  (bind _result (Utilities|Set|ToArray (Variables|Default|GetActiveEnemies)))
  (for _array_element _result
    (Utilities|IsValid _array_element
      (:Is%20Valid
        (return false))
      (:Is%20Not%20Valid
        (Utilities|Set|Remove (Variables|Default|GetActiveEnemies) 0))))
  (return true))

(fn ClearActiveEnemyListBP
  (Utilities|Set|Clear (Variables|Default|GetActiveEnemies)))

(fn AddtoPrioritizedListBP
  (params (NewParam :type BP%20Enemy%20Base%20Object%20Reference))
  (Utilities|IsValid NewParam
    (:Is%20Valid
      (Utilities|Set|Add (Variables|Default|GetPrioritizedEnemyListBP) NewParam)
      (return))))

(fn DeletefromPrioritizedListBP
  (params (InEnemy :type BP%20Enemy%20Base%20Object%20Reference))
  (Utilities|IsValid InEnemy
    (:Is%20Valid
      (Utilities|Set|Remove (Variables|Default|GetPrioritizedEnemyListBP) InEnemy)
      (return))))