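; Player controller that handles the pause menu and the hold-to-open tower selection radial wheel.
; The pause widget is created hidden at BeginPlay; OpenMenu pauses the game and reveals it with the cursor, with no toggle back here.
; SelectTower notifies BP_PlayerCharacter, shows the wheel unless a tower is being placed, and removes it on release, restoring game-only input.
; GetJoystickDirection returns a stick's 2D vector, inverting Y for the left stick.
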(event EventBeginPlay
  (bind _returnvalue (UserInterface|CreateWidget "/Game/UI/UMG_Pause.UMG_Pause_C"))
  (bind _output_get (Variables|Default|SetPauseMenu _returnvalue))
  (Widget|SetVisibility _output_get "Hidden")
  (UserInterface|Viewport|AddtoViewport _output_get 0))

(event Input|ActionEvents|InputActionSelectTower
  (params (Key :type Key%20Structure :default "None"))
  (:Pressed
    (bind _asbp_player_character (Utilities|Casting|CastToBP_PlayerCharacter (Game|GetPlayerCharacter 0)))
    (Default|CallOnPlayerSelectingTower _asbp_player_character true)
    (if (not (Variables|/Script/ProjectGoat.TPSCharacterQ|GetIsCharacterPlacingTower _asbp_player_character))
      (Variables|Default|GetSelectionWheel
        (:then
          _)
        (:else
          (bind _returnvalue (Game|ConstructObjectfromClass "/Game/UI/UMG_BulkhedRadialMenu.UMG_BulkhedRadialMenu_C" self))
          (Variables|Default|SetSelectionWheel _returnvalue)))
      (UserInterface|Viewport|AddtoViewport (Variables|Default|GetSelectionWheel) 0)
      (Input|SetInputModeGameandUI (Game|GetPlayerController 0) (Variables|Default|GetSelectionWheel) "DoNotLock" true)))
  (:Released
    (bind _asbp_player_character_2 (Utilities|Casting|CastToBP_PlayerCharacter (Game|GetPlayerCharacter 0)))
    (Default|CallOnPlayerSelectingTower _asbp_player_character_2 false)
    (bind _selectionwheel (Variables|Default|GetSelectionWheel)
      (:then
        (Widget|RemovefromParent _selectionwheel)
        (Variables|Default|SetSelectionWheel 0)
        (Input|SetInputModeGameOnly (Game|GetPlayerController 0)))
      (:else))))

(event Input|ActionEvents|InputActionOpenMenu
  (params (Key :type Key%20Structure :default "None"))
  (:Pressed
    (Game|SetGamePaused true)
    (Variables|Default|SetbShowMouseCursor true)
    (Input|SetInputModeGameandUI (Game|GetPlayerController 0) 0 "DoNotLock" true)
    (Widget|SetVisibility (Variables|Default|GetPauseMenu) "Visible")))

(fn ConstructionScript)

(fn GetJoystickDirection
  (params (Stick :type EJoystickTypes%20Enum :default "NewEnumerator0"))
  (switch Utilities|FlowControl|Switch|SwitchonEJoystickTypes Stick
    (:NewEnumerator0
      (return (Math|Vector2D|MakeVector2D (Class|Actor|GetInputAxisKeyValue) (* (Class|Actor|GetInputAxisKeyValue) -1.0))))
    (:NewEnumerator1
      (return (Math|Vector2D|MakeVector2D (Class|Actor|GetInputAxisKeyValue) (Class|Actor|GetInputAxisKeyValue))))))