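; Game mode for Project Goat that sets game-only input at BeginPlay and controls a fast-forward for the building phase.
; Each Tick, while the player character's IsTdown flag is set, global time dilation becomes 5x during BUILDINGPHASE and normal otherwise; it is untouched when the flag is clear.
; An air strike system with target and tower lists, firing and timed recharge remains, but its logic is disconnected and never runs.
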(event EventBeginPlay
  (Input|SetInputModeGameOnly (Game|GetPlayerController 0)))

(event EventTick
  (params (DeltaSeconds :type Float%20%28single-precision%29))
  (bind _asbp_player_character (Utilities|Casting|CastToBP_PlayerCharacter (Game|GetPlayerCharacter 0)))
  (if (Variables|/Game/Character/PlayerCharacter/BP_PlayerCharacter.BP_PlayerCharacter_C|GetIsTdown _asbp_player_character)
    (if (Utilities|Enum|Equal(Enum) (Variables|Default|GetGamePhase) "BUILDINGPHASE")
      (Utilities|Time|SetGlobalTimeDilation 5.0)
      (else
        (Utilities|Time|SetGlobalTimeDilation 1.0)))))

(fn ConstructionScript)

(fn AddtoStrikeList
  (params (NewTarget :type BP%20Enemy%20Base%20Object%20Reference)))

(fn RemovefromStrikeList
  (params (NewTarget :type BP%20Enemy%20Base%20Object%20Reference)))

(fn AirStrike)

(fn AddAirStrikeTower
  (params (NewAirStrikeTower :type BP%20Air%20Strike%20Tower%20Object%20Reference)))

(fn AirStrikeTimerTick)