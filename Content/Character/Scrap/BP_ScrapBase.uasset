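; Base scrap pickup that flies to the player and is collected as coin value.
; FlyToPlayer_Event builds a two-point spline from the scrap to the player, while Tick keeps the end point on the player's moving position.
; A timeline slides the skeletal mesh along the spline, then ConsumeSelf passes CoinValue to BP_PlayerCharacter and destroys the actor.
; The overlap handler is empty and the raised midpoint for an arc is disconnected.
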(event OnComponentBeginOverlap(SphereComp)
  (params (OverlappedComponent :type Primitive%20Component%20Object%20Reference) (OtherActor :type Actor%20Object%20Reference) (OtherComp :type Primitive%20Component%20Object%20Reference) (OtherBodyIndex :type Integer) (bFromSweep :type Boolean) (SweepResult :type Hit%20Result%20Structure%20%28by%20ref%29)))

(event Custom|FlyToPlayer_Event
  (bind _spline (Variables|Default|GetSpline))
  (if (not (Variables|Default|GetIsMoving))
    (CallFunction|SetSplinePointstoPlayer)
    (Variables|Default|SetIsMoving true)
    (bind _newtrack_0 (Timeline|Timeline_0 PlayFromStart)
      (:Update
        (Transformation|SetRelativeLocation (Variables|Default|GetSkeletalMesh) (Spline|GetLocationatDistanceAlongSpline _spline (* _newtrack_0 (Spline|GetSplineLength _spline)) "Local") false false))
      (:Finished
        (CallFunction|ConsumeSelf)))))

(event EventBeginPlay)

(event Collision|EventActorBeginOverlap
  (params (OtherActor :type Actor%20Object%20Reference)))

(event EventTick
  (params (DeltaSeconds :type Float%20%28single-precision%29))
  (if (Variables|Default|GetIsMoving)
    (Spline|SetLocationatSplinePoint (Variables|Default|GetSpline) (- (Spline|GetNumberOfSplinePoints (Variables|Default|GetSpline)) 1) (Transformation|GetActorLocation (Game|GetPlayerCharacter 0)) "World" true)))

(fn ConstructionScript)

(fn SetSplinePointstoPlayer
  (Spline|ClearSplinePoints (Variables|Default|GetSpline) true)
  (Spline|AddSplinePoint (Variables|Default|GetSpline) (Transformation|GetActorLocation) "World" true)
  (Spline|AddSplinePoint (Variables|Default|GetSpline) (Transformation|GetActorLocation (Game|GetPlayerCharacter 0)) "World" true)
  (Development|PrintString (Utilities|String|Append "numer of spline now: " (Utilities|String|ToString(Integer) (Spline|GetNumberOfSplinePoints (Variables|Default|GetSpline)))) false false))

(fn ConsumeSelf
  (Utilities|IsValid self
    (:Is%20Valid
      (bind _asbp_player_character (Utilities|Casting|CastToBP_PlayerCharacter (Game|GetPlayerCharacter 0)))
      (Class|TPSCharacterQ|CoinCollect _asbp_player_character (Variables|Default|GetCoinValue))
      (Actor|DestroyActor))))