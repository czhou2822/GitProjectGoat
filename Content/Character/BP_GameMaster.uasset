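; Game master that runs the match loop, alternating timed collecting phases with enemy waves.
; When collecting ends, it loads the next wave's DataTable row, configures spawn points by index and broadcasts the wave start.
; Spawn point completion events count down to the next collecting phase.
; Reaching the player inventory's bulk target opens the end-game level, while base explosion or a missing wave row opens the fail level.
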(event BaseExploded(BaseObject)
  (CallFunction|EndGameFailed))

(event Custom|BindOnCollectingPhaseComplete
  ;[1 1 1] DataBinding
  (CallFunction|HandleonCollectingPhaseComplete))

(event Custom|OnWaveComplete_Event_0
  ;[1 1 1] DataBinding
  (CallFunction|HandleonWaveComplete))

(event Custom|BindOnBulkChanged
  (params (CurrentBulkCount :type Integer))
  (CallFunction|HandleonBulkChanged CurrentBulkCount))

(event EventBeginPlay
  (Utilities|FlowControl|Sequence
    (:then_0
      (bind _result (Utilities|Set|ToArray (Variables|Spawn|GetSpawnPointsArray)))
      ;[1 1 1] DataBinding
      (for _array_element _result
        (Utilities|IsValid _array_element
          (:Is%20Valid
            (EventDispatchers|AssignOnWaveComplete _array_element (delegate Custom|OnWaveComplete_Event_0))
            (EventDispatchers|AssignOnCollectingPhaseComplete (delegate Custom|BindOnCollectingPhaseComplete))
            (Variables|/Game/Character/Misc/BP_EnemySpawn.BP_EnemySpawn_C|SetBaseLocation _array_element (Transformation|GetActorLocation (Variables|Gameplay|GetBaseObject))))))
      (bind _asbp_player_character (Utilities|Casting|CastToBP_PlayerCharacter (Game|GetPlayerCharacter 0)))
      (bind _output_get (Variables|Gameplay|SetPlayerCharacter _asbp_player_character))
      (EventDispatchers|AssignOnBulkChanged (Variables|/Script/ProjectGoat.TPSCharacterQ|GetInventoryComp _output_get) (delegate Custom|BindOnBulkChanged))
      (Variables|Gameplay|SetBulkCountString (Utilities|String|Append "BulkCount:  0/" (Utilities|String|ToString(Integer) (Variables|Gameplay|GetBulkTarget)))))
    (:then_2
      (if (Variables|Spawn|GetIsSpawning)
        (CallFunction|StartCollectionPhase)))))

(fn ConstructionScript)

(fn HandleonWaveComplete
  (bind _result (Math|Integer|DecrementInt (Variables|Default|GetSpawnPointNumbers))
    (:%20%20
      (if (== _result 0)
        (Development|PrintString "WaveComplete")
        (CallFunction|StartCollectionPhase)))))

(fn HandleonCollectingPhaseComplete
  (if (Variables|Gameplay|GetisGameEnd)
    (CallFunction|EndGameSuccess)
    (else
      (bind _result (Math|Integer|IncrementInt (Variables|Spawn|GetWaveCounter))
        (:%20%20
          (CallFunction|StartWave _result))))))

(fn HandleonBulkChanged
  (params (InBulkCount :type Integer))
  (Variables|Gameplay|SetBulkCountString (Utilities|String|Append "BulkCount: " (Utilities|String|ToString(Integer) InBulkCount) "/" (Utilities|String|ToString(Integer) (Variables|Gameplay|GetBulkTarget))))
  (if (>= InBulkCount (Variables|Gameplay|GetBulkTarget))
    (CallFunction|EndGameSuccess)))

(fn CollectingPhaseTick
  (if (> (Variables|Spawn|GetCollectingPhaseTickCount) 0.0)
    (Math|Float|DecrementFloat (Variables|Spawn|GetCollectingPhaseTickCount))
    (else
      (Default|CallOnCollectingPhaseComplete)
      (Development|PrintString "Collecting Phase complete")
      (Utilities|Time|ClearandInvalidateTimerbyHandle (Variables|Spawn|GetCollectingPhaseTimerHandler)))))

(fn EndGameSuccess
  (Development|PrintString "Thanks for playing" true true "(R=1.000000,G=0.000000,B=0.008526,A=1.000000)" 3e+01)
  (Game|OpenLevel(byName) "EndGameLevel"))

(fn GetandSetWaveStat
  (params (InWaveNumber :type Name))
  (Development|PrintString (Utilities|String|Append "WaveNumber: " (Utilities|String|ToString(Name) InWaveNumber)))
  (bind _returnvalue (Utilities|GetDataTableRow "/Game/DataTable/DataTable_WaveStructProto.DataTable_WaveStructProto" InWaveNumber)
    (:then
      (bind _output_get (Variables|Default|SetSpawnWaveDetails _returnvalue))
      (return _output_get))
    (:RowNotFound
      (Development|PrintString "Wave Number Not Found")
      (CallFunction|EndGameFailed))))

(fn StartWave
  (params (WaveNumber :type Integer))
  (Variables|Default|SetSpawnPointNumbers (Utilities|Set|Length (Variables|Spawn|GetSpawnPointsArray)))
  (bind _output (CallFunction|GetandSetWaveStat (Utilities|String|StringToName (Utilities|String|ToString(Integer) WaveNumber))))
  (CallFunction|StruttoString _output true)
  (CallFunction|ParseandSetActiveSpawnPoints _output)
  (Default|CallOnStartWaveGM))

(fn IsGameEnded
  (Variables|Gameplay|SetisGameEnd (== (Variables|/Script/ProjectGoat.InventoryComponent|GetBulkCount (Actor|GetComponentbyClass (Variables|Gameplay|GetPlayerCharacter) "/Script/ProjectGoat.InventoryComponent")) (Variables|Gameplay|GetBulkTarget)))
  (return))

(fn StruttoString
  (params (InStruct :type Spawn%20Wave%20Detail%20Structure) (PrintString :type Boolean))
  (bind (_wavenumber _spawnpoints) (Utilities|Struct|BreakSpawnWaveDetail InStruct))
  (if PrintString
    (Development|PrintString (Utilities|String|Append (Utilities|String|Append "Number: " (Utilities|String|ToString(Integer) _wavenumber)) (Utilities|String|Append " ActiveSpawnPointNumbers: " (Utilities|String|ToString(Integer) (Utilities|Array|Length _spawnpoints)))))
    (for _array_element _spawnpoints
      (for _array_element_2 (.miniwavenumbers _array_element)
        (Development|PrintString (Utilities|String|Append "MiniWave: " (Utilities|String|ToString(Integer) (.miniwavenumbers _array_element_2)) " route number: " (.route _array_element_2) " GruntID: " (Utilities|String|ToString(Integer) (.gruntsid _array_element_2)) " Grunt Number: " (Utilities|String|ToString(Integer) (.gruntsnumber _array_element_2))))
        (return)))))

(fn StartCollectionPhase
  (Variables|Spawn|SetCollectingPhaseTickCount (/ (Variables|Spawn|GetCollectingPhaseInSecond) (Variables|Spawn|GetCollectingPhaseTickInterval)))
  (bind _returnvalue (Utilities|Time|SetTimerbyFunctionName 0 "CollectingPhaseTick" (Variables|Spawn|GetCollectingPhaseTickInterval) true))
  (Variables|Spawn|SetCollectingPhaseTimerHandler _returnvalue))

(fn EndGameFailed
  (Game|OpenLevel(byName) "FailLevel"))

(fn ParseandSetActiveSpawnPoints
  (params (InWave :type Spawn%20Wave%20Detail%20Structure))
  (bind (_wavenumber _spawnpoints) (Utilities|Struct|BreakSpawnWaveDetail InWave))
  (bind _spawnpointsarray (Variables|Spawn|GetSpawnPointsArray))
  (bind _returnvalue (Utilities|Array|Length _spawnpoints))
  (bind _returnvalue_2 (Utilities|Set|Length _spawnpointsarray))
  (if (> _returnvalue _returnvalue_2)
    (Development|PrintString (Utilities|String|Append "Wave " (Utilities|String|ToString(Integer) _wavenumber) " number invalid. " "SpawnPoints in table: " (Utilities|String|ToString(Integer) _returnvalue) "SpawnPoints in world: " (Utilities|String|ToString(Integer) _returnvalue_2)))
    (return)
    (else
      (for _array_element _spawnpoints
        (bind _result (Utilities|Set|ToArray (Variables|Spawn|GetSpawnPointsArray)))
        (Variables|/Game/Character/Misc/BP_EnemySpawn.BP_EnemySpawn_C|SetCurrentWaveStat (Utilities|Array|Get(acopy) _result (.spawnpointindex _array_element)) (.miniwavenumbers _array_element))
        (Variables|/Game/Character/Misc/BP_EnemySpawn.BP_EnemySpawn_C|SetSpawnInterval (Utilities|Array|Get(acopy) _result (.spawnpointindex _array_element)) (.spawninterval _array_element)))
      (return))))

(fn SetActiveWaveSpawnPoint
  (params (SpawnPointIndex :type Integer))
  (bind _result (Utilities|Set|ToArray (Variables|Spawn|GetSpawnPointsArray)))
  (return (Utilities|Array|Get(acopy) _result SpawnPointIndex)))