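; BP_Trap is an actor with its own hit points that destroys enemies reaching its trigger box, losing health for each one.
; When a BP_EnemyBase overlaps the box, it plays a damage sound, destroys that enemy and decrements BaseHP.
; At zero or below, it plays a destruction sound and fires the BaseExploded dispatcher; otherwise it prints remaining against default HP.
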(event OnComponentBeginOverlap(Box)
  (params (OverlappedComponent :type Primitive%20Component%20Object%20Reference) (OtherActor :type Actor%20Object%20Reference) (OtherComp :type Primitive%20Component%20Object%20Reference) (OtherBodyIndex :type Integer) (bFromSweep :type Boolean) (SweepResult :type Hit%20Result%20Structure%20%28by%20ref%29))
  (bind _asbp_enemy_base (Utilities|Casting|CastToBP_EnemyBase OtherActor))
  (Audio|PlaySoundatLocation (Variables|Audio|GetTrapDamage) (Transformation|GetActorLocation) "0, 0, 0" 1.0 1.0 0.0 0 0 0)
  (Actor|DestroyActor _asbp_enemy_base)
  (bind _result (Math|Integer|DecrementInt (Variables|Default|GetBaseHP))
    (:%20%20
      (if (<= _result 0)
        (Audio|PlaySoundatLocation (Variables|Audio|GetTrapDestruction) (Transformation|GetActorLocation) "0, 0, 0" 1.0 1.0 0.0 0 0 0)
        (Default|CallBaseExploded)
        (else
          (Development|PrintString (Utilities|String|Append (Utilities|String|ToString(Integer) (Variables|Default|GetBaseHP)) "/" (Utilities|String|ToString(Integer) (Variables|Default|GetBaseHPDefault)))))))))

(event EventBeginPlay)

(event Collision|EventActorBeginOverlap
  (params (OtherActor :type Actor%20Object%20Reference)))

(event EventTick
  (params (DeltaSeconds :type Float%20%28single-precision%29)))

(fn ConstructionScript)