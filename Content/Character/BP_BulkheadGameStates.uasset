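; BP_BulkheadGameStates is a game state Blueprint that keeps track of enemies in two collections, active and prioritized.
; Functions add, remove and clear active enemies, while CheckAllActiveEnemy prunes invalid entries and returns true only when no valid enemy remains.
; The prioritized list takes validity-checked adds and removes and is emptied in the construction script.
; BeginPlay and Tick are empty, and a debug print of the prioritized count is disconnected.
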(event EventBeginPlay)

(event EventTick
  (params (DeltaSeconds :type Float%20%28single-precision%29)))

(fn ConstructionScript
  (Utilities|Set|Clear (Variables|Default|GetPrioritizedEnemyList)))

(fn AddActiveEnemy
  (params (InEnemy :type BP%20Enemy%20Base%20Object%20Reference))
  (Utilities|Set|Add (Variables|Default|GetActiveEnemies) InEnemy))

(fn CheckActiveEnemy
  (params (NewParam :type BP%20Enemy%20Base%20Object%20Reference))
  (Utilities|IsValid NewParam
    (:Is%20Not%20Valid
      (CallFunction|DeleteActiveEnemy NewParam))))

(fn DeleteActiveEnemy
  (params (NewParam :type BP%20Enemy%20Base%20Object%20Reference))
  (Utilities|Set|Remove (Variables|Default|GetActiveEnemies) NewParam))

(fn CheckAllActiveEnemy
  (bind _result (Utilities|Set|ToArray (Variables|Default|GetActiveEnemies)))
  (for _array_element _result
    (Utilities|IsValid _array_element
      (:Is%20Valid
        (return false))
      (:Is%20Not%20Valid
        (Utilities|Set|Remove (Variables|Default|GetActiveEnemies) 0))))
  (return true))

(fn ClearActiveEnemyList
  (Utilities|Set|Clear (Variables|Default|GetActiveEnemies)))

(fn AddtoPrioritizedList
  (params (NewParam :type BP%20Enemy%20Base%20Object%20Reference))
  (Utilities|IsValid NewParam
    (:Is%20Valid
      (Utilities|Set|Add (Variables|Default|GetPrioritizedEnemyList) NewParam)
      (return))))

(fn DeletefromPrioritizedList
  (params (InEnemy :type BP%20Enemy%20Base%20Object%20Reference))
  (Utilities|IsValid InEnemy
    (:Is%20Valid
      (Utilities|Set|Remove (Variables|Default|GetPrioritizedEnemyList) InEnemy)
      (return))))