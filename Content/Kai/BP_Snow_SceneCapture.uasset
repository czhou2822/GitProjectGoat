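; Scene capture actor for a snow depth effect, accumulating into a persistent render target, likely to record trails.
; On BeginPlay it sets the capture's ortho width from the Snow_Parameter collection, creates a Snow_ADDRTT dynamic material and clears both render targets to white.
; Each Tick draws that material into the second target without clearing, so results build up over time.
; A ShowDepthMap debug widget is left unconnected.
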(event EventBeginPlay
  (Utilities|FlowControl|Sequence
    (:then_1
      (bind _returnvalue (Rendering|Material|GetScalarParameterValue "/Game/Kai/Materials/Snow_Parameter.Snow_Parameter" "CaptureWidth" :!class /Script/Engine.KismetMaterialLibrary))
      (Variables|/Script/Engine.SceneCaptureComponent2D|SetOrthoWidth (Variables|DecalActor|GetCaptureComponent2D) _returnvalue)
      (bind _returnvalue_2 (Rendering|Material|CreateDynamicMaterialInstance "/Game/Kai/Materials/SnowDeformation/Snow_ADDRTT.Snow_ADDRTT" "None" :!class /Script/Engine.KismetMaterialLibrary))
      (Variables|Default|SetSnow_capture _returnvalue_2)
      (Rendering|ClearRenderTarget2D "/Game/Kai/Snow_Scene_Capture_RTT1.Snow_Scene_Capture_RTT1" "(R=1.000000,G=1.000000,B=1.000000,A=1.000000)")
      (Rendering|ClearRenderTarget2D "/Game/Kai/Snow_Scene_Capture_RTT2.Snow_Scene_Capture_RTT2" "(R=1.000000,G=1.000000,B=1.000000,A=1.000000)"))))

(event EventTick
  (params (DeltaSeconds :type Float%20%28single-precision%29))
  ;[1 1 1] draw to rt, doesn't clear the rtt
  (Rendering|DrawMaterialtoRenderTarget "/Game/Kai/Snow_Scene_Capture_RTT2.Snow_Scene_Capture_RTT2" (Variables|Default|GetSnow_capture)))

(fn ConstructionScript)