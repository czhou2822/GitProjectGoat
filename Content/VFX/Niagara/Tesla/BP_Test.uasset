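; Test actor for a Niagara effect in the Tesla VFX folder that steps the effect's endpoints along the X axis over time.
; A looping timer started at BeginPlay deactivates the Niagara component, writes the Start and End vector parameters, then reactivates it without a reset.
; Each stored vector advances by a fixed X offset after being written, so the next cycle uses the shifted position.
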(event Custom|CustomEvent_0
  (Components|Activation|Deactivate (Variables|Default|GetNiagara))
  (Niagara|SetNiagaraVariable(Vector3) (Variables|Default|GetNiagara) "Start" (Variables|Default|GetStart))
  (Variables|Default|SetStart (+ (Variables|Default|GetStart) "50.000000, 0, 0"))
  (Niagara|SetNiagaraVariable(Vector3) (Variables|Default|GetNiagara) "End" (Variables|Default|GetEnd))
  (Variables|Default|SetEnd (+ (Variables|Default|GetEnd) "50.000000, 0, 0"))
  (Components|Activation|Activate (Variables|Default|GetNiagara) false))

(event EventBeginPlay
  (Utilities|Time|SetTimerbyEvent (delegate Custom|CustomEvent_0) 0.5 true))

(event Collision|EventActorBeginOverlap
  (params (OtherActor :type Actor%20Object%20Reference)))

(event EventTick
  (params (DeltaSeconds :type Float%20%28single-precision%29)))

(fn ConstructionScript)