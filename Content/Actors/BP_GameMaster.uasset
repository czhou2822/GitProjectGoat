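; Game master actor that runs the match loop of timed collecting phases alternating with enemy waves.
; A looping timer ends each collecting phase, then a data table row sets the next wave and the spawn points it uses.
; Spawn point completion events record durations for waves 1–5 and restart collecting.
; Reaching the player inventory's bulk target opens the end level; a base explosion or missing wave row opens the fail level.
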(event BaseExploded(BaseObject)
  (CallFunction|EndGameFailed))

(event Custom|BindOnCollectingPhaseComplete
  ;[1 1 1] DataBinding
  (CallFunction|HandleonCollectingPhaseComplete))

(event Custom|BindOnBulkChanged
  (params (CurrentBulkCount :type Integer))
  (CallFunction|HandleonBulkChanged CurrentBulkCount))

(event Custom|BindOnWaveComplete
  ;[1 1 1] DataBinding
  (CallFunction|HandleonWaveComplete))

(event EventBeginPlay
  (Utilities|FlowControl|Sequence
    (:then_0
      ;[1 1 1] DataBinding
      (bind _result (Utilities|Set|ToArray (Variables|Spawn|GetSpawnPointsArray)))
      (for _array_element _result
        (Utilities|IsValid _array_element
          (:Is%20Valid
            (EventDispatchers|BindEventtoOnWaveComplete _array_element (delegate Custom|BindOnWaveComplete))
            (EventDispatchers|AssignOnCollectingPhaseComplete (delegate Custom|BindOnCollectingPhaseComplete)))))
      (bind _asbp_player_character (Utilities|Casting|CastToBP_PlayerCharacter (Game|GetPlayerCharacter 0)))
      (bind _output_get (Variables|Gameplay|SetPlayerCharacter _asbp_player_character))
      (EventDispatchers|AssignOnBulkChanged (Variables|/Script/ProjectGoat.TPSCharacterQ|GetInventoryComp _output_get) (delegate Custom|BindOnBulkChanged))
      (Variables|Gameplay|SetBulkCountString (Utilities|String|Append "BulkCount:  0/" (Utilities|String|ToString(Integer) (Variables|Gameplay|GetBulkTarget)))))
    (:then_2
      (if (Variables|Spawn|GetIsSpawning)
        (CallFunction|StartCollectionPhase)))))

(fn ConstructionScript)

(fn HandleonWaveComplete
  (bind _returnvalue (Math|DateTime|Now))
  (bind _wavebegindate (Variables|Spawn|GetWaveBeginDate))
  (bind _returnvalue_2 (- _returnvalue _wavebegindate))
  (bind _returnvalue_3 (Utilities|String|ToString(Integer) (.minutes _returnvalue_2)))
  (bind _returnvalue_4 (Utilities|String|ToString(Integer) (.seconds _returnvalue_2)))
  (bind _returnvalue_5 (Utilities|String|Append _returnvalue_3 ":" _returnvalue_4))
  (Development|PrintString "WaveComplete")
  (switch int (.WaveNumber (Utilities|Struct|BreakWaveStructData (Variables|Spawn|GetCurrentWaveStat)))
    (:1
      (Variables|WaveTimer|SetFirstTime_1 _returnvalue_5))
    (:2
      (Variables|WaveTimer|SetFirstTime_2 _returnvalue_5))
    (:3
      (Variables|WaveTimer|SetFirstTime_3 _returnvalue_5))
    (:4
      (Variables|WaveTimer|SetFirstTime_4 _returnvalue_5))
    (:5
      (Variables|WaveTimer|SetFirstTime_5 _returnvalue_5)))
  (CallFunction|StartCollectionPhase))

(fn HandleonCollectingPhaseComplete
  (if (Variables|Gameplay|GetisGameEnd)
    (CallFunction|EndGameSuccess)
    (else
      (bind _result (Math|Integer|IncrementInt (Variables|Spawn|GetWaveCounter))
        (:%20%20
          (CallFunction|StartWave _result))))))

(fn HandleonBulkChanged
  (params (InBulkCount :type Integer))
  (Variables|Gameplay|SetBulkCountString (Utilities|String|Append "BulkCount: " (Utilities|String|ToString(Integer) InBulkCount) "/" (Utilities|String|ToString(Integer) (Variables|Gameplay|GetBulkTarget))))
  (if (>= InBulkCount (Variables|Gameplay|GetBulkTarget))
    (CallFunction|EndGameSuccess)))

(fn CollectingPhaseTick
  (if (> (Variables|Spawn|GetCollectingPhaseTickCount) 0.0)
    (Math|Float|DecrementFloat (Variables|Spawn|GetCollectingPhaseTickCount))
    (else
      (Default|CallOnCollectingPhaseComplete)
      (Development|PrintString "Collecting Phase complete")
      (Utilities|Time|ClearandInvalidateTimerbyHandle (Variables|Spawn|GetCollectingPhaseTimerHandler)))))

(fn EndGameSuccess
  (Development|PrintString "Thanks for playing" true true "(R=1.000000,G=0.000000,B=0.008526,A=1.000000)" 3e+01)
  (Game|OpenLevel(byName) "EndGameLevel"))

(fn SetWaveStat
  (params (InWaveNumber :type Name))
  (Development|PrintString (Utilities|String|Append "WaveNumber: " (Utilities|String|ToString(Name) InWaveNumber)))
  (bind _returnvalue (Utilities|GetDataTableRow "/Game/DataTable/DataTable_WaveStruct.DataTable_WaveStruct" InWaveNumber)
    (:then
      (bind _output_get (Variables|Spawn|SetCurrentWaveStat _returnvalue))
      (return _output_get))
    (:RowNotFound
      (Development|PrintString "Wave Number Not Found")
      (CallFunction|EndGameFailed))))

(fn StartWave
  (params (WaveNumber :type Integer))
  (bind _output (CallFunction|SetWaveStat (Utilities|String|StringToName (Utilities|String|ToString(Integer) WaveNumber))))
  (bind _stringoutput (CallFunction|StruttoString _output))
  (Development|PrintString _stringoutput)
  (bind _output_2 (CallFunction|ParseRouteNumbers (Variables|Spawn|GetCurrentWaveStat)))
  (for _array_element _output_2
    (bind _output_3 (CallFunction|SetActiveWaveSpawnPoint _array_element))
    (Default|SpawnWave _output_3 (Variables|Spawn|GetSpawnSingleEnemyInterval) (Variables|Spawn|GetCurrentWaveStat)))
  (Variables|Spawn|SetWaveBeginDate (Math|DateTime|Now)))

(fn IsGameEnded
  (Variables|Gameplay|SetisGameEnd (== (Variables|/Script/ProjectGoat.InventoryComponent|GetBulkCount (Actor|GetComponentbyClass (Variables|Gameplay|GetPlayerCharacter) "/Script/ProjectGoat.InventoryComponent")) (Variables|Gameplay|GetBulkTarget)))
  (return))

(fn StruttoString
  (params (InStruct :type Wave%20Struct%20Data%20Structure))
  (bind (_wavenumber _gruntnumber _gruntid _reavernumber _reaverid _minibossnumber _minibossid _routenumber) (Utilities|Struct|BreakWaveStructData InStruct))
  (return (Utilities|String|Append (Utilities|String|Append (Utilities|String|Append "Number: " (Utilities|String|ToString(Integer) _wavenumber)) (Utilities|String|Append " Enemy Count: " (Utilities|String|ToString(Integer) _gruntnumber))) (Utilities|String|Append "Route number: " _routenumber))))

(fn StartCollectionPhase
  (Variables|Spawn|SetCollectingPhaseTickCount (/ (Variables|Spawn|GetCollectingPhaseInSecond) (Variables|Spawn|GetCollectingPhaseTickInterval)))
  (bind _returnvalue (Utilities|Time|SetTimerbyFunctionName 0 "CollectingPhaseTick" (Variables|Spawn|GetCollectingPhaseTickInterval) true))
  (Variables|Spawn|SetCollectingPhaseTimerHandler _returnvalue))

(fn EndGameFailed
  (Game|OpenLevel(byName) "FailLevel"))

(fn ParseRouteNumbers
  (params (InWave :type Wave%20Struct%20Data%20Structure))
  (CallFunction|StruttoString InWave)
  (for _array_element (Utilities|String|ParseIntoArray (.RouteNumber (Utilities|Struct|BreakWaveStructData InWave)) ",")
    (bind _returnvalue (Utilities|Array|Add (LocalVariables|GetRouteNumber) (Math|Conversions|ToInteger(Byte) _array_element)))
    (Development|PrintString (Utilities|String|ToString(Integer) _returnvalue)))
  (return (LocalVariables|GetRouteNumber)))

(fn SetActiveWaveSpawnPoint
  (params (SpawnPointIndex :type Integer))
  (bind _result (Utilities|Set|ToArray (Variables|Spawn|GetSpawnPointsArray)))
  (return (Utilities|Array|Get(acopy) _result SpawnPointIndex)))