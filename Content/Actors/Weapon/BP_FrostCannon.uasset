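; Prototype frost cannon weapon that spends the player's snow to slow enemies in its line of fire.
; Tick stretches and rotates a capsule from the fire point toward a camera-forward point at weapon range.
; Firing enables the capsule, whose overlaps maintain FrostList, and calls SlowDown on listed enemies; release disables it.
; Aiming toggles AimBox, but its air-strike marking handlers are disconnected.
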(event OnComponentBeginOverlap(AimBox)
  (params (OverlappedComponent :type Primitive%20Component%20Object%20Reference) (OtherActor :type Actor%20Object%20Reference) (OtherComp :type Primitive%20Component%20Object%20Reference) (OtherBodyIndex :type Integer) (bFromSweep :type Boolean) (SweepResult :type Hit%20Result%20Structure%20%28by%20ref%29))
  ;[1 1 1] AirStrikeBox
)

(event OnComponentEndOverlap(AimBox)
  (params (OverlappedComponent :type Primitive%20Component%20Object%20Reference) (OtherActor :type Actor%20Object%20Reference) (OtherComp :type Primitive%20Component%20Object%20Reference) (OtherBodyIndex :type Integer))
  ;[1 1 1] AirStrikeBox
)

(event OnComponentBeginOverlap(FrostHitCapsule)
  (params (OverlappedComponent :type Primitive%20Component%20Object%20Reference) (OtherActor :type Actor%20Object%20Reference) (OtherComp :type Primitive%20Component%20Object%20Reference) (OtherBodyIndex :type Integer) (bFromSweep :type Boolean) (SweepResult :type Hit%20Result%20Structure%20%28by%20ref%29))
  (bind _frostlist (Variables|Default|GetFrostList))
  ;[1 1 1] Frost cannon overlap
  (bind _asbp_enemy_base (Utilities|Casting|CastToBP_EnemyBase OtherActor))
  (Utilities|Set|Add _frostlist _asbp_enemy_base)
  (Development|PrintString (Utilities|String|ToString(Integer) (Utilities|Set|Length _frostlist)) false false "(R=0.000000,G=0.660000,B=1.000000,A=1.000000)" 0.0))

(event OnComponentEndOverlap(FrostHitCapsule)
  (params (OverlappedComponent :type Primitive%20Component%20Object%20Reference) (OtherActor :type Actor%20Object%20Reference) (OtherComp :type Primitive%20Component%20Object%20Reference) (OtherBodyIndex :type Integer))
  (bind _frostlist (Variables|Default|GetFrostList))
  ;[1 1 1] Frost cannon overlap
  (bind _asbp_enemy_base (Utilities|Casting|CastToBP_EnemyBase OtherActor))
  (Utilities|Set|Remove _frostlist _asbp_enemy_base)
  (Development|PrintString (Utilities|String|ToString(Integer) (Utilities|Set|Length _frostlist)) false false "(R=0.000000,G=0.660000,B=1.000000,A=1.000000)" 0.0))

(event EventBeginPlay
  (bind _frosthitcapsule (Variables|Default|GetFrostHitCapsule))
  (Utilities|FlowControl|Sequence
    (:then_0
      (Collision|SetCollisionResponsetoChannel _frosthitcapsule "ECC_GameTraceChannel9" "ECR_Ignore")
      (Variables|Default|SetDrawDebugCapsule false))
    (:then_1
      (Rendering|SetVisibility _frosthitcapsule (Variables|Default|GetDrawDebugCapsule) false))))

(event EventTick
  (params (DeltaSeconds :type Float%20%28single-precision%29))
  (bind _returnvalue (Game|GetPlayerCameraManager 0))
  (bind _firepoint (Variables|Default|GetFirePoint))
  (bind _returnvalue_2 (Transformation|GetWorldLocation _firepoint))
  (Utilities|FlowControl|Sequence
    (:then_0
      (Development|PrintString (Utilities|String|ToString(Vector) _returnvalue_2) false false)
      (Variables|Default|SetfireStartPoint _returnvalue_2)
      (Variables|Default|SetfireEndPoint (+ (* (Math|Vector|GetForwardVector (Variables|/Script/Engine.Actor|GetRootComponent _returnvalue)) (Variables|Default|GetWeaponRange)) (Camera|GetCameraLocation _returnvalue) "")))
    (:then_1
      (bind _output_get (Variables|Default|Sethalfheight (/ (- (Math|Vector|Distance(Vector) (Variables|Default|GetfireStartPoint) (Variables|Default|GetfireEndPoint)) 0.0) 2.0)))
      (Components|Capsule|SetCapsuleSize (Variables|Default|GetFrostHitCapsule) (Variables|Default|GetCapsuleRadius) (* (Variables|Default|Gethalfheight) 1.0) true)
      (Transformation|SetWorldLocation (Variables|Default|GetFrostHitCapsule) (/ (+ (Variables|Default|GetfireStartPoint) (Variables|Default|GetfireEndPoint)) 2) true false)
      (Transformation|SetWorldRotation (Variables|Default|GetFrostHitCapsule) (Math|Rotator|MakeRotator (.Roll (Math|Rotator|BreakRotator (Math|Rotator|FindLookatRotation (Variables|Default|GetfireStartPoint) (Variables|Default|GetfireEndPoint)))) (+ (.Pitch (Math|Rotator|BreakRotator (Math|Rotator|FindLookatRotation (Variables|Default|GetfireStartPoint) (Variables|Default|GetfireEndPoint)))) 9e+01) (.Yaw (Math|Rotator|BreakRotator (Math|Rotator|FindLookatRotation (Variables|Default|GetfireStartPoint) (Variables|Default|GetfireEndPoint))))) false false))))

(event EventOnAimUp
  ;[1 1 1] OnAim
  (Development|PrintString "Aim Up" false false)
  (Rendering|SetVisibility (Variables|Default|GetAimBox) true false)
  (Collision|SetCollisionResponsetoChannel (Variables|Default|GetAimBox) "ECC_GameTraceChannel9" "ECR_Overlap"))

(event EventOnAimDown
  ;[1 1 1] OnAim
  (Development|PrintString "Aim Down" false false)
  (Rendering|SetVisibility (Variables|Default|GetAimBox) false false)
  (Collision|SetCollisionResponsetoChannel (Variables|Default|GetAimBox) "ECC_GameTraceChannel9" "ECR_Ignore"))

(event EventOnFireStart
  (bind _frosthitcapsule (Variables|Default|GetFrostHitCapsule))
  (bind _astpscharacter_q (Utilities|Casting|CastToTPSCharacterQ (Game|Player|GetPlayerPawn 0)))
  ;[1 1 1] Frost Canon prototype
  (if (> (Variables|/Script/ProjectGoat.TPSCharacterQ|GetsnowCount _astpscharacter_q) 0.0)
    (Utilities|FlowControl|Sequence
      (:then_0
        (Collision|SetCollisionResponsetoChannel _frosthitcapsule "ECC_GameTraceChannel9" "ECR_Overlap")
        (Variables|Default|SetDrawDebugCapsule true))
      (:then_1
        (Rendering|SetVisibility _frosthitcapsule (Variables|Default|GetDrawDebugCapsule) false))
      (:then_2
        (bind _astpscharacter_q_2 (Utilities|Casting|CastToTPSCharacterQ (Game|Player|GetPlayerPawn 0)))
        (Variables|/Script/ProjectGoat.TPSCharacterQ|SetsnowCount _astpscharacter_q_2 (- (Variables|/Script/ProjectGoat.TPSCharacterQ|GetsnowCount _astpscharacter_q_2) 0.5))
        (Audio|PlaySoundatLocation (Variables|Default|GetFireSound) (Transformation|GetActorLocation) "0, 0, 0" 0.2 1.0 0.0 0 0 0))
      (:then_3
        (CallFunction|SlowEnemies)))))

(event EventOnFireEnd
  (bind _frosthitcapsule (Variables|Default|GetFrostHitCapsule))
  (Utilities|FlowControl|Sequence
    (:then_0
      (Collision|SetCollisionResponsetoChannel _frosthitcapsule "ECC_GameTraceChannel9" "ECR_Ignore")
      (Variables|Default|SetDrawDebugCapsule false))
    (:then_1
      (Rendering|SetVisibility _frosthitcapsule (Variables|Default|GetDrawDebugCapsule) false))))

(fn ConstructionScript)

(fn SlowEnemies
  (if (> (Utilities|Set|Length (Variables|Default|GetFrostList)) 0)
    (bind _result (Utilities|Set|ToArray (Variables|Default|GetFrostList)))
    (for _array_element _result
      (Class|EnemyBase|SlowDown _array_element))))

(fn HandleAimBeginOverlap
  (params (InOverlappedEnemy :type Object%20Object%20Reference))
  (bind _airstrikelist (Variables|Default|GetAirStrikeList))
  (bind _asbp_player_character (Utilities|Casting|CastToBP_PlayerCharacter (Game|GetPlayerCharacter 0)))
  (if (> (Variables|/Game/Actors/PlayerCharacter/BP_PlayerCharacter.BP_PlayerCharacter_C|GetMissileCount _asbp_player_character) (Utilities|Set|Length (Variables|Default|GetAirStrikeList)))
    (bind _asbp_enemy_base (Utilities|Casting|CastToBP_EnemyBase InOverlappedEnemy))
    (bind _output_get (LocalVariables|SetOverlappedEnemy _asbp_enemy_base))
    (Utilities|Set|Add _airstrikelist _output_get)
    (Development|PrintString (Utilities|String|ToString(Integer) (Utilities|Set|Length _airstrikelist)) false false)
    (Development|PrintString (Utilities|String|Append (Utilities|GetDisplayName (LocalVariables|GetOverlappedEnemy)) " overlapped") false false)
    (bind _output_get_2 (Variables|/Game/Actors/Enemy/EnemyBase/BP_EnemyBase.BP_EnemyBase_C|SetIsMark (LocalVariables|GetOverlappedEnemy) true))
    (Default|OnMarkedEvent (LocalVariables|GetOverlappedEnemy) _output_get_2)))

(fn HandleAimEndOverlap
  (params (ExitedObject :type Object%20Object%20Reference))
  (bind _airstrikelist (Variables|Default|GetAirStrikeList))
  (bind _asbp_enemy_base (Utilities|Casting|CastToBP_EnemyBase ExitedObject))
  (bind _output_get (LocalVariables|SetExitedEnemy _asbp_enemy_base))
  (Utilities|Set|Remove _airstrikelist _output_get)
  (Development|PrintString (Utilities|String|ToString(Integer) (Utilities|Set|Length _airstrikelist)) false false)
  (Development|PrintString (Utilities|String|Append (Utilities|GetDisplayName ExitedObject) " exits ") false false)
  (bind _output_get_2 (Variables|/Game/Actors/Enemy/EnemyBase/BP_EnemyBase.BP_EnemyBase_C|SetIsMark (LocalVariables|GetExitedEnemy) false))
  (Default|OnMarkedEvent (LocalVariables|GetExitedEnemy) _output_get_2))