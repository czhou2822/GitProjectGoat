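; Grenade-launching tower that turns toward its target and fires grenade projectiles.
; Tick calls TurnTo while TargetActor is valid, and FireEvent calls FireGrenade.
; FireGrenade spawns a BP_Grenade at FirePoint aimed at TargetLocation, passes it TowerDamage and plays the fire sound at the mesh.
; A direct DealDamage call on the target's HealthComponent remains in the graph unconnected, so this tower deals no damage itself.
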(event EventBeginPlay
  (|CallParentFunction) ; This node is disabled and will not be called.\nDrag off pins to build functionality.
)

(event Collision|EventActorBeginOverlap
  (params (OtherActor :type Actor%20Object%20Reference)))

(event EventTick
  (params (DeltaSeconds :type Float%20%28single-precision%29))
  (|CallParentFunction DeltaSeconds)
  (Utilities|IsValid (Variables|Default|GetTargetActor)
    (:Is%20Valid
      (CallFunction|Turnto DeltaSeconds))))

(event EventFireEvent
  (CallFunction|FireGrenade))

(fn ConstructionScript
  (|CallParentFunction))

(fn FireGrenade
  (bind _firepoint (Variables|Default|GetFirePoint))
  (bind _returnvalue (Game|SpawnActorfromClass "/Game/Actors/Tower/Projectiles/BP_Grenade.BP_Grenade_C" (Math|Transform|MakeTransform _firepoint (Math|Rotator|FindLookatRotation _firepoint (Variables|Default|GetTargetLocation))) "Undefined" 0 0))
  (Variables|/Game/Actors/Tower/Projectiles/BP_ProjectileBase.BP_ProjectileBase_C|SetProjectileDamage _returnvalue (Variables|Default|GetTowerDamage))
  (Audio|PlaySoundatLocation (Variables|Default|GetFireSound) (Transformation|GetWorldLocation (Variables|Character|GetMesh)) "0, 0, 0" 0.2 1.0 0.0 0 0 0))