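; Tower homing missile that deals radial falloff damage when it explodes on overlapping an enemy.
; Tick waits until upward velocity nearly runs out, then switches ProjectileMovement to home on the target's HomingPoint.
; Without a valid target at BeginPlay, it explodes after a delay.
; SetDamageParameter configures damage, radii and delays, though TriggerDelay is only stored; Explode also draws a debug sphere.
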(event OnComponentBeginOverlap(TriggerSphere)
  (params (OverlappedComponent :type Primitive%20Component%20Object%20Reference) (OtherActor :type Actor%20Object%20Reference) (OtherComp :type Primitive%20Component%20Object%20Reference) (OtherBodyIndex :type Integer) (bFromSweep :type Boolean) (SweepResult :type Hit%20Result%20Structure%20%28by%20ref%29))
  (Utilities|Casting|CastToBP_EnemyBase OtherActor)
  (CallFunction|Explode))

(event OnComponentBeginOverlap(TriggerRadius)
  (params (OverlappedComponent :type Primitive%20Component%20Object%20Reference) (OtherActor :type Actor%20Object%20Reference) (OtherComp :type Primitive%20Component%20Object%20Reference) (OtherBodyIndex :type Integer) (bFromSweep :type Boolean) (SweepResult :type Hit%20Result%20Structure%20%28by%20ref%29))
  (Utilities|Casting|CastToBP_EnemyBase OtherActor)
  (CallFunction|Explode)
  (Development|PrintString "exploded"))

(event EventBeginPlay
  (Utilities|IsValid (Variables|Default|GetTargetEnemy)
    (:Is%20Not%20Valid
      (Development|PrintString "Target Not valid")
      (Utilities|FlowControl|Delay (Variables|Default|GetExplosionDelay))
      (CallFunction|Explode))))

(event EventTick
  (params (DeltaSeconds :type Float%20%28single-precision%29))
  (bind _mesh (Variables|Character|GetMesh))
  (bind _projectilemovement (Variables|Default|GetProjectileMovement))
  (bind _targetenemy (Variables|Default|GetTargetEnemy))
  (bind _returnvalue (Transformation|GetComponentVelocity _mesh))
  (bind _homingpoint (Variables|/Script/ProjectGoat.BulkheadCharacterBase|GetHomingPoint _targetenemy))
  (Utilities|IsValid (Variables|Default|GetTargetEnemy)
    (:Is%20Valid
      (if (not (Variables|/Script/Engine.ProjectileMovementComponent|GetbIsHomingProjectile (Variables|Default|GetProjectileMovement)))
        (if (and (<= (.z _returnvalue) 2e+01) (> (.z _returnvalue) 0.0))
          (Development|PrintString (Utilities|String|ToString(Float) (.z _returnvalue)))
          (Utilities|IsValid _homingpoint
            (:Is%20Valid
              (Variables|/Script/Engine.ProjectileMovementComponent|SetHomingTargetComponent _projectilemovement _homingpoint)
              (Variables|/Script/Engine.ProjectileMovementComponent|SetbRotationFollowsVelocity _projectilemovement true)
              (Variables|/Script/Engine.ProjectileMovementComponent|SetbIsHomingProjectile _projectilemovement true)
              (Variables|/Script/Engine.ProjectileMovementComponent|SetHomingAccelerationMagnitude _projectilemovement 1.5e+04))
            (:Is%20Not%20Valid
              (Development|PrintString "homing target not valid"))))))))

(fn ConstructionScript
  (if (== (Variables|Default|GetExplosiveRange) 0.0)
    (Variables|Default|SetExplosiveRange (Variables|/Script/Engine.SphereComponent|GetSphereRadius (Variables|Default|GetCollisionExplosiveRange)))))

(fn Explode
  (Class|GameplayStatics|ApplyRadialDamagewithFalloff (Variables|Default|GetProjectileDamage) 0.0 (Transformation|GetActorLocation) (Variables|/Script/Engine.SphereComponent|GetSphereRadius (Variables|Default|GetTriggerRadius)) (Variables|Default|GetExplosiveRange) 0.0 0 0 0 0 "ECC_Visibility")
  (Rendering|Debug|DrawDebugSphere (Transformation|GetActorLocation) (Variables|Default|GetExplosiveRange) 12 "(R=1.000000,G=1.000000,B=1.000000,A=1.000000)" 2.0 3.0)
  (Actor|DestroyActor))

(fn SetDamageParameter
  (params (InDamage :type Float%20%28single-precision%29) (InTriggerRange :type Float%20%28single-precision%29) (InExplosiveRange :type Float%20%28single-precision%29) (InExplosionDelay :type Float%20%28single-precision%29) (InTriggerDelay :type Float%20%28single-precision%29))
  (Utilities|FlowControl|Sequence
    (:then_0
      (Variables|Default|SetProjectileDamage InDamage))
    (:then_1
      (Components|Sphere|SetSphereRadius (Variables|Default|GetTriggerRadius) InTriggerRange true))
    (:then_2
      (Variables|Default|SetExplosiveRange InExplosiveRange))
    (:then_3
      (Variables|Default|SetExplosionDelay InExplosionDelay))
    (:then_4
      (Variables|Default|SetTriggerDelay InTriggerDelay))))