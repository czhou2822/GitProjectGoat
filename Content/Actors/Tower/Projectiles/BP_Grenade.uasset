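; Tower grenade projectile that deals radial damage on a timer or when an enemy comes close.
; Explode runs after a fixed delay from BeginPlay, or shortly after a BP_EnemyBase overlaps the trigger sphere.
; SetDamageParameter sets damage, radii and delay variables, though both delays in the event graph are hard-coded.
; Explode only applies damage; the per-target damage, effects and DestroyActor logic is disconnected.
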(event OnComponentBeginOverlap(TriggerRadius)
  (params (OverlappedComponent :type Primitive%20Component%20Object%20Reference) (OtherActor :type Actor%20Object%20Reference) (OtherComp :type Primitive%20Component%20Object%20Reference) (OtherBodyIndex :type Integer) (bFromSweep :type Boolean) (SweepResult :type Hit%20Result%20Structure%20%28by%20ref%29))
  (Utilities|FlowControl|Delay 0.2)
  (Utilities|Casting|CastToBP_EnemyBase OtherActor)
  (CallFunction|Explode))

(event EventBeginPlay
  (|CallParentFunction)
  (Utilities|FlowControl|Delay 3.0)
  (CallFunction|Explode))

(event Collision|EventActorBeginOverlap
  (params (OtherActor :type Actor%20Object%20Reference))
  (|CallParentFunction OtherActor) ; This node is disabled and will not be called.\nDrag off pins to build functionality.
)

(event EventTick
  (params (DeltaSeconds :type Float%20%28single-precision%29))
  (|CallParentFunction DeltaSeconds))

(fn ConstructionScript
  (|CallParentFunction))

(fn Explode
  (Game|Damage|ApplyRadialDamage (Variables|Default|GetGrenadeDamage) (Transformation|GetActorLocation) (Variables|Default|GetExplosiveRange) 0 0 0 0 false "ECC_Visibility"))

(fn SetDamageParameter
  (params (InDamage :type Float%20%28single-precision%29) (InTriggerRange :type Float%20%28single-precision%29) (InExplosiveRange :type Float%20%28single-precision%29) (InExplosionDelay :type Float%20%28single-precision%29) (InTriggerDelay :type Float%20%28single-precision%29))
  (Utilities|FlowControl|Sequence
    (:then_0
      (Variables|Default|SetGrenadeDamage InDamage))
    (:then_1
      (Components|Sphere|SetSphereRadius (Variables|Default|GetTriggerRadius) InTriggerRange true))
    (:then_2
      (Variables|Default|SetExplosiveRange InExplosiveRange))
    (:then_3
      (Variables|Default|SetExplosionDelay InExplosionDelay))
    (:then_4
      (Variables|Default|SetTriggerDelay InTriggerDelay))))