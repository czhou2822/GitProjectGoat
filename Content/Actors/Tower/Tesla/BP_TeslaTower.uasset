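; BP_TeslaTower is a Tesla tower that damages a target actor, built on a parent class.
; The construction script sets TowerDamage from the Attack value in its character data.
; FireEvent passes that damage to Attack on the current target.
; While a target is valid, Tick draws a blue debug line from the fire point to the target as the beam visual.
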(event EventBeginPlay
  (|CallParentFunction))

(event Collision|EventActorBeginOverlap
  (params (OtherActor :type Actor%20Object%20Reference))
  (|CallParentFunction OtherActor) ; This node is disabled and will not be called.\nDrag off pins to build functionality.
)

(event EventTick
  (params (DeltaSeconds :type Float%20%28single-precision%29))
  (|CallParentFunction DeltaSeconds)
  (Utilities|IsValid (Variables|Default|GetTargetActor)
    (:Is%20Valid
      (Rendering|Debug|DrawDebugLine (Variables|Default|GetFirePoint) (Variables|Default|GetTargetLocation) "(R=0.000000,G=0.132017,B=1.000000,A=1.000000)" 0.0 3.0))))

(event EventFireEvent
  (bind _towerdamage (Variables|Default|GetTowerDamage))
  (Development|PrintString (Utilities|String|ToString(Float) _towerdamage) false false)
  (Class|BulkheadCharacterBase|Attack self (Variables|Default|GetTargetActor) _towerdamage))

(fn ConstructionScript
  (|CallParentFunction)
  (bind _returnvalue (Class|BulkheadCharacterBase|GetCharacterData))
  (Variables|Default|SetTowerDamage (.attack _returnvalue)))