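; Gatling tower Blueprint that tracks and attacks a target, building on a parent class.
; Each tick it lerps the anim instance's DoomRotation toward the yaw from FireSocket to the target, using TurnSpeed as a fixed alpha independent of frame time.
; FireEvent applies TowerDamage to the target through Attack and draws a brief debug line from FirePoint to the target location as the shot.
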(event EventTick
  (params (DeltaSeconds :type Float%20%28single-precision%29))
  (|CallParentFunction DeltaSeconds)
  (Utilities|FlowControl|Sequence
    (:then_1
      (CallFunction|Turnto 0.0))))

(event EventFireEvent
  (bind _towerdamage (Variables|Default|GetTowerDamage))
  (Development|PrintString (Utilities|String|ToString(Float) _towerdamage) false false "(R=0.000000,G=0.660000,B=1.000000,A=1.000000)" 0.3)
  (Class|BulkheadCharacterBase|Attack self (Variables|Default|GetTargetActor) _towerdamage)
  (Rendering|Debug|DrawDebugLine (Variables|Default|GetFirePoint) (Variables|Default|GetTargetLocation) "(R=0.000000,G=0.132017,B=1.000000,A=1.000000)" 0.05 3.0))

(fn ConstructionScript
  (|CallParentFunction))

(fn Turnto
  (params (DeltaTime :type Float%20%28single-precision%29))
  (Utilities|IsValid (Variables|Default|GetTargetActor)
    (:Is%20Valid
      (Utilities|IsValid (Variables|Default|GetAnimGatling)
        (:Is%20Valid
          (Variables|/Game/Actors/Tower/Gatling/Anim/ABP_GatlingTower.ABP_GatlingTower_C|SetDoomRotation (Variables|Default|GetAnimGatling) (Math|Rotator|Lerp(Rotator) (Variables|/Game/Actors/Tower/Gatling/Anim/ABP_GatlingTower.ABP_GatlingTower_C|GetDoomRotation (Variables|Default|GetAnimGatling)) (Math|Rotator|MakeRotator 0.0 0.0 (.Yaw (Math|Rotator|BreakRotator (Math|Rotator|FindLookatRotation (Transformation|GetSocketLocation (Variables|Character|GetMesh) "FireSocket") (Variables|Default|GetTargetLocation))))) (Variables|Default|GetTurnSpeed)))
          (Development|PrintString (Utilities|String|ToString(Rotator) (Variables|/Game/Actors/Tower/Gatling/Anim/ABP_GatlingTower.ABP_GatlingTower_C|GetDoomRotation (Variables|Default|GetAnimGatling))) false false))))
    (:Is%20Not%20Valid
      (Development|PrintString "no actor in range" false false "(R=0.000000,G=0.660000,B=1.000000,A=1.000000)" 0.0)
      (return))))