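; Air strike tower actor that registers with the game mode on construction completion, takes its damage from character data, and announces when a strike is ready.
; AirStrike spawns an upward-pitched homing missile at the FirePoint socket, passing it the target and damage.
; Tick runs terrain snapping.
; A timer-based cooldown countdown exists, but its reset and start code is disconnected, as is an older grenade spawn.
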(event Custom|HandleOnConstructionCompleted
  (bind _asbp_project_goat_game_mode (Utilities|Casting|CastToBP_ProjectGoatGameMode (Game|GetGameMode)))
  (Default|AddAirStrikeTower _asbp_project_goat_game_mode self)
  (bind _returnvalue (Class|BulkheadCharacterBase|GetCharacterData))
  (Variables|Default|SetTowerDamage (.attack _returnvalue)))

(event EventBeginPlay
  (|CallParentFunction)
  (Variables|Default|SetCooldownTickDefault (Math|Float|Truncate (/ (Variables|Default|GetCooldownInSecond) (Variables|Default|GetCooldownTickInterval))))
  (EventDispatchers|BindEventtoOnConstructionComplete (delegate Custom|HandleOnConstructionCompleted)))

(event EventOnConstructionCompleteEvent
  (CallFunction|AirStrikeReadyFunction self))

(event EventTick
  (params (DeltaSeconds :type Float%20%28single-precision%29))
  (CallFunction|TerrianSnapping))

(fn ConstructionScript
  (|CallParentFunction))

(fn AirStrikeReadyFunction
  (params (NewParam :type BP%20Air%20Strike%20Tower%20Object%20Reference))
  (Default|CallOnAirStrikeReady NewParam)
  (Utilities|Time|ClearandInvalidateTimerbyHandle (Variables|Default|GetAirStrikeTimer))
  (Development|PrintString "AirStrikeReady" false false))

(fn AirStrikeCooldownTick
  (if (== (Variables|Default|GetCooldownTick) 0)
    (CallFunction|AirStrikeReadyFunction self)
    (else
      (Math|Integer|DecrementInt (Variables|Default|GetCooldownTick)
        (:%20%20
          (return))))))

(fn AirStrike
  (params (Target :type BP%20Enemy%20Base%20Object%20Reference))
  (bind _mesh (Variables|Character|GetMesh))
  (bind _returnvalue (Transformation|GetSocketTransform _mesh "FirePoint" "RTS_World"))
  (bind (_location _rotation _scale) (Math|Transform|BreakTransform _returnvalue))
  (bind (_roll _pitch _yaw) (Math|Rotator|BreakRotator _rotation))
  (Development|PrintString (Utilities|String|Append (Utilities|GetDisplayName self) " air strikes " (Utilities|GetObjectName Target)) true true "(R=1.000000,G=0.000000,B=0.329775,A=1.000000)")
  (Variables|Default|SetTowerTarget Target)
  (bind _returnvalue_2 (Game|SpawnActorfromClass "/Game/John/Blueprints/BP_HomingMissile.BP_HomingMissile_C" (Math|Transform|MakeTransform _location (Math|Rotator|MakeRotator _roll 9e+01 _yaw) _scale) "AdjustIfPossibleButAlwaysSpawn" 0 0))
  (Variables|/Game/John/Blueprints/BP_HomingMissile.BP_HomingMissile_C|SetTargetEnemy _returnvalue_2 (Variables|Default|GetTowerTarget))
  (Variables|/Game/Actors/Tower/Projectiles/BP_ProjectileBase.BP_ProjectileBase_C|SetProjectileDamage _returnvalue_2 (Variables|Default|GetTowerDamage)))