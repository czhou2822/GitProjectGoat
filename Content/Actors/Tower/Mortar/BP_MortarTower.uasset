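; Mortar tower that fires explosive grenades at its target actor.
; Tick calls TurnTo while the target is valid; the override passes a zero delta time to the parent rather than the frame's.
; FireEvent spawns BP_Grenade at the fire point, gives it a spline path to the target plus damage and blast radius, and plays a fire sound.
; A direct-damage call on the target is left unconnected.
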(event EventBeginPlay
  (|CallParentFunction) ; This node is disabled and will not be called.\nDrag off pins to build functionality.
)

(event Collision|EventActorBeginOverlap
  (params (OtherActor :type Actor%20Object%20Reference)))

(event EventTick
  (params (DeltaSeconds :type Float%20%28single-precision%29))
  (|CallParentFunction DeltaSeconds)
  (Utilities|IsValid (Variables|Default|GetTargetActor)
    (:Is%20Valid
      (CallFunction|Turnto DeltaSeconds))))

(event EventFireEvent
  (CallFunction|FireGrenade))

(fn ConstructionScript
  (|CallParentFunction))

(fn FireGrenade
  (bind _firepoint (Variables|Default|GetFirePoint))
  (bind _returnvalue (Game|SpawnActorfromClass "/Game/Actors/Tower/Projectiles/BP_Grenade.BP_Grenade_C" (Math|Transform|MakeTransform _firepoint (Math|Rotator|FindLookatRotation _firepoint (Variables|Default|GetTargetLocation))) "Undefined" 0 0))
  (Default|SetTargetSplineLinePoints _returnvalue (Variables|Default|GetTargetActor) 5e+02)
  (Default|SetDamageParameter _returnvalue (Variables|Default|GetTowerDamage) 0.0 1e+03 0.0 0.3)
  (Audio|PlaySoundatLocation (Variables|Default|GetFireSound) (Transformation|GetWorldLocation (Variables|Character|GetMesh)) "0, 0, 0" 0.2 1.0 0.0 0 0 0))

(fn Turnto
  (params (DeltaTime :type Float%20%28single-precision%29))
  (|CallParentFunction 0.0))