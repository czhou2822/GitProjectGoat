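; Base tower actor that the player places, buys through the inventory and that fires at enemy targets.
; On placement it is destroyed if the purchase fails or it overlaps another tower; otherwise the anim instance plays construction.
; When construction completes it caches its AI controller and attack stat, then Tick copies the AI's target and broadcasts TowerFire on an interval.
; Debug shapes show padding and range; outline and terrain-snapping logic are disconnected.
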(event OnComponentBeginOverlap(TowerPadding)
  (params (OverlappedComponent :type Primitive%20Component%20Object%20Reference) (OtherActor :type Actor%20Object%20Reference) (OtherComp :type Primitive%20Component%20Object%20Reference) (OtherBodyIndex :type Integer) (bFromSweep :type Boolean) (SweepResult :type Hit%20Result%20Structure%20%28by%20ref%29))
  ;[1 1 1] CheckNearDistance
  (if (not (Variables|Default|GetIsPlaced))
    (bind _asbp_tower_base (Utilities|Casting|CastToBP_TowerBase OtherActor))
    (CallFunction|SetRedOutLine true)
    (Development|PrintString (Utilities|String|Append (Utilities|GetDisplayName _asbp_tower_base) " overlapped！"))
    (Utilities|Set|Add (Variables|Default|GetOverlappedTower) _asbp_tower_base)))

(event OnComponentEndOverlap(TowerPadding)
  (params (OverlappedComponent :type Primitive%20Component%20Object%20Reference) (OtherActor :type Actor%20Object%20Reference) (OtherComp :type Primitive%20Component%20Object%20Reference) (OtherBodyIndex :type Integer))
  ;[1 1 1] CheckNearDistance
  (bind _asbp_tower_base (Utilities|Casting|CastToBP_TowerBase OtherActor))
  (CallFunction|SetRedOutLine false)
  (Utilities|Set|Remove (Variables|Default|GetOverlappedTower) _asbp_tower_base)
  (Development|PrintString (Utilities|String|Append (Utilities|GetDisplayName _asbp_tower_base) " removed！")))

(event Custom|FireEvent
  ;[1 1 1] HookupAI and initialize
  ;;[1 1 1] If not collide, initilize
)

(event Custom|HandleOnConstructionComplete
  ;[1 1 1] HookupAI and initialize
  ;;[1 1 1] If not collide, initilize
  (CallFunction|TowerInit)
  (EventDispatchers|BindEventtoTowerFire (delegate Custom|FireEvent))
  (bind _asbp_player_character (Utilities|Casting|CastToBP_PlayerCharacter (Game|GetPlayerCharacter 0)))
  (EventDispatchers|BindEventtoOnCharacterStartPlacing _asbp_player_character (delegate Custom|HandleOnCharacterStartPlacing))
  (EventDispatchers|BindEventtoOnConstructionComplete (delegate Custom|OnConstructionComplete_Event))
  (Default|CallOnConstructionComplete))

(event Custom|OnConstructionComplete_Event
  ;[1 1 1] HookupAI and initialize
)

(event Custom|HandleOnCharacterStartPlacing
  (params (EnterPlacingMode :type Boolean))
  ;[1 1 1] HookupAI and initialize
  (Variables|Default|SetShowRange EnterPlacingMode))

(event Custom|HandleTowerPlacedEvent
  ;[1 1 1] Remember to reset to cast for player character base
  (EventDispatchers|UnbindEventfromOnTowerPlaced (stale EventBeginPlay _asbp_player_character) (delegate Custom|HandleTowerPlacedEvent))
  ;[1 1 1] HookupAI and initialize
  (bind _returnvalue (Class|InventoryComponent|PurchaseItem (Actor|GetComponentbyClass (Game|GetPlayerCharacter 0) "/Script/ProjectGoat.InventoryComponent") self))
  (if (and _returnvalue (== (Utilities|Set|Length (Variables|Default|GetOverlappedTower)) 0))
    (Utilities|IsValid (Variables|Default|GetAnimInstance)
      (:Is%20Valid
        ;;[1 1 1] If not collide, initilize
        (EventDispatchers|BindEventtoOnConstructionComplete (Variables|Default|GetAnimInstance) (delegate Custom|HandleOnConstructionComplete))
        (bind _output_get (Variables|Default|SetIsPlaced true))
        (Variables|/Game/Actors/Tower/TowerBase/ABP_TowerBase.ABP_TowerBase_C|SetisPlaced (Variables|Default|GetAnimInstance) _output_get))
      (:Is%20Not%20Valid
        (EventDispatchers|BindEventtoOnConstructionComplete (Variables|Default|GetAnimTesla) (delegate Custom|HandleOnConstructionComplete))
        (bind _output_get_2 (Variables|Default|SetIsPlaced true))
        (Variables|/Game/Actors/Tower/ABP_TeslaTower.ABP_TeslaTower_C|SetisPlaced (Variables|Default|GetAnimTesla) _output_get_2)))
    (else
      ;;[1 1 1] else, destroy
      (Actor|DestroyActor)
      (bind _result (Utilities|Set|ToArray (Variables|Default|GetOverlappedTower)))
      (for _array_element _result
        (Development|PrintString (Utilities|String|Append "overlap with " (Utilities|GetDisplayName _array_element)))))))

(event EventBeginPlay
  (bind _mesh (Variables|Character|GetMesh))
  (bind _returnvalue (Components|SkeletalMesh|GetAnimInstance _mesh))
  ;[1 1 1] Remember to reset to cast for player character base
  (bind _asbp_player_character (Utilities|Casting|CastToBP_PlayerCharacter (Game|GetPlayerCharacter 0)))
  (EventDispatchers|BindEventtoOnTowerPlaced _asbp_player_character (delegate Custom|HandleTowerPlacedEvent))
  (bind _asabp_tower_base (Utilities|Casting|CastToABP_TowerBase _returnvalue)
    (:then
      (Variables|Default|SetAnimInstance _asabp_tower_base))
    (:CastFailed
      (bind _asabp_tesla_tower (Utilities|Casting|CastToABP_TeslaTower _returnvalue))
      (Variables|Default|SetAnimTesla _asabp_tesla_tower))))

(event EventTick
  (params (DeltaSeconds :type Float%20%28single-precision%29))
  (Utilities|FlowControl|Sequence
    (:then_0
      ;[1 1 1] Tick
      (CallFunction|SetTargetActor))
    (:then_1
      (CallFunction|FireTimer (Variables|Default|GetNextFire)))
    (:then_2
      (|DrawTowerPadding))
    (:then_3
      (|DrawRange))
    (:then_4
      (CallFunction|TerrianSnapping))
    (:then_5
      (Variables|Default|SetFirePoint (Transformation|GetSocketLocation (Variables|Character|GetMesh) "FirePoint")))))

(fn ConstructionScript)

(fn SetTargetActor
  (bind _towerai (Variables|Default|GetTowerAI))
  (Utilities|IsValid _towerai
    (:Is%20Valid
      (Utilities|IsValid (Variables|/Game/Actors/Tower/TowerBase/AI_TowerBase.AI_TowerBase_C|GetTargetActor _towerai)
        (:Is%20Valid
          (bind _output_get (Variables|Default|SetTargetActor (Variables|/Game/Actors/Tower/TowerBase/AI_TowerBase.AI_TowerBase_C|GetTargetActor _towerai)))
          (Variables|Default|SetTargetLocation (Transformation|GetActorLocation _output_get)))))))

(fn Turnto
  (params (DeltaTime :type Float%20%28single-precision%29))
  (Utilities|IsValid (Variables|Default|GetTargetActor)
    (:Is%20Valid
      (Utilities|IsValid (Variables|Default|GetAnimInstance)
        (:Is%20Valid
          (Variables|/Game/Actors/Tower/TowerBase/ABP_TowerBase.ABP_TowerBase_C|SetDoomRotation (Variables|Default|GetAnimInstance) (Math|Rotator|Lerp(Rotator) (Variables|/Game/Actors/Tower/TowerBase/ABP_TowerBase.ABP_TowerBase_C|GetDoomRotation (Variables|Default|GetAnimInstance)) (Math|Rotator|MakeRotator 0.0 0.0 (.Yaw (Math|Rotator|BreakRotator (Math|Rotator|FindLookatRotation (Transformation|GetSocketLocation (Variables|Character|GetMesh) "FireSocket") (Variables|Default|GetTargetLocation))))) (Variables|Default|GetTurnSpeed))))))
    (:Is%20Not%20Valid
      (Development|PrintString "no actor in range" true true "(R=0.000000,G=0.660000,B=1.000000,A=1.000000)" 0.0)
      (return))))

(fn SetRedOutLine
  (params (isOutline :type Boolean)))

(fn TowerInit
  (bind _asai_tower_base (Utilities|Casting|CastToAI_TowerBase (Pawn|GetController)))
  (Variables|Default|SetTowerAI _asai_tower_base)
  (bind _returnvalue (Class|BulkheadCharacterBase|GetCharacterData))
  (Variables|Default|SetTowerDamage (.attack _returnvalue)))

(fn TerrianSnapping)

(fn FireTimer
  (params (B :type Float%20%28single-precision%29))
  (bind _returnvalue (Utilities|Time|GetGameTimeinSeconds))
  (if (> _returnvalue B)
    (Utilities|IsValid (Variables|Default|GetTargetActor)
      (:Is%20Valid
        (Default|CallTowerFire)
        (Variables|Default|SetNextFire (+ (Variables|Default|GetFireInterval) _returnvalue))))))