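; BP_Shop is a shop actor that the player uses by walking into its sphere trigger.
; When a BP_PlayerCharacter begins overlapping and is not placing a tower, it sets the character's IsInShop flag and enables the ApproximateMenu.
; Ending the overlap clears the flag and disables the menu, regardless of tower placement state.
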(event OnComponentBeginOverlap(Sphere)
  (params (OverlappedComponent :type Primitive%20Component%20Object%20Reference) (OtherActor :type Actor%20Object%20Reference) (OtherComp :type Primitive%20Component%20Object%20Reference) (OtherBodyIndex :type Integer) (bFromSweep :type Boolean) (SweepResult :type Hit%20Result%20Structure%20%28by%20ref%29))
  (bind _asbp_player_character (Utilities|Casting|CastToBP_PlayerCharacter OtherActor))
  (if (not (Variables|/Game/Actors/PlayerCharacter/BP_PlayerCharacter.BP_PlayerCharacter_C|GetIsCharacterPlacingTower _asbp_player_character))
    (Variables|/Game/Actors/PlayerCharacter/BP_PlayerCharacter.BP_PlayerCharacter_C|SetIsInShop _asbp_player_character true)
    (Default|Enable (Variables|Default|GetApproximateMenu))))

(event OnComponentEndOverlap(Sphere)
  (params (OverlappedComponent :type Primitive%20Component%20Object%20Reference) (OtherActor :type Actor%20Object%20Reference) (OtherComp :type Primitive%20Component%20Object%20Reference) (OtherBodyIndex :type Integer))
  (bind _asbp_player_character (Utilities|Casting|CastToBP_PlayerCharacter OtherActor))
  (Variables|/Game/Actors/PlayerCharacter/BP_PlayerCharacter.BP_PlayerCharacter_C|SetIsInShop _asbp_player_character false)
  (Default|Disable (Variables|Default|GetApproximateMenu)))

(fn ConstructionScript)