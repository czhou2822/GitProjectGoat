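; Base enemy Blueprint with health, an air-strike marking meter and a frozen visual effect.
; Health changes update a widget bar, and death from either the component or Bulkhead event spawns a coin and destroys the actor.
; A looping timer raises or decays the mark meter, adding the enemy to the GameMode's strike list when full.
; Slow events control a timeline for material snow; widget-facing and FrostCannon overlap logic are disconnected.
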(event OnComponentBeginOverlap(CapsuleComponent)
  (params (OverlappedComponent :type Primitive%20Component%20Object%20Reference) (OtherActor :type Actor%20Object%20Reference) (OtherComp :type Primitive%20Component%20Object%20Reference) (OtherBodyIndex :type Integer) (bFromSweep :type Boolean) (SweepResult :type Hit%20Result%20Structure%20%28by%20ref%29)))

(event OnHealthChange(HealthComponent)
  (bind _asumg_enemy_health (Utilities|Casting|CastToUMG_EnemyHealth (UserInterface|GetUserWidgetObject (Variables|Default|GetHealthWidget))))
  (Progress|SetPercent (Variables|/Game/Actors/Enemy/UMG_EnemyHealth.UMG_EnemyHealth_C|GetPG_HealthBar _asumg_enemy_health) (Variables|/Game/Actors/Components/HealthComponent.HealthComponent_C|GetHealthPercentage (Variables|Default|GetHealthComponent))))

(event OnComponentEndOverlap(CapsuleComponent)
  (params (OverlappedComponent :type Primitive%20Component%20Object%20Reference) (OtherActor :type Actor%20Object%20Reference) (OtherComp :type Primitive%20Component%20Object%20Reference) (OtherBodyIndex :type Integer)))

(event Custom|HandleOnCharacterDead
  (Game|SpawnActorfromClass "/Game/Actors/Misc/BP_Coin.BP_Coin_C" (Transformation|GetActorTransform) "Undefined" 0 0)
  (Actor|DestroyActor))

(event Custom|HandleOnBulkheadCharacterDead
  (Game|SpawnActorfromClass "/Game/Actors/Misc/BP_Coin.BP_Coin_C" (Transformation|GetActorTransform) "Undefined" 0 0)
  (Actor|DestroyActor))

(event Custom|OnMarked_Event
  (params (InMark :type Boolean))
  (if InMark
    (Rendering|SetVisibility (Variables|Default|GetMarkup) true false)
    (else
      (Rendering|SetVisibility (Variables|Default|GetMarkup) false false))))

(event EventBeginPlay
  (EventDispatchers|AssignOnCharacterDead (Variables|Default|GetHealthComponent) (delegate Custom|HandleOnCharacterDead))
  (EventDispatchers|BindEventtoOnBulkheadCharacterDead (delegate Custom|HandleOnBulkheadCharacterDead)))

(event EventTick
  (params (DeltaSeconds :type Float%20%28single-precision%29)))

(event EventOnSlowStart
  (Components|Timeline|PlayfromStart (Variables|Default|GetTimeline_Frozen)))

(event EventOnSlowEnd
  (Audio|Components|Audio|Stop (Variables|Default|GetTimeline_Frozen))
  (CallFunction|SetFrozenEffect 0.0)
  (Variables|Default|SetIsFrozen false))

(event EventOnFrozenStart
  (Variables|Default|SetIsFrozen true))

(fn ConstructionScript
  (Rendering|Material|SetScalarParameterValueonMaterials (Variables|Character|GetMesh) "SnowAmount" 0.0))

(fn SetDefaultHealth
  (params (InDefaultHealth :type Float%20%28single-precision%29))
  (bind _healthcomponent (Variables|Default|GetHealthComponent))
  (bind _output_get (Variables|/Game/Actors/Components/HealthComponent.HealthComponent_C|SetDefaultHealth _healthcomponent InDefaultHealth))
  (Variables|/Game/Actors/Components/HealthComponent.HealthComponent_C|SetHealth _healthcomponent _output_get))

(fn BeingAirStrikeAimed
  (Development|PrintString "I am being aimed"))

(fn StartMarking
  (params (Duration :type Float%20%28single-precision%29))
  (bind _asbp_project_goat_game_mode (Utilities|Casting|CastToBP_ProjectGoatGameMode (Game|GetGameMode)))
  (Math|Integer|IncrementInt (Variables|/Game/Actors/BP_BulkheadGameStates.BP_BulkheadGameStates_C|GetAimingCount (Variables|/Game/Actors/BP_ProjectGoatGameMode.BP_ProjectGoatGameMode_C|GetBulkheadGameState _asbp_project_goat_game_mode))
    (:%20%20
      (if (not (Variables|Default|GetHasMarked))
        (Rendering|SetVisibility (Variables|Default|GetMarkup) true false)
        (Variables|Default|SetMaxMarkCounter (* 60 Duration))
        (Development|PrintString "StartMakring" true true "(R=0.000000,G=0.660000,B=1.000000,A=1.000000)" 0.0)
        (bind _returnvalue (Utilities|Time|SetTimerbyFunctionName 0 "HandleMarking" 0.016667 true))
        (Variables|Default|SetMarkTimerHandle _returnvalue)))))

(fn HandleMarking
  (if (Variables|Default|GetIsBeingMarked)
    (LocalVariables|SetIncrement 1.0)
    (if (<= (+ (LocalVariables|GetIncrement) (Variables|Default|GetMarkCounter)) (* (Variables|Default|GetMaxMarkCounter) 1.5))
      (Variables|Default|SetMarkCounter (+ (LocalVariables|GetIncrement) (Variables|Default|GetMarkCounter)) :!label _label)
      (bind _output_get (Variables|Default|SetMarkMeter (/ (+ (LocalVariables|GetIncrement) (Variables|Default|GetMarkCounter)) (Variables|Default|GetMaxMarkCounter))))
      (Development|PrintString (Utilities|String|ToString(Float) _output_get) false false)
      (if (>= _output_get 1.0)
        (CallFunction|UpdateMarkMeter)
        (Variables|Default|SetHasMarked true)
        (bind _asbp_project_goat_game_mode (Utilities|Casting|CastToBP_ProjectGoatGameMode (Game|GetGameMode)))
        (Default|AddtoStrikeList _asbp_project_goat_game_mode self)
        (elif (<= _output_get 0.0)
          (CallFunction|EndMarking)
          (else
            (CallFunction|UpdateMarkMeter)))))
    (else
      (LocalVariables|SetIncrement -1.0)
      (goto _label))))

(fn EndMarking
  (bind _asbp_project_goat_game_mode (Utilities|Casting|CastToBP_ProjectGoatGameMode (Game|GetGameMode)))
  (Math|Integer|DecrementInt (Variables|/Game/Actors/BP_BulkheadGameStates.BP_BulkheadGameStates_C|GetAimingCount (Variables|/Game/Actors/BP_ProjectGoatGameMode.BP_ProjectGoatGameMode_C|GetBulkheadGameState _asbp_project_goat_game_mode))
    (:%20%20
      (Variables|Default|SetHasMarked false)
      (Variables|Default|SetMarkCounter 0.0)
      (Variables|Default|SetMarkMeter 0.0)
      (Rendering|SetVisibility (Variables|Default|GetMarkup) false false)
      (Utilities|Time|ClearandInvalidateTimerbyHandle (Variables|Default|GetMarkTimerHandle))
      (CallFunction|UpdateMarkMeter)
      (bind _asbp_project_goat_game_mode_2 (Utilities|Casting|CastToBP_ProjectGoatGameMode (Game|GetGameMode)))
      (Default|RemovefromStrikeList _asbp_project_goat_game_mode_2 self))))

(fn UpdateMarkMeter
  (if (== (Variables|Default|GetMarkMeter) 0.0)
    (Rendering|SetVisibility (Variables|Default|GetMarkup) false false)
    (else
      (Rendering|SetVisibility (Variables|Default|GetMarkup) true false)))
  (bind _asumg_markup (Utilities|Casting|CastToUMG_Markup (UserInterface|GetUserWidgetObject (Variables|Default|GetMarkup))))
  (Progress|SetPercent (Variables|/Game/Actors/Enemy/UMG_Markup.UMG_Markup_C|GetMarkUpProgressBar _asumg_markup) (Variables|Default|GetMarkMeter)))

(fn ResetMark
  (Variables|Default|SetHasMarked false)
  (Variables|Default|SetMarkMeter 0.0)
  (Variables|Default|SetMarkCounter 0.0)
  (CallFunction|UpdateMarkMeter))

(fn SetFrozenEffect
  (params (snowAmount :type Float%20%28single-precision%29))
  (Rendering|Material|SetScalarParameterValueonMaterials (Variables|Character|GetMesh) "SnowAmount" snowAmount))