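; Enemy spawner actor that runs one wave of grunts at its Arrow's transform and signals when the wave is complete.
; SpawnWave takes a wave stat and starts a looping timer that spawns each grunt through BulkheadGameState's SpawnMonster, tracking them in EnemyArray.
; Once spawning ends, a second timer prunes invalid enemies, firing OnWaveComplete when none remain or a tick-counted timeout expires.
; An older direct BP_Grunt spawn path remains unconnected.
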(event Custom|OnWaitForWaveToComplete_Event
  (Variables|Default|SetWaitForWaveToCompleteTickCount (Variables|Default|GetWaitForWaveToCompleteTickCountDefault))
  (bind _returnvalue (Utilities|Time|SetTimerbyFunctionName 0 "WaitForWaveToCompleteTick" (Variables|Default|GetWaitForWaveToCompleteTickInterval) true))
  (Variables|Default|SetWaitForWaveToCompleteTimer _returnvalue))

(event EventBeginPlay
  (EventDispatchers|BindEventtoOnWaitforWavetoComplete (delegate Custom|OnWaitForWaveToComplete_Event))
  (Variables|Default|SetWaitForWaveToCompleteTickCountDefault (Math|Float|Truncate (/ (Variables|Default|GetWaitForWaveToCompleteInSecond) (Variables|Default|GetWaitForWaveToCompleteTickInterval)))))

(fn ConstructionScript)

(fn SpawnSingleEnemy
  (bind _arrow (Variables|Default|GetArrow))
  (bind _returnvalue (Transformation|GetWorldTransform _arrow))
  (bind (_location _rotation) (Math|Transform|BreakTransform _returnvalue))
  (if (> (Variables|Default|GetEnemyToBeSpawn) 0)
    (bind _asbulkhead_game_state (Utilities|Casting|CastToBulkheadGameState (Game|GetGameState)))
    (bind _returnvalue_2 (Class|BulkheadGameState|SpawnMonster _asbulkhead_game_state (.GruntID (Utilities|Struct|BreakWaveStructData (Variables|Default|GetCurrentWaveStat))) 0 _location _rotation))
    (Utilities|Set|Add (Variables|Default|GetEnemyArray) _returnvalue_2)
    (Math|Integer|DecrementInt (Variables|Default|GetEnemyToBeSpawn)
      (:%20%20
        (return)))
    (else
      ;[1 1 1] Spawn complete, wait for wave to be complete
      (Default|CallOnWaitforWavetoComplete)
      (Utilities|Time|ClearandInvalidateTimerbyHandle (Variables|Default|GetSpawnWaveTimer))
      (return))))

(fn SpawnWave
  (params (SpawnInterval :type Float%20%28single-precision%29) (WaveStat :type Wave%20Struct%20Data%20Structure))
  (bind _output_get (Variables|Default|SetCurrentWaveStat WaveStat))
  (Utilities|Set|Clear (Variables|Default|GetEnemyArray))
  (Variables|Default|SetEnemyToBeSpawn (.GruntNumber (Utilities|Struct|BreakWaveStructData _output_get)))
  (bind _returnvalue (Utilities|Time|SetTimerbyFunctionName 0 "SpawnSingleEnemy" SpawnInterval true))
  (Variables|Default|SetSpawnWaveTimer _returnvalue))

(fn WaitforWavetoCompleteTick
  (bind _result (Utilities|Set|ToArray (Variables|Default|GetEnemyArray)))
  (for _array_element _result
    (Utilities|IsValid _array_element
      (:Is%20Not%20Valid
        (Utilities|Set|Remove (Variables|Default|GetEnemyArray) _array_element))))
  (if (== (Utilities|Set|Length (Variables|Default|GetEnemyArray)) 0)
    (Default|CallOnWaveComplete)
    (Utilities|Time|ClearandInvalidateTimerbyHandle (Variables|Default|GetWaitForWaveToCompleteTimer))
    (elif (> (Variables|Default|GetWaitForWaveToCompleteTickCount) 0)
      (Math|Integer|DecrementInt (Variables|Default|GetWaitForWaveToCompleteTickCount))
      (else
        (Default|CallOnWaveComplete)
        (Utilities|Time|ClearandInvalidateTimerbyHandle (Variables|Default|GetWaitForWaveToCompleteTimer))))))