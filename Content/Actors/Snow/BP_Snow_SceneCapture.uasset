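; Scene capture actor for snow that follows the player at a height offset from the Snow_Parameter collection.
; On BeginPlay it sets the orthographic width from that collection and clears two render targets to white.
; Each Tick it publishes the XY movement offset, draws the Snow_ADDRTT material into the second target, then moves the capture and publishes its position.
; A depth-map debug widget is left unconnected.
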(event EventBeginPlay
  (bind _returnvalue (Game|GetPlayerCharacter 0))
  (bind _scenecomponent (Variables|Default|GetSceneComponent))
  (bind _returnvalue_2 (Transformation|GetActorLocation _returnvalue))
  (Utilities|FlowControl|Sequence
    (:then_0
      (Transformation|SetWorldRotation _scenecomponent "90.000000, 0, 0" false false)
      (bind _returnvalue_3 (Rendering|Material|GetScalarParameterValue "/Game/Material/Snow/SnowDeformation/Snow_Parameter.Snow_Parameter" "CaptureZ" :!class /Script/Engine.KismetMaterialLibrary))
      (Transformation|SetWorldLocation _scenecomponent (Math|Vector|MakeVector (.x _returnvalue_2) (.y _returnvalue_2) (+ (.z _returnvalue_2) _returnvalue_3)) false false)
      (Rendering|Material|SetVectorParameterValue "/Game/Material/Snow/SnowDeformation/Snow_Parameter.Snow_Parameter" "CaptureCamerCurrentPos" (Utilities|Struct|MakeLinearColor (.x _returnvalue_2) (.y _returnvalue_2) (+ (.z _returnvalue_2) _returnvalue_3) 0.0) :!class /Script/Engine.KismetMaterialLibrary))
    (:then_1
      ;[1 1 1] set captureWidth by using Collection
      (bind _returnvalue_4 (Rendering|Material|GetScalarParameterValue "/Game/Material/Snow/SnowDeformation/Snow_Parameter.Snow_Parameter" "CaptureWidth" :!class /Script/Engine.KismetMaterialLibrary))
      (Variables|/Script/Engine.SceneCaptureComponent2D|SetOrthoWidth (Variables|DecalActor|GetCaptureComponent2D) _returnvalue_4)
      (bind _returnvalue_5 (Rendering|Material|CreateDynamicMaterialInstance "/Game/Material/Snow/SnowDeformation/Snow_ADDRTT.Snow_ADDRTT" "None" :!class /Script/Engine.KismetMaterialLibrary))
      (Variables|Default|SetSnowCaptureSave _returnvalue_5)
      (Rendering|ClearRenderTarget2D "/Game/Material/Snow/SnowDeformation/Snow_Scene_Capture_RTT1.Snow_Scene_Capture_RTT1" "(R=1.000000,G=1.000000,B=1.000000,A=1.000000)")
      (Rendering|ClearRenderTarget2D "/Game/Material/Snow/SnowDeformation/Snow_Scene_Capture_RTT2.Snow_Scene_Capture_RTT2" "(R=1.000000,G=1.000000,B=1.000000,A=1.000000)"))))

(event EventTick
  (params (DeltaSeconds :type Float%20%28single-precision%29))
  (bind _returnvalue (Transformation|GetActorLocation))
  (bind _returnvalue_2 (Game|GetPlayerCharacter 0))
  (bind _returnvalue_3 (Transformation|GetActorLocation _returnvalue_2))
  (bind _returnvalue_4 (Transformation|GetActorLocation _returnvalue_2))
  (bind _returnvalue_5 (- _returnvalue_4 _returnvalue))
  (Rendering|Material|SetVectorParameterValue "/Game/Material/Snow/SnowDeformation/Snow_Parameter.Snow_Parameter" "MoveOffset" (Utilities|Struct|MakeLinearColor (.x _returnvalue_5) (.y _returnvalue_5) 0.0 0.0) :!class /Script/Engine.KismetMaterialLibrary)
  (Rendering|DrawMaterialtoRenderTarget "/Game/Material/Snow/SnowDeformation/Snow_Scene_Capture_RTT2.Snow_Scene_Capture_RTT2" (Variables|Default|GetSnowCaptureSave))
  (bind _returnvalue_6 (Rendering|Material|GetScalarParameterValue "/Game/Material/Snow/SnowDeformation/Snow_Parameter.Snow_Parameter" "CaptureZ" :!class /Script/Engine.KismetMaterialLibrary))
  (Transformation|SetWorldLocation (Variables|Default|GetSceneComponent) (Math|Vector|MakeVector (.x _returnvalue_3) (.y _returnvalue_3) (+ (.z _returnvalue_3) _returnvalue_6)) false false)
  (Rendering|Material|SetVectorParameterValue "/Game/Material/Snow/SnowDeformation/Snow_Parameter.Snow_Parameter" "CaptureCamerCurrentPos" (Utilities|Struct|MakeLinearColor (.x _returnvalue_3) (.y _returnvalue_3) (+ (.z _returnvalue_3) _returnvalue_6) 0.0) :!class /Script/Engine.KismetMaterialLibrary))

(fn ConstructionScript)