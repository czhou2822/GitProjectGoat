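; Player character Blueprint handling tower building, air strikes, coin collection, pausing and snow-hit effects.
; Holding Build spawns the selected tower through BulkheadGameState, pulls the camera out, and snaps it to a screen-center capsule trace on a looping timer.
; Holding AirStrike enables a sphere that marks overlapping enemies up to the available strike count; release triggers the game mode's strike.
; Collected snow draws hit locations into a render target via a dynamic material.
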(event OnComponentBeginOverlap(NearPlayerSphere)
  (params (OverlappedComponent :type Primitive%20Component%20Object%20Reference) (OtherActor :type Actor%20Object%20Reference) (OtherComp :type Primitive%20Component%20Object%20Reference) (OtherBodyIndex :type Integer) (bFromSweep :type Boolean) (SweepResult :type Hit%20Result%20Structure%20%28by%20ref%29))
  ;[1 1 1] AirStrikeCheckBox
  (bind _asbp_project_goat_game_mode (Utilities|Casting|CastToBP_ProjectGoatGameMode (Game|GetGameMode)))
  (if (< (Variables|/Game/Actors/BP_BulkheadGameStates.BP_BulkheadGameStates_C|GetAimingCount (Variables|/Game/Actors/BP_ProjectGoatGameMode.BP_ProjectGoatGameMode_C|GetBulkheadGameState _asbp_project_goat_game_mode)) (Variables|/Game/Actors/BP_BulkheadPlayerState.BP_BulkheadPlayerState_C|GetAirStrikeCount (Variables|/Game/Actors/BP_ProjectGoatGameMode.BP_ProjectGoatGameMode_C|GetBulkheadPlayerState _asbp_project_goat_game_mode)))
    (bind _asbp_enemy_base (Utilities|Casting|CastToBP_EnemyBase OtherActor))
    (Variables|/Game/Actors/Enemy/EnemyBase/BP_EnemyBase.BP_EnemyBase_C|SetIsBeingMarked _asbp_enemy_base true)
    (Default|StartMarking _asbp_enemy_base 1.0)))

(event OnComponentEndOverlap(NearPlayerSphere)
  (params (OverlappedComponent :type Primitive%20Component%20Object%20Reference) (OtherActor :type Actor%20Object%20Reference) (OtherComp :type Primitive%20Component%20Object%20Reference) (OtherBodyIndex :type Integer))
  ;[1 1 1] AirStrikeCheckBox
  (bind _asbp_enemy_base (Utilities|Casting|CastToBP_EnemyBase OtherActor))
  (Variables|/Game/Actors/Enemy/EnemyBase/BP_EnemyBase.BP_EnemyBase_C|SetIsBeingMarked _asbp_enemy_base false))

(event OnComponentBeginOverlap(GoldCollectingSphere)
  (params (OverlappedComponent :type Primitive%20Component%20Object%20Reference) (OtherActor :type Actor%20Object%20Reference) (OtherComp :type Primitive%20Component%20Object%20Reference) (OtherBodyIndex :type Integer) (bFromSweep :type Boolean) (SweepResult :type Hit%20Result%20Structure%20%28by%20ref%29))
  ;[1 1 1] GoldSucking
  (bind _asbp_coin (Utilities|Casting|CastToBP_Coin OtherActor))
  (Utilities|Set|Add (Variables|Default|GetCoinList) _asbp_coin))

(event OnComponentEndOverlap(GoldCollectingSphere)
  (params (OverlappedComponent :type Primitive%20Component%20Object%20Reference) (OtherActor :type Actor%20Object%20Reference) (OtherComp :type Primitive%20Component%20Object%20Reference) (OtherBodyIndex :type Integer))
  ;[1 1 1] GoldSucking
  (bind _asbp_coin (Utilities|Casting|CastToBP_Coin OtherActor))
  (Utilities|Set|Remove (Variables|Default|GetCoinList) _asbp_coin))

(event Custom|WhichTower
  ;[1 1 1] Spawn Different Towers
  (bind _hitpoint (CallFunction|GetScreentoWorldLocation))
  (switch Utilities|FlowControl|Switch|SwitchonTower_Type (Variables|Default|GetTower)
    (:NewEnumerator0
      (bind _asbulkhead_game_state (Utilities|Casting|CastToBulkheadGameState (Game|GetGameState)))
      (bind _returnvalue (Class|BulkheadGameState|SpawnTower _asbulkhead_game_state 1 1 (.Location (Math|Transform|BreakTransform (Math|Conversions|ToTransform(Vector) (.Location (Collision|BreakHitResult _hitpoint))))) (.Rotation (Math|Transform|BreakTransform (Math|Conversions|ToTransform(Vector) (.Location (Collision|BreakHitResult _hitpoint)))))))
      (bind _asbp_tower_base (Utilities|Casting|CastToBP_TowerBase _returnvalue))
      (Variables|Default|SetSpawnedTower _asbp_tower_base))
    (:NewEnumerator1
      (bind _asbulkhead_game_state_2 (Utilities|Casting|CastToBulkheadGameState (Game|GetGameState)))
      (bind _returnvalue_2 (Class|BulkheadGameState|SpawnTower _asbulkhead_game_state_2 0 1 (.Location (Math|Transform|BreakTransform (Math|Conversions|ToTransform(Vector) (.Location (Collision|BreakHitResult _hitpoint))))) (.Rotation (Math|Transform|BreakTransform (Math|Conversions|ToTransform(Vector) (.Location (Collision|BreakHitResult _hitpoint)))))))
      (bind _asbp_tower_base_2 (Utilities|Casting|CastToBP_TowerBase _returnvalue_2))
      (Variables|Default|SetSpawnedTower _asbp_tower_base_2))))

(event Custom|OnConstructionComplete_Event
  ;[1 1 1] Spawn Different Towers
  (Development|PrintString "AirStrike tower complete" true false))

(event EventOnCollectSnow
  (params (location :type Vector :default "0, 0, 0"))
  (bind _hitsonwmaterial (Variables|Default|GetHitSonwMaterial))
  ;[1 1 1] collecting snow RTT
  (Rendering|Material|SetVectorParameterValue _hitsonwmaterial "HitLocationW" (Math|Conversions|ToLinearColor(Vector) location) :!class /Script/Engine.MaterialInstanceDynamic)
  (Rendering|DrawMaterialtoRenderTarget "/Game/Material/Snow/SnowDeformation/Snow_Scene_Capture_RTT2.Snow_Scene_Capture_RTT2" _hitsonwmaterial)
  (Audio|PlaySoundatLocation (Variables|Default|GetOnSnowCollectSound) location "0, 0, 0" 0.2 1.0 0.0 0 0 0))

(event EventTick
  (params (DeltaSeconds :type Float%20%28single-precision%29)))

(event EventBeginPlay
  (Utilities|FlowControl|Sequence
    (:then_0
      (CallFunction|LockPitchLimit))
    (:then_1
      ;[1 1 1] set up hit snow material
      (bind _returnvalue (Rendering|Material|CreateDynamicMaterialInstance "/Game/Material/Snow/SnowDeformation/HitOnSnow.HitOnSnow" "None" :!class /Script/Engine.KismetMaterialLibrary))
      (Variables|Default|SetHitSonwMaterial _returnvalue))
    (:then_2
      ;[1 1 1] Setup Variables
      (CallFunction|SetupVariables))))

(event EventFootstep
  (params (NewParam :type String))
  (Development|PrintText (Utilities|Text|ToText(String) NewParam) false false)
  (Audio|PlaySoundatLocation (Variables|Default|GetFoodprintSound) (Transformation|GetWorldLocation (Variables|Character|GetMesh)) "0, 0, 0" 0.2 1.0 0.0 0 0 0))

(event Input|ActionEvents|InputActionDestroyTower
  (params (Key :type Key%20Structure :default "None"))
  ;[1 1 1] Press Button
  (:Pressed
    (if (Variables|Default|GetIsCharacterPlacingTower)
      (Variables|Default|SetDestroyTowerMode true)
      (switch Utilities|FlowControl|Switch|SwitchonTower_Type (Variables|Default|GetTower)
        (:NewEnumerator0
          (Actor|DestroyActor (Variables|Default|GetBlue%20Tower)))
        (:NewEnumerator1
          (Actor|DestroyActor (Variables|Default|GetRed%20Tower)))
        (:NewEnumerator2
          (Actor|DestroyActor (Variables|Default|GetGreen%20Tower))))
      (Variables|Default|SetIsCharacterPlacingTower false)))
  (:Released
    (Variables|Default|SetDestroyTowerMode false)))

(event Input|ActionEvents|InputActionBuild
  (params (Key :type Key%20Structure :default "None"))
  ;[1 1 1] Press Button
  (:Pressed
    (if (not (Variables|Default|GetIsInShop))
      (|PulloutBuildingCamera)
      (CallFunction|WhichTower)
      (Variables|Default|SetIsCharacterPlacingTower true)
      (Default|CallOnCharacterStartPlacing true)
      (bind _returnvalue (Utilities|Time|SetTimerbyFunctionName 0 "AdjustTowerLocation" 0.016667 true))
      (Variables|TimerHandles|SetTowerAdjustTimer _returnvalue)
      (CallFunction|UnlockPitchLimit)))
  (:Released
    (if (not (Variables|Default|GetIsInShop))
      (Variables|Default|SetIsCharacterPlacingTower false)
      (Default|CallOnTowerPlaced)
      (Default|CallOnCharacterStartPlacing false)
      (Utilities|Time|ClearandInvalidateTimerbyHandle (Variables|TimerHandles|GetTowerAdjustTimer))
      (|ResetBuildingCamera)
      (CallFunction|LockPitchLimit))))

(event Input|ActionEvents|InputActionBuild
  (params (Key :type Key%20Structure :default "None"))
  ;[1 1 1] TowerSeedThrowing
)

(event Input|ActionEvents|InputActionOpenMenu
  (params (Key :type Key%20Structure :default "None"))
  (bind _returnvalue (Game|GetPlayerController 0))
  ;[1 1 1] Press Button
  (:Pressed
    (Game|SetGamePaused true)
    (bind _returnvalue_2 (UserInterface|CreateWidget "/Game/CC/widget/widget/UMG_Pause.UMG_Pause_C" _returnvalue))
    (UserInterface|Viewport|AddtoViewport _returnvalue_2 0)
    (Input|SetInputModeUIOnly _returnvalue 0 "DoNotLock")
    (Variables|/Script/Engine.PlayerController|SetbShowMouseCursor _returnvalue true)))

(event Input|ActionEvents|InputActionSelectTower
  (params (Key :type Key%20Structure :default "None"))
  ;[1 1 1] Press Button
  (:Pressed
    (Variables|Default|SetIsSelecting true)
    (switch Utilities|FlowControl|Switch|SwitchonTower_Type (Variables|Default|GetTower)
      (:NewEnumerator0
        (Variables|Default|SetTower "NewEnumerator1"))
      (:NewEnumerator1
        (Variables|Default|SetTower "NewEnumerator2"))
      (:NewEnumerator2
        (Variables|Default|SetTower "NewEnumerator0"))))
  (:Released
    (Variables|Default|SetIsSelecting false)))

(event Input|ActionEvents|InputActionCollectGold
  (params (Key :type Key%20Structure :default "None"))
  ;[1 1 1] GoldSucking
  (:Pressed
    (CollectingGold|EnableGoldSucking))
  (:Released
    (CollectingGold|DisableGoldSucking)))

(event Input|ActionEvents|InputActionAirStrike
  (params (Key :type Key%20Structure :default "None"))
  ;[1 1 1] AirStrike
)

(event Input|ActionEvents|InputActionAirStrike
  (params (Key :type Key%20Structure :default "None"))
  (:Pressed
    (AirStrike|OnAirStrikeAimUp))
  (:Released
    (AirStrike|OnAirStrikeAimDown)))

(fn ConstructionScript)

(fn GetScreentoWorldLocation
  (bind _returnvalue (Game|GetPlayerController 0))
  (bind _returnvalue_2 (Viewport|GetViewportSize))
  (bind _returnvalue_3 (/ _returnvalue_2 2.0))
  (bind (_worldposition _worlddirection) (Class|GameplayStatics|DeprojectScreentoWorld _returnvalue _returnvalue_3))
  (bind _outhit (Collision|LineTraceForObjects _worldposition (+ _worldposition (* _worlddirection 5000)) (Variables|Default|GetTowerTraceObjectArray) false 0 "None" true "(R=1.000000,G=0.000000,B=0.000000,A=1.000000)" "(R=0.000000,G=1.000000,B=0.000000,A=1.000000)" 0.2))
  (return _outhit))

(fn SetupVariables
  (Variables|Default|SetTower "NewEnumerator0")
  (Variables|Default|SetDefaultFOV (Variables|/Script/Engine.CameraComponent|GetFieldOfView (Variables|Default|GetCamera)))
  (Variables|Default|SetDefaultCamaraTransform (Transformation|GetRelativeTransform (Variables|Default|GetCamera))))

(fn HandleStrikeAim
  (bind _result (Utilities|Set|ToArray (Variables|Default|GetEnemiesAroundPlayer)))
  (for _array_element _result
    (if (.ReturnValue (Class|PlayerController|ProjectWorldLocationtoScreen (Game|GetPlayerController 0) (Transformation|GetActorLocation _array_element) false))
      (Development|PrintString (Utilities|String|Append "Screen location: " (Utilities|String|ToString(Vector2d) (.ScreenLocation (Class|PlayerController|ProjectWorldLocationtoScreen (Game|GetPlayerController 0) (Transformation|GetActorLocation _array_element) false)))) false true "(R=0.000000,G=0.660000,B=1.000000,A=1.000000)" 0.0)
      (Utilities|Array|Add (LocalVariables|GetEnemiesBeingAimed) _array_element)
      (Default|StartMarking _array_element 1.0))))

(fn OnAirStrikeAimUp
  (bind _nearplayersphere (Variables|Default|GetNearPlayerSphere))
  (Rendering|SetVisibility _nearplayersphere true false)
  (Collision|SetCollisionResponsetoChannel _nearplayersphere "ECC_GameTraceChannel9" "ECR_Overlap"))

(fn OnAirStrikeAimDown
  (bind _nearplayersphere (Variables|Default|GetNearPlayerSphere))
  (Rendering|SetVisibility _nearplayersphere false false)
  (Collision|SetCollisionResponsetoChannel _nearplayersphere "ECC_GameTraceChannel9" "ECR_Ignore")
  (bind _asbp_project_goat_game_mode (Utilities|Casting|CastToBP_ProjectGoatGameMode (Game|GetGameMode)))
  (Default|AirStrike _asbp_project_goat_game_mode))

(fn HandleonAirStrikeReady
  (params (ReadyedTower :type BP%20Air%20Strike%20Tower%20Object%20Reference))
  (Development|PrintString (Utilities|String|Append (Utilities|GetDisplayName ReadyedTower) " is ready"))
  (Utilities|Set|Add (Variables|Default|GetAirStrikeTowerSet) ReadyedTower)
  (Math|Integer|IncrementInt (Variables|Default|GetMissileCount)))

(fn AdjustTowerLocation
  (bind _returnvalue (Game|GetPlayerController 0))
  (bind _returnvalue_2 (Viewport|GetViewportSize))
  (bind _spawnedtower (Variables|Default|GetSpawnedTower))
  (bind _returnvalue_3 (/ _returnvalue_2 2.0))
  (bind _capsulecomponent (Variables|/Script/Engine.Character|GetCapsuleComponent _spawnedtower))
  (bind (_worldposition _worlddirection) (Class|GameplayStatics|DeprojectScreentoWorld _returnvalue _returnvalue_3))
  (bind (_outradius _outhalfheight) (Components|Capsule|GetScaledCapsuleSize _capsulecomponent))
  (Utilities|IsValid _spawnedtower
    (:Is%20Valid
      (bind _outhit (Collision|CapsuleTraceByChannel _worldposition (+ _worldposition (* _worlddirection 5000)) _outradius _outhalfheight "TraceTypeQuery2" false 0 "None" true "(R=1.000000,G=0.000000,B=0.000000,A=1.000000)" "(R=0.000000,G=1.000000,B=0.000000,A=1.000000)" 0.3))
      (Transformation|SetActorLocation (Variables|Default|GetSpawnedTower) (.Location (Collision|BreakHitResult _outhit)) false true))))

(fn AirStrike
  (bind _asbp_frost_cannon (Utilities|Casting|CastToBP_FrostCannon (Variables|/Script/Engine.ChildActorComponent|GetChildActor (Variables|Default|GetWeaponSlot))))
  (bind _output_get (LocalVariables|SetAirStrikeList (Variables|/Game/Actors/Weapon/BP_FrostCannon.BP_FrostCannon_C|GetAirStrikeList _asbp_frost_cannon)))
  (if (and (> (Utilities|Set|Length _output_get) 0) (> (Utilities|Set|Length (Variables|Default|GetAirStrikeTowerSet)) 0))
    (bind _result (Utilities|Set|ToArray (Variables|Default|GetAirStrikeTowerSet)))
    (for _array_element _result
      (Utilities|FlowControl|Sequence
        (:then_0
          (bind _result_2 (Utilities|Set|ToArray (LocalVariables|GetAirStrikeList)))
          (Utilities|IsValid (Utilities|Array|Get(acopy) _result_2)
            (:Is%20Valid
              (bind _output_get_2 (LocalVariables|SetSingleEnemy (Utilities|Array|Get(acopy) _result_2)))
              (Default|AirStrike _array_element _output_get_2)
              (bind _returnvalue (Utilities|Set|Remove (LocalVariables|GetAirStrikeList) _output_get_2))
              (if _returnvalue
                (Math|Integer|DecrementInt (Variables|Default|GetMissileCount))))
            (:Is%20Not%20Valid
              (Utilities|Set|Remove (LocalVariables|GetAirStrikeList) (Utilities|Array|Get(acopy) _result_2)))))))
    (Utilities|Set|Clear (Variables|Default|GetAirStrikeTowerSet))))

(fn LockPitchLimit
  (bind _returnvalue (Game|GetPlayerCameraManager 0))
  ;[1 1 1] limiting the camera pitch
  (Variables|/Script/Engine.PlayerCameraManager|SetViewPitchMin _returnvalue -8e+01)
  (Variables|/Script/Engine.PlayerCameraManager|SetViewPitchMax _returnvalue 1e+01))

(fn UnlockPitchLimit
  (bind _returnvalue (Game|GetPlayerCameraManager 0))
  ;[1 1 1] limiting the camera pitch
  (Variables|/Script/Engine.PlayerCameraManager|SetViewPitchMin _returnvalue -1e+01)
  (Variables|/Script/Engine.PlayerCameraManager|SetViewPitchMax _returnvalue 6e+01))

(fn IsinMonitor
  (params (InLocation :type Vector%202D%20Structure) (ComparingArea :type Vector%202D%20Structure))
  (if (<= (.x InLocation) (.x ComparingArea))
    (if (<= (.y InLocation) (.y ComparingArea))
      (return true)
      (else
        (return false)))
    (else
      (return false))))

(fn EnableGoldSucking
  (Rendering|SetVisibility (Variables|Default|GetGoldCollectingSphere) true false)
  (bind _result (Utilities|Set|ToArray (Variables|Default|GetCoinList)))
  (for _array_element _result
    (Default|FlytoPlayerEvent _array_element))
  (Utilities|Set|Clear (Variables|Default|GetCoinList)))

(fn DisableGoldSucking
  (Rendering|SetVisibility (Variables|Default|GetGoldCollectingSphere) false false))