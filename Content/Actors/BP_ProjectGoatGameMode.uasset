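; Game mode that manages the player's air strikes: target marking, tower registration, firing and charge recharge.
; On BeginPlay it caches the Bulkhead player state and game state, then starts a looping timer that counts toward recharges while charges are below maximum.
; Target marking is capped by available charges, and each registered tower raises the maximum.
; Firing pairs targets with towers by array index, spends a charge per valid pair and clears the target list.
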(event EventBeginPlay
  (Utilities|FlowControl|Sequence
    (:then_0
      (CallFunction|Init))
    (:then_1
      (bind _returnvalue (Utilities|Time|SetTimerbyFunctionName 0 "AirStrikeTimerTick" 0.033333 true))
      (Variables|AirStrike|SetAirStrikeTimerHandle _returnvalue))))

(event EventTick
  (params (DeltaSeconds :type Float%20%28single-precision%29)))

(fn ConstructionScript)

(fn AddtoStrikeList
  (params (NewTarget :type BP%20Enemy%20Base%20Object%20Reference))
  (if (<= (+ (Utilities|Set|Length (Variables|/Game/Actors/BP_BulkheadGameStates.BP_BulkheadGameStates_C|GetAirStrikeTargetsList (Variables|Default|GetBulkheadGameState))) 1) (Variables|/Game/Actors/BP_BulkheadPlayerState.BP_BulkheadPlayerState_C|GetAirStrikeCount (Variables|Default|GetBulkheadPlayerState)))
    (Utilities|Set|Add (Variables|/Game/Actors/BP_BulkheadGameStates.BP_BulkheadGameStates_C|GetAirStrikeTargetsList (Variables|Default|GetBulkheadGameState)) NewTarget)))

(fn RemovefromStrikeList
  (params (NewTarget :type BP%20Enemy%20Base%20Object%20Reference))
  (bind _returnvalue (Utilities|Set|Remove (Variables|/Game/Actors/BP_BulkheadGameStates.BP_BulkheadGameStates_C|GetAirStrikeTargetsList (Variables|Default|GetBulkheadGameState)) NewTarget))
  (return _returnvalue))

(fn AirStrike
  (bind _bulkheadgamestate (Variables|Default|GetBulkheadGameState))
  (bind _airstriketargetslist (Variables|/Game/Actors/BP_BulkheadGameStates.BP_BulkheadGameStates_C|GetAirStrikeTargetsList _bulkheadgamestate))
  (bind _returnvalue (Utilities|Set|Length _airstriketargetslist))
  (Development|PrintString (Utilities|String|Append "strike target length: " (Utilities|String|ToString(Integer) _returnvalue) " strike tower length: " (Utilities|String|ToString(Integer) (Utilities|Set|Length (Variables|/Game/Actors/BP_BulkheadGameStates.BP_BulkheadGameStates_C|GetAirStrikeTowerList (Variables|Default|GetBulkheadGameState))))))
  (if (>= _returnvalue 1)
    (bind _result (Utilities|Set|ToArray _airstriketargetslist))
    (for (_array_element _array_index) _result
      (Development|PrintString (Utilities|String|Append "Current index: " (Utilities|String|ToString(Integer) _array_index)))
      (bind _result_2 (Utilities|Set|ToArray (Variables|/Game/Actors/BP_BulkheadGameStates.BP_BulkheadGameStates_C|GetAirStrikeTowerList (Variables|Default|GetBulkheadGameState))))
      (Default|ResetMark _array_element)
      (Utilities|IsValid (Utilities|Array|Get(acopy) _result_2 _array_index)
        (:Is%20Valid
          (Utilities|IsValid _array_element
            (:Is%20Valid
              (Default|AirStrike (Utilities|Array|Get(acopy) _result_2 _array_index) _array_element)
              (Math|Integer|DecrementInt (Variables|/Game/Actors/BP_BulkheadPlayerState.BP_BulkheadPlayerState_C|GetAirStrikeCount (Variables|Default|GetBulkheadPlayerState))))))
        (:Is%20Not%20Valid
          (Development|PrintString (Utilities|String|Append "tower index: " (Utilities|String|ToString(Integer) _array_index) " not valid")))))
    (Utilities|Set|Clear (Variables|/Game/Actors/BP_BulkheadGameStates.BP_BulkheadGameStates_C|GetAirStrikeTargetsList (Variables|Default|GetBulkheadGameState)))
    (else
      (Development|PrintString "Air strike not firing"))))

(fn AddAirStrikeTower
  (params (NewAirStrikeTower :type BP%20Air%20Strike%20Tower%20Object%20Reference))
  (Utilities|Set|Add (Variables|/Game/Actors/BP_BulkheadGameStates.BP_BulkheadGameStates_C|GetAirStrikeTowerList (Variables|Default|GetBulkheadGameState)) NewAirStrikeTower)
  (Math|Integer|IncrementInt (Variables|/Game/Actors/BP_BulkheadPlayerState.BP_BulkheadPlayerState_C|GetMaxAirStrikeCount (Variables|Default|GetBulkheadPlayerState))))

(fn AirStrikeTimerTick
  (bind _bulkheadplayerstate (Variables|Default|GetBulkheadPlayerState))
  (if (< (Variables|/Game/Actors/BP_BulkheadPlayerState.BP_BulkheadPlayerState_C|GetAirStrikeCount _bulkheadplayerstate) (Variables|/Game/Actors/BP_BulkheadPlayerState.BP_BulkheadPlayerState_C|GetMaxAirStrikeCount _bulkheadplayerstate))
    (bind _result (Math|Integer|IncrementInt (Variables|AirStrike|GetAirStrikeCounter))
      (:%20%20
        (if (>= _result (Variables|AirStrike|GetMaxAirStrikeCounter))
          (Default|RechargeAirStrike (Variables|Default|GetBulkheadPlayerState))
          (Variables|AirStrike|SetAirStrikeCounter 0)
          (return)
          (else
            (return)))))
    (else
      (return))))

(fn Init
  (bind _asbp_bulkhead_player_state (Utilities|Casting|CastToBP_BulkheadPlayerState (Variables|/Script/Engine.Controller|GetPlayerState (Game|GetPlayerController 0))))
  (Variables|Default|SetBulkheadPlayerState _asbp_bulkhead_player_state)
  (bind _asbp_bulkhead_game_states (Utilities|Casting|CastToBP_BulkheadGameStates (Game|GetGameState)))
  (Variables|Default|SetBulkheadGameState _asbp_bulkhead_game_states))