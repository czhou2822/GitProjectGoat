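; BP_Projectile_Test is a test actor for lobbing a grenade in an arc at a referenced target actor.
; It enables input on BeginPlay, and the 0 key drives a FlipFlop between aiming and firing.
; The first press computes a high-arc toss velocity with debug drawing and no collision trace.
; The next press spawns BP_RealGrenade at the actor's location with that velocity.
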(event EventBeginPlay
  (Input|EnableInput (Game|GetPlayerController 0)))

(event Collision|EventActorBeginOverlap
  (params (OtherActor :type Actor%20Object%20Reference)))

(event EventTick
  (params (DeltaSeconds :type Float%20%28single-precision%29)))

(event Input|KeyboardEvents|0
  (params (Key :type Key%20Structure :default "None"))
  (bind _returnvalue (Transformation|GetActorLocation))
  (:Pressed
    (Utilities|FlowControl|FlipFlop
      (:A
        (bind _tossvelocity (Class|GameplayStatics|BlueprintSuggestProjectileVelocity _returnvalue (Transformation|GetActorLocation (Variables|Default|GetEndlocation)) (Variables|Default|GetLaunch%20Speed) 0.0 "DoNotTrace" 0.0 true true)))
      (:B
        (Game|SpawnActorfromClass "/Game/Character/Tower/Mortar/BP_RealGrenade.BP_RealGrenade_C" (Math|Conversions|ToTransform(Vector) _returnvalue) "Undefined" 0 _tossvelocity 3e+03 0)))))

(fn ConstructionScript)