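; Test tower base Blueprint that handles a placeable defence tower's placement, construction, targeting and damage effects.
; Placement clears instanced foliage via sphere trace and flags the anim instance, whose construction-complete event caches the AI controller and sizes the range sphere.
; Enemy overlaps run a looping timer copying the AI's target.
; Damage drives an HP material parameter plus one-shot smoke and fire stages; TowerFire, Tick and terrain snapping are stubs.
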(event OnComponentBeginOverlap(RangeBP)
  (params (OverlappedComponent :type Primitive%20Component%20Object%20Reference) (OtherActor :type Actor%20Object%20Reference) (OtherComp :type Primitive%20Component%20Object%20Reference) (OtherBodyIndex :type Integer) (bFromSweep :type Boolean) (SweepResult :type Hit%20Result%20Structure%20%28by%20ref%29))
  (bind _enemylist (Variables|Default|GetEnemyList))
  ;[1 1 1] Enemy overlap
  (bind _asenemy_base (Utilities|Casting|CastToEnemyBase OtherActor))
  (Utilities|Set|Add _enemylist _asenemy_base)
  (Development|PrintString "Enemy Detected" false false)
  (if (== (Utilities|Set|Length _enemylist) 1)
    (bind _returnvalue (Utilities|Time|SetTimerbyFunctionName 0 "SetTargetEnemy" 0.5 true))
    (Variables|Default|SetTargetingTimer _returnvalue)))

(event OnComponentEndOverlap(RangeBP)
  (params (OverlappedComponent :type Primitive%20Component%20Object%20Reference) (OtherActor :type Actor%20Object%20Reference) (OtherComp :type Primitive%20Component%20Object%20Reference) (OtherBodyIndex :type Integer))
  (bind _enemylist (Variables|Default|GetEnemyList))
  ;[1 1 1] Enemy overlap
  (bind _asenemy_base (Utilities|Casting|CastToEnemyBase OtherActor))
  (Utilities|Set|Remove _enemylist _asenemy_base)
  (if (not (Math|Conversions|ToBoolean(Integer) (Utilities|Set|Length _enemylist)))
    (Utilities|Time|ClearandInvalidateTimerbyHandle (Variables|Default|GetTargetingTimer))))

(event Custom|OnTowerDead
  (bind _self self)
  (bind _returnvalue (Transformation|GetActorLocation _self))
  ;[1 1 1] Tower dead
  (bind _swtowerdestruction (Variables|Default|GetSWTowerDestruction)
    (:then
      (Audio|PlaySoundatLocation _swtowerdestruction _returnvalue "0, 0, 0" 1.0 1.0 0.0 "/Game/Audio/Attenuation/MasterSoundAttenuation.MasterSoundAttenuation" 0 0)
      (Niagara|SpawnSystematLocation "/Game/VFX/Niagara/Damage/NS_Damage_Burst.NS_Damage_Burst" _returnvalue)
      ;;[1 1 1] Stop construction sound
      (bind _constructionaudiocomponent (Variables|Default|GetConstructionAudioComponent)
        (:then
          (Audio|Components|Audio|Stop _constructionaudiocomponent))
        (:else)))
    (:else)))

(event Custom|HandleABPOnConstructionComplete
  (bind _towerrange (Variables|Default|GetTowerRange))
  ;[1 1 1] Construction complete
  (Class|TowerBase|HandleonConstructionComplete)
  (bind _asai_tower_base (Utilities|Casting|CastToAI_TowerBase (Pawn|GetController)))
  (Variables|Default|SetTowerAI _asai_tower_base)
  (CallFunction|TowerInitBP)
  (Development|PrintString (Utilities|String|Append "TowerRange: " (Utilities|String|ToString(Float) _towerrange)) false false)
  (Components|Sphere|SetSphereRadius (Variables|Default|GetRangeBP) _towerrange true)
  (Transformation|SetWorldScale3D (Variables|Default|GetRangeMeshC) (Math|Conversions|ToVector(Float) (/ 0.0 5e+01))))

(event Custom|HandleInternalTowerPlaced
  ;[1 1 1] Tower placed
  (CallFunction|DestroyPossibleFoliage)
  (Utilities|IsValid (Variables|Default|GetAnimBase)
    (:Is%20Valid
      (EventDispatchers|BindEventtoOnConstructionComplete (Variables|Default|GetAnimBase) (delegate Custom|HandleABPOnConstructionComplete))
      (Variables|/Script/ProjectGoat.AnimTowerBase|SetbIsPlaced (Variables|Default|GetAnimBase) true)
      (EventDispatchers|BindEventtoOnBulkheadCharacterDead (delegate Custom|OnTowerDead)))))

(event EventBeginPlay
  ;[1 1 1] Begin play
  (bind _asanim_tower_base (Utilities|Casting|CastToAnimTowerBase (Components|SkeletalMesh|GetAnimInstance (Variables|Character|GetMesh))))
  (Variables|Default|SetAnimBase _asanim_tower_base)
  (EventDispatchers|AssignInternalTowerPlaced (delegate Custom|HandleInternalTowerPlaced))
  ;;[1 1 1] Randomly place DamageSmoke FX system
  (Transformation|SetRelativeLocation (Variables|Default|GetDamageSmoke) (.OutItem (Utilities|Array|Random (Variables|Default|GetDamageSmokeLocations))) false false))

(event EventConstructionStarts
  ;[1 1 1] Construction start
  (bind _construcionsound (Variables|Audio|GetConstrucionSound)
    (:then
      (bind _returnvalue (Audio|SpawnSoundatLocation _construcionsound (Transformation|GetActorLocation self) "0, 0, 0" 1.0 1.0 0.0 "/Game/Audio/Attenuation/MasterSoundAttenuation.MasterSoundAttenuation" 0))
      (bind _output_get (Variables|Default|SetConstructionAudioComponent _returnvalue))
      (Audio|Components|Audio|Play _output_get 0.0))
    (:else)))

(event EventTick
  (params (DeltaSeconds :type Float%20%28single-precision%29))
  ;[1 1 1] Tick
)

(event EventTowerFire
  ;[1 1 1] Tower fire
  (Development|PrintString "base tower fire" false false))

(event EventOnReceivedDamage
  (params (ReceivedDamage :type Float%20%28single-precision%29) (RemainingHealthPercentage :type Float%20%28single-precision%29))
  (bind _damageburst (Variables|Default|GetDamageBurst))
  ;[1 1 1] Receive Damage
  (Development|PrintString (Utilities|String|Append "Object: " (Utilities|GetObjectName self) " Received Damage: " (Utilities|String|ToString(Float) ReceivedDamage) " Remaning Percentage: " (Utilities|String|ToString(Float) RemainingHealthPercentage)) false)
  ;[1 1 1] Set Material Parameter
  (Rendering|Material|SetScalarParameterValueonMaterials (Variables|Character|GetMesh) "NormalizedHP" RemainingHealthPercentage)
  ;[1 1 1] Damage Burst FX
  (Math|Float|CompareFloat RemainingHealthPercentage 0.666667
    (:==
      (Utilities|FlowControl|DoOnce false :!label _label
        (:Completed
          (Components|Activation|Activate (Variables|Default|GetDamageSmoke) false))))
    (:<
      (Utilities|FlowControl|Sequence
        (:then_0
          (goto _label))
        (:then_1
          (Math|Float|CompareFloat RemainingHealthPercentage 0.333333
            (:==
              _)
            (:<
              _))
          (Utilities|FlowControl|DoOnce false
            (:Completed
              (Class|NiagaraComponent|SetVariableBool (Variables|Default|GetDamageSmoke) "Fire?" true)))))))
  (Components|Activation|Deactivate _damageburst)
  (Components|Activation|Activate _damageburst false))

(fn ConstructionScript)

(fn SetTargetEnemy
  (bind _towerai (Variables|Default|GetTowerAI))
  (bind _targetactor (Variables|/Game/Character/Tower/TowerBase/AI_TowerBase.AI_TowerBase_C|GetTargetActor _towerai))
  (Development|PrintString "Hello" false false)
  (Utilities|IsValid _towerai
    (:Is%20Valid
      (Utilities|IsValid _targetactor
        (:Is%20Valid
          (bind _output_get (Variables|Default|SetTargetEnemy _targetactor))
          (Variables|Default|SetTargetLocation (Transformation|GetActorLocation _output_get)))
        (:Is%20Not%20Valid
          (Variables|Default|SetTargetEnemy 0))))))

(fn Turnto
  (params (DeltaTime :type Float%20%28single-precision%29))
  (bind _returnvalue (Transformation|GetActorRotation))
  (bind _targetenemy (Variables|Default|GetTargetEnemy)
    (:then
      (if (< (.y (Math|Vector|Normalize (- (Transformation|GetActorLocation _targetenemy) (Transformation|GetActorLocation)))) 0.0)
        (Variables|/Script/ProjectGoat.AnimTowerBase|SetDoomRotation (Variables|Default|GetAnimBase) (Math|Rotator|MakeRotator 0.0 0.0 (- (- 3.6e+02 (Class|KismetMathLibrary|DegAcos (Math|Vector|DotProduct (Math|Vector|MakeVector (.x (Math|Vector|Normalize (- (Transformation|GetActorLocation _targetenemy) (Transformation|GetActorLocation)))) (.y (Math|Vector|Normalize (- (Transformation|GetActorLocation _targetenemy) (Transformation|GetActorLocation)))) (.z (Math|Vector|Normalize (- (Transformation|GetActorLocation _targetenemy) (Transformation|GetActorLocation))))) (Math|Vector|MakeVector 1.0 0.0 0.0)))) (.yaw _returnvalue))))
        (else
          (Variables|/Script/ProjectGoat.AnimTowerBase|SetDoomRotation (Variables|Default|GetAnimBase) (Math|Rotator|MakeRotator 0.0 0.0 (- (Class|KismetMathLibrary|DegAcos (Math|Vector|DotProduct (Math|Vector|MakeVector (.x (Math|Vector|Normalize (- (Transformation|GetActorLocation _targetenemy) (Transformation|GetActorLocation)))) (.y (Math|Vector|Normalize (- (Transformation|GetActorLocation _targetenemy) (Transformation|GetActorLocation)))) (.z (Math|Vector|Normalize (- (Transformation|GetActorLocation _targetenemy) (Transformation|GetActorLocation))))) (Math|Vector|MakeVector 1.0 0.0 0.0))) (.yaw _returnvalue)))))))
    (:else)))

(fn TowerInitBP
  (bind _asai_tower_base (Utilities|Casting|CastToAI_TowerBase (Pawn|GetController)))
  (Variables|Default|SetTowerAI _asai_tower_base))

(fn TerrianSnapping)

(fn DestroyPossibleFoliage
  (bind _returnvalue (Transformation|GetActorLocation))
  ;[1 1 1] basically, when a tower is landed/before construction, do a multi-trace at the location and look for any number of foliages and delete them.
  (bind _outhits (Collision|MultiSphereTraceByChannel (Transformation|GetActorLocation) (Math|Vector|MakeVector (.x _returnvalue) (.y _returnvalue) (- (.z _returnvalue) 1e+02)) (Variables|/Script/Engine.CapsuleComponent|GetCapsuleRadius (Variables|Default|GetCapsuleComponent)) "TraceTypeQuery5" false 0 "None"))
  (for _array_element _outhits
    (Audio|PlaySoundatLocation "/Game/Audio/SFX/Destruction/A_Tree_Cue.A_Tree_Cue" (.Location (Collision|BreakHitResult _array_element)) "0, 0, 0" 1.0 1.0 0.1 0 0 0)
    (Niagara|SpawnSystematLocation "/Game/VFX/NS_Environment_Destruction.NS_Environment_Destruction" (.Location (Collision|BreakHitResult _array_element)))
    (Development|PrintString (Utilities|String|Append "component:  " (Utilities|GetDisplayName (.HitComponent (Collision|BreakHitResult _array_element))) " hit item: " (Utilities|String|ToString(Integer) (.HitItem (Collision|BreakHitResult _array_element)))) false false)
    (bind _asinstanced_static_mesh_component (Utilities|Casting|CastToInstancedStaticMeshComponent (.HitComponent (Collision|BreakHitResult _array_element))))
    (Class|InstancedStaticMeshComponent|RemoveInstance _asinstanced_static_mesh_component (.HitItem (Collision|BreakHitResult _array_element)))))