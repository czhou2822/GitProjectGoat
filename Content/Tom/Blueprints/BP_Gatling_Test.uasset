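; Gatling tower Blueprint, apparently a test version, that extends a parent tower class to aim at and damage a target enemy.
; Tick calls TurnTo and feeds a clamped look-at pitch between enemy and elevation socket into the AnimBP's barrel rotation as roll.
; The tower fire tick starts or stops the attack montage as IsAttack changes, guarded by a playing flag.
; A separate FireBullet event applies tower damage directly to the target.
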(event EventTowerFireTickInterface
  (if (Variables|Default|GetbIsAttack)
    (if (not (Variables|Default|GetIsPlayingAttackMontage))
      (Animation|Montage|PlayMontage (Variables|Character|GetMesh) "/Game/Character/Tower/Gatling/Animations/AM_GatlingAttacks.AM_GatlingAttacks"
        (:then
          (Variables|Default|SetIsPlayingAttackMontage true))))
    (elif (Variables|Default|GetIsPlayingAttackMontage)
      (Animation|StopAnimMontage "/Game/Character/Tower/Gatling/Animations/AM_GatlingAttacks.AM_GatlingAttacks")
      (Variables|Default|SetIsPlayingAttackMontage false))))

(event EventFireBullet
  (Class|BulkheadCharacterBase|Attack self (Variables|Default|GetTargetEnemy) (Variables|Default|GetTowerDamage)))

(event EventHandleABPonConstructionComplete
  (|CallParentFunction))

(event EventTick
  (params (DeltaSeconds :type Float%20%28single-precision%29))
  (|CallParentFunction DeltaSeconds)
  (CallFunction|Turnto 0.0)
  (bind _targetenemy (Variables|Default|GetTargetEnemy)
    (:then
      (Variables|/Script/ProjectGoat.AnimTowerBase|SetBarrelRotation (Variables|Default|GetAnimBase) (Math|Rotator|MakeRotator (Math|Float|ClampAngle (.pitch (Math|Rotator|FindLookatRotation (Transformation|GetActorLocation _targetenemy) (Transformation|GetSocketLocation (Variables|Character|GetMesh) "Turret_Elevation_JNT"))) -2e+01 1e+01) 0.0 0.0)))
    (:else)))

(fn ConstructionScript
  (|CallParentFunction))