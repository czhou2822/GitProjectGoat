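; BP_TutorialBuildingGround_test is a test tutorial building ground actor that toggles its construction-area tag based on the player's selected tower.
; On BeginPlay it binds to the selected-tower-changed event of the first player state, cast to BP_BulkheadPlayerState.
; When the selected tower matches DesiredTower, its tags become ConstructionArea, otherwise None.
; The Box overlap events are empty and the Decal is unused.
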(event OnComponentBeginOverlap(Box)
  (params (OverlappedComponent :type Primitive%20Component%20Object%20Reference) (OtherActor :type Actor%20Object%20Reference) (OtherComp :type Primitive%20Component%20Object%20Reference) (OtherBodyIndex :type Integer) (bFromSweep :type Boolean) (SweepResult :type Hit%20Result%20Structure%20%28by%20ref%29)))

(event OnComponentEndOverlap(Box)
  (params (OverlappedComponent :type Primitive%20Component%20Object%20Reference) (OtherActor :type Actor%20Object%20Reference) (OtherComp :type Primitive%20Component%20Object%20Reference) (OtherBodyIndex :type Integer)))

(event Custom|OnSelectedTowerChanged_Event_0
  (params (NewTower :type ETowerType%20Enum :default "TESLA"))
  (if (Utilities|Enum|Equal(Enum) NewTower (Variables|Default|GetDesiredTower))
    (Variables|Default|SetTags (Utilities|Array|MakeArray "ConstructionArea"))
    (else
      (Variables|Default|SetTags (Utilities|Array|MakeArray "None")))))

(event EventBeginPlay
  (bind _asbp_bulkhead_player_state (Utilities|Casting|CastToBP_BulkheadPlayerState (Utilities|Array|Get(acopy) (Variables|/Script/Engine.GameStateBase|GetPlayerArray (Game|GetGameState)))))
  (EventDispatchers|AssignOnSelectedTowerChanged _asbp_bulkhead_player_state (delegate Custom|OnSelectedTowerChanged_Event_0)))

(fn ConstructionScript)