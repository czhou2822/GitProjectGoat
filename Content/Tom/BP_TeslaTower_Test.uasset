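; Test Tesla tower that fires chain lightning from its FirePoint socket through nearby enemies.
; BeginPlay pools hidden beam emitters, one per possible link.
; TowerFire starts a looping LightingTick that shows a beam, applies exponentially decaying damage, then sphere-searches for the next living, unhit enemy until none remains or the link cap is reached.
; StopLightingEffect hides the beams but is uncalled here, and the timed LightingEffectTick is undefined here.
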(event EventBeginPlay
  (|CallParentFunction)
  (for _index (range 0 (- (Variables|Default|GetMaxChainLinks) 1))
    (bind _returnvalue (Effects|SpawnEmitteratLocation "/Game/Character/Tower/Tesla/Particles/P_Lighting.P_Lighting" "0, 0, 0" "0, 0, 0" "1.000000,1.000000,1.000000" false))
    (Rendering|SetVisibility _returnvalue false false)
    (Utilities|Array|Add (Variables|Default|GetLightingBeams) _returnvalue)))

(event Collision|EventActorBeginOverlap
  (params (OtherActor :type Actor%20Object%20Reference))
  (|CallParentFunction OtherActor) ; This node is disabled and will not be called.\nDrag off pins to build functionality.
)

(event EventTick
  (params (DeltaSeconds :type Float%20%28single-precision%29))
  (|CallParentFunction DeltaSeconds))

(event EventTowerFire
  (bind _targetenemy (Variables|Default|GetTargetEnemy))
  (Development|PrintString "Tesla Fire" false)
  (Utilities|IsValid _targetenemy
    (:Is%20Valid
      (Variables|Default|SetNextEnemy _targetenemy)
      (Variables|Default|SetLastLightingLocation (Transformation|GetSocketLocation (Variables|Character|GetMesh) "FirePoint"))
      (Variables|Default|SetChainLinks 0)
      (bind _returnvalue (Utilities|Time|SetTimerbyFunctionName 0 "LightingTick" 0.1 true))
      (Variables|Default|SetLightingHandle _returnvalue)
      (Utilities|Time|SetTimerbyFunctionName 0 "LightingEffectTick" 0.1 true)
      (Class|TowerBase|PlayFireSound))))

(fn ConstructionScript
  (|CallParentFunction))

(fn LightingTick
  (if (== (Variables|Default|GetChainLinks) (Variables|Default|GetMaxChainLinks))
    (CallFunction|StopLightingAttack)
    (return)
    (else
      (bind _nextenemy (Variables|Default|GetNextEnemy)
        (:then
          (Utilities|Array|Add (Variables|Default|GetLightingIgnoreList) _nextenemy)
          (CallFunction|PlayLightingEffect (Variables|Default|GetLastLightingLocation) (Transformation|GetActorLocation _nextenemy))
          (Variables|Default|SetLastLightingLocation (Transformation|GetActorLocation _nextenemy))
          (bind (_outactors _returnvalue) (Collision|SphereOverlapActors (Transformation|GetActorLocation _nextenemy) (Variables|Default|GetLIghtingStrikeRadius) (LocalVariables|GetNewLocalVar_2) "/Game/Character/Enemy/EnemyBase/BP_EnemyBase.BP_EnemyBase_C" (Variables|Default|GetLightingIgnoreList)))
          (CallFunction|LightingAttack)
          (if _returnvalue
            (bind _array_element (Utilities|Array|ForEachLoopwithBreak _outactors)
              (:LoopBody
                (Utilities|IsValid _array_element
                  (:Is%20Valid
                    (bind _asbp_enemy_base (Utilities|Casting|CastToBP_EnemyBase _array_element))
                    (bind _returnvalue_2 (Class|BulkheadCharacterBase|GetCharacterData _asbp_enemy_base))
                    (if (> (.health _returnvalue_2) 0.0)
                      (Variables|Default|SetNextEnemy _asbp_enemy_base)
                      (Math|Integer|IncrementInt (Variables|Default|GetChainLinks)
                        (:%20%20
                          (return)))))))
              (:Completed
                (CallFunction|StopLightingAttack)
                (return)))
            (else
              (CallFunction|StopLightingAttack)
              (return))))
        (:else
          (return))))))

(fn LightingAttack
  (bind _nextenemy (Variables|Default|GetNextEnemy))
  (Utilities|IsValid _nextenemy
    (:Is%20Valid
      (Class|BulkheadCharacterBase|Attack self _nextenemy (* (Variables|Default|GetTowerDamage) (Math|Float|Power 0.7 (Math|Conversions|ToFloat(Integer) (Variables|Default|GetChainLinks))))))))

(fn StopLightingAttack
  (Utilities|Time|ClearandInvalidateTimerbyHandle (Variables|Default|GetLightingHandle))
  (Utilities|Array|Clear (Variables|Default|GetLightingIgnoreList)))

(fn PlayLightingEffect
  (params (Start :type Vector) (End :type Vector))
  (bind _lightingbeams (Variables|Default|GetLightingBeams))
  (bind _chainlinks (Variables|Default|GetChainLinks))
  (bind _output (Utilities|Array|Get(acopy) _lightingbeams _chainlinks))
  (Class|ParticleSystemComponent|SetBeamSourcePoint _output 0 Start)
  (Class|ParticleSystemComponent|SetBeamTargetPoint _output 0 End)
  (Rendering|SetVisibility _output true false))

(fn StopLightingEffect
  (for _array_element (Variables|Default|GetLightingBeams)
    (Rendering|SetVisibility _array_element false false))
  (return))