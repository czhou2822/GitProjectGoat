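; Game mode that runs an endless loop of enemy waves and timed collecting phases.
; On BeginPlay it takes the first spawn point, binds its wave-complete event and, if IsSpawning is set, starts the first wave.
; Wave completion starts a looping timer countdown, whose end fires OnCollectingPhaseComplete to spawn the next wave.
; The wave-counter and EndGame pause logic are disconnected and never run.
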(event Custom|BindOnCollectingPhaseComplete
  ;[1 1 1] Spawn New Wave
  (CallFunction|HandleonCollectingPhaseComplete))

(event Custom|BindOnWaveComplete
  ;[1 1 1] Spawn New Wave
  (CallFunction|HandleonWaveComplete))

(event EventBeginPlay
  (Utilities|FlowControl|Sequence
    (:then_0
      (bind _result (Utilities|Set|ToArray (Variables|Default|GetSpawnPointsArray)))
      ;[1 1 1] Spawn New Wave
      (Utilities|IsValid (Utilities|Array|Get(acopy) _result)
        (:Is%20Valid
          (bind _output_get (Variables|Default|SetActiveSpawnPoint (Utilities|Array|Get(acopy) _result)))
          (EventDispatchers|BindEventtoOnWaveComplete _output_get (delegate Custom|BindOnWaveComplete))
          (EventDispatchers|AssignOnCollectingPhaseComplete (delegate Custom|BindOnCollectingPhaseComplete)))))
    (:then_1
      (if (Variables|Default|GetIsSpawning)
        (CallFunction|StartGame)))))

(fn ConstructionScript)

(fn HandleonWaveComplete
  (Development|PrintString "WaveComplete")
  (Variables|Default|SetCollectingPhaseTickCount (/ (Variables|Default|GetCollectingPhaseInSecond) (Variables|Default|GetCollectingPhaseTickInterval)))
  (bind _returnvalue (Utilities|Time|SetTimerbyFunctionName 0 "CollectingPhaseTick" (Variables|Default|GetCollectingPhaseTickInterval) true))
  (Variables|Default|SetCollectingPhaseTimerHandler _returnvalue))

(fn HandleonCollectingPhaseComplete
  (Default|SpawnWave (Variables|Default|GetActiveSpawnPoint) (Variables|Default|GetSpawnSingleEnemyInterval) (Variables|Default|GetWaveEnemyCount)))

(fn StartGame
  (Default|SpawnWave (Variables|Default|GetActiveSpawnPoint) (Variables|Default|GetSpawnSingleEnemyInterval) (Variables|Default|GetWaveEnemyCount)))

(fn CollectingPhaseTick
  (if (> (Variables|Default|GetCollectingPhaseTickCount) 0.0)
    (Math|Float|DecrementFloat (Variables|Default|GetCollectingPhaseTickCount))
    (else
      (Default|CallOnCollectingPhaseComplete)
      (Development|PrintString "Collecting Phase complete")
      (Utilities|Time|ClearandInvalidateTimerbyHandle (Variables|Default|GetCollectingPhaseTimerHandler)))))

(fn EndGame
  (Game|SetGamePaused true)
  (Development|PrintString "Thanks for playing" true true "(R=1.000000,G=0.000000,B=0.008526,A=1.000000)" 3e+01))