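; BP_GameMaster runs the wave-based game loop, alternating timed collecting phases with enemy waves and deciding win or loss.
; A looping timer ends each collecting phase, then a data table row keyed by wave number configures the first spawn point's wave.
; Wave completion restarts collecting.
; Reaching the player inventory's bulk target opens the end level, while a base explosion or missing wave row opens the fail level.
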(event BaseExploded(BaseObject)
  (CallFunction|EndGameFailed))

(event Custom|BindOnCollectingPhaseComplete
  ;[1 1 1] DataBinding
  (CallFunction|HandleonCollectingPhaseComplete))

(event Custom|BindOnBulkChanged
  (params (CurrentBulkCount :type Integer))
  ;[1 1 1] DataBinding
  (CallFunction|HandleonBulkChanged CurrentBulkCount))

(event Custom|BindOnWaveComplete
  ;[1 1 1] DataBinding
  (CallFunction|HandleonWaveComplete))

(event EventBeginPlay
  (Utilities|FlowControl|Sequence
    (:then_0
      ;[1 1 1] DataBinding
      (bind _result (Utilities|Set|ToArray (Variables|Default|GetSpawnPointsArray)))
      (Utilities|IsValid (Utilities|Array|Get(acopy) _result)
        (:Is%20Valid
          (bind _output_get (Variables|Default|SetActiveSpawnPoint (Utilities|Array|Get(acopy) _result)))
          (EventDispatchers|BindEventtoOnWaveComplete _output_get (delegate Custom|BindOnWaveComplete))
          (EventDispatchers|AssignOnCollectingPhaseComplete (delegate Custom|BindOnCollectingPhaseComplete))
          (bind _asbp_player_character (Utilities|Casting|CastToBP_PlayerCharacter (Game|GetPlayerCharacter 0)))
          (bind _output_get_2 (Variables|Default|SetPlayerCharacter _asbp_player_character))
          (EventDispatchers|AssignOnBulkChanged (Variables|/Script/ProjectGoat.TPSCharacterQ|GetInventoryComp _output_get_2) (delegate Custom|BindOnBulkChanged))
          (Variables|Default|SetBulkCountString (Utilities|String|Append "BulkCount:  0/" (Utilities|String|ToString(Integer) (Variables|Default|GetBulkTarget)))))))
    (:then_2
      (if (Variables|Default|GetIsSpawning)
        (CallFunction|StartCollectionPhase)))))

(fn ConstructionScript)

(fn HandleonWaveComplete
  (Development|PrintString "WaveComplete")
  (CallFunction|StartCollectionPhase))

(fn HandleonCollectingPhaseComplete
  (if (Variables|Default|GetisGameEnd)
    (CallFunction|EndGameSuccess)
    (else
      (bind _result (Math|Integer|IncrementInt (Variables|Default|GetWaveCounter))
        (:%20%20
          (CallFunction|StartWave _result))))))

(fn HandleonBulkChanged
  (params (InBulkCount :type Integer))
  (Variables|Default|SetBulkCountString (Utilities|String|Append "BulkCount: " (Utilities|String|ToString(Integer) InBulkCount) "/" (Utilities|String|ToString(Integer) (Variables|Default|GetBulkTarget))))
  (if (>= InBulkCount (Variables|Default|GetBulkTarget))
    (CallFunction|EndGameSuccess)))

(fn CollectingPhaseTick
  (if (> (Variables|Default|GetCollectingPhaseTickCount) 0.0)
    (Math|Float|DecrementFloat (Variables|Default|GetCollectingPhaseTickCount))
    (else
      (Default|CallOnCollectingPhaseComplete)
      (Development|PrintString "Collecting Phase complete")
      (Utilities|Time|ClearandInvalidateTimerbyHandle (Variables|Default|GetCollectingPhaseTimerHandler)))))

(fn EndGameSuccess
  (Development|PrintString "Thanks for playing" true true "(R=1.000000,G=0.000000,B=0.008526,A=1.000000)" 3e+01)
  (Game|OpenLevel(byName) "EndGameLevel"))

(fn SetWaveStat
  (params (InWaveNumber :type Name))
  (bind _returnvalue (Utilities|GetDataTableRow "/Game/Blueprint/GameMaster/DataTable_WaveStats.DataTable_WaveStats" InWaveNumber)
    (:then
      (bind _output_get (Variables|Default|SetWaveStat _returnvalue))
      (return _output_get))
    (:RowNotFound
      (CallFunction|EndGameFailed))))

(fn StartWave
  (params (WaveNumber :type Integer))
  (bind _outwavestat (CallFunction|SetWaveStat (Utilities|String|StringToName (Utilities|String|ToString(Integer) WaveNumber))))
  (bind _stringoutput (CallFunction|StruttoString _outwavestat))
  (Development|PrintString _stringoutput)
  (Default|SpawnWave (Variables|Default|GetActiveSpawnPoint) (Variables|Default|GetSpawnSingleEnemyInterval) (.WaveEnemies (Utilities|Struct|BreakWaveStatStructure _outwavestat)) (.GoldDropRate (Utilities|Struct|BreakWaveStatStructure _outwavestat)) (.EnemyHealth (Utilities|Struct|BreakWaveStatStructure _outwavestat))))

(fn IsGameEnded
  (Variables|Default|SetisGameEnd (== (Variables|/Script/ProjectGoat.InventoryComponent|GetBulkCount (Actor|GetComponentbyClass (Variables|Default|GetPlayerCharacter) "/Script/ProjectGoat.InventoryComponent")) (Variables|Default|GetBulkTarget)))
  (return))

(fn StruttoString
  (params (InStruct :type Wave%20Stat%20Structure%20Structure))
  (bind (_wavenumber _waveenemies _enemyhealth _golddroprate) (Utilities|Struct|BreakWaveStatStructure InStruct))
  (return (Utilities|String|Append (Utilities|String|Append (Utilities|String|Append "Number: " (Utilities|String|ToString(Integer) _wavenumber)) (Utilities|String|Append " Enemy Count: " (Utilities|String|ToString(Integer) _waveenemies))) (Utilities|String|Append (Utilities|String|Append " EnemyHealth:  " (Utilities|String|ToString(Float) _enemyhealth)) (Utilities|String|Append " GoldDropRate:  " (Utilities|String|ToString(Float) _golddroprate))))))

(fn StartCollectionPhase
  (Variables|Default|SetCollectingPhaseTickCount (/ (Variables|Default|GetCollectingPhaseInSecond) (Variables|Default|GetCollectingPhaseTickInterval)))
  (bind _returnvalue (Utilities|Time|SetTimerbyFunctionName 0 "CollectingPhaseTick" (Variables|Default|GetCollectingPhaseTickInterval) true))
  (Variables|Default|SetCollectingPhaseTimerHandler _returnvalue))

(fn EndGameFailed
  (Game|OpenLevel(byName) "FailLevel"))