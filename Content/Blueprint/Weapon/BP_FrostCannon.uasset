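; Prototype frost cannon weapon that projects a hit capsule from the muzzle while firing, spending the player's SnowCount.
; Tick centers the capsule between the muzzle and a camera-forward range point, pitched from the player's view.
; Fire start, if snow remains, enables overlap on a custom channel; BeginPlay and fire end restore ignore.
; DrawDebugCapsule doubles as firing state, driving visibility, debug drawing and the player character's IsFire flag.
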(event EventBeginPlay
  (bind _frosthitcapsule (Variables|Default|GetFrostHitCapsule))
  (Utilities|FlowControl|Sequence
    (:then_0
      (Collision|SetCollisionResponsetoChannel _frosthitcapsule "ECC_GameTraceChannel9" "ECR_Ignore")
      (Variables|Default|SetDrawDebugCapsule false))
    (:then_1
      (Rendering|SetVisibility _frosthitcapsule (Variables|Default|GetDrawDebugCapsule) false))))

(event EventTick
  (params (DeltaSeconds :type Float%20%28single-precision%29))
  (bind _returnvalue (Game|Player|GetPlayerPawn 0))
  (bind _returnvalue_2 (Game|Player|GetPlayerPawn 0))
  (bind _frosthitcapsule (Variables|Default|GetFrostHitCapsule))
  (bind _frosthitcapsule_2 (Variables|Default|GetFrostHitCapsule))
  (bind _weaponmesh (Variables|Default|GetWeaponMesh))
  (bind _outrotation (Actor|GetActorEyesViewPoint _returnvalue))
  (bind _outrotation_2 (Actor|GetActorEyesViewPoint _returnvalue_2))
  (bind (_roll _pitch _yaw) (Math|Rotator|BreakRotator _outrotation))
  (bind (_roll_2 _pitch_2 _yaw_2) (Math|Rotator|BreakRotator _outrotation_2))
  (Utilities|FlowControl|Sequence
    (:then_0
      (Components|Capsule|SetCapsuleSize (Variables|Default|GetFrostHitCapsule) (Variables|/Script/Engine.CapsuleComponent|GetCapsuleRadius _frosthitcapsule) (Variables|/Script/Engine.CapsuleComponent|GetCapsuleHalfHeight _frosthitcapsule) true)
      (Transformation|SetWorldLocation (Variables|Default|GetFrostHitCapsule) (/ (+ (Variables|Default|GetfireStartPoint) (Variables|Default|GetfireEndPoint)) 2) true false)
      (Transformation|SetWorldRotation (Variables|Default|GetFrostHitCapsule) (Math|Rotator|MakeRotator _roll (+ _pitch 105.0) _yaw) false false))
    (:then_1
      (Variables|Default|SetfireStartPoint (Transformation|GetSocketLocation _weaponmesh "Muzzle"))
      (Variables|Default|SetfireEndPoint (+ (* (Math|Vector|GetForwardVector (Variables|/Script/Engine.Actor|GetRootComponent (Game|GetPlayerCameraManager 0))) (Variables|Default|GetWeaponRange)) (Transformation|GetSocketLocation _weaponmesh "Muzzle"))))
    (:then_2
      (if (Variables|Default|GetDrawDebugCapsule)
        (Rendering|Debug|DrawDebugCapsule (Transformation|GetWorldLocation (Variables|Default|GetFrostHitCapsule)) (+ (Variables|/Script/Engine.CapsuleComponent|GetCapsuleHalfHeight _frosthitcapsule_2) 0.0) (+ (Variables|/Script/Engine.CapsuleComponent|GetCapsuleRadius _frosthitcapsule_2) 0.0) (Math|Rotator|MakeRotator _roll_2 (+ _pitch_2 105.0) _yaw_2) "(R=1.000000,G=1.000000,B=1.000000,A=1.000000)" 0.0 3.0)
        (bind _asbp_player_character (Utilities|Casting|CastToBP_PlayerCharacter (Game|GetPlayerCharacter 0)))
        (Variables|/Game/Blueprint/Character/BP_PlayerCharacter.BP_PlayerCharacter_C|SetIsFire _asbp_player_character true)
        (else
          (bind _asbp_player_character_2 (Utilities|Casting|CastToBP_PlayerCharacter (Game|GetPlayerCharacter 0)))
          (Variables|/Game/Blueprint/Character/BP_PlayerCharacter.BP_PlayerCharacter_C|SetIsFire _asbp_player_character_2 false))))))

(event EventOnFireStart
  (bind _frosthitcapsule (Variables|Default|GetFrostHitCapsule))
  (bind _astpscharacter_q (Utilities|Casting|CastToTPSCharacterQ (Game|Player|GetPlayerPawn 0)))
  ;[1 1 1] Frost Canon prototype
  (if (> (Variables|/Script/ProjectGoat.TPSCharacterQ|GetsnowCount _astpscharacter_q) 0.0)
    (Utilities|FlowControl|Sequence
      (:then_0
        (Collision|SetCollisionResponsetoChannel _frosthitcapsule "ECC_GameTraceChannel9" "ECR_Overlap")
        (Variables|Default|SetDrawDebugCapsule true))
      (:then_1
        (Rendering|SetVisibility _frosthitcapsule (Variables|Default|GetDrawDebugCapsule) false))
      (:then_2
        (bind _astpscharacter_q_2 (Utilities|Casting|CastToTPSCharacterQ (Game|Player|GetPlayerPawn 0)))
        (Variables|/Script/ProjectGoat.TPSCharacterQ|SetsnowCount _astpscharacter_q_2 (- (Variables|/Script/ProjectGoat.TPSCharacterQ|GetsnowCount _astpscharacter_q_2) 0.5))))))

(event EventOnFireEnd
  (bind _frosthitcapsule (Variables|Default|GetFrostHitCapsule))
  (Utilities|FlowControl|Sequence
    (:then_0
      (Collision|SetCollisionResponsetoChannel _frosthitcapsule "ECC_GameTraceChannel9" "ECR_Ignore")
      (Variables|Default|SetDrawDebugCapsule false))
    (:then_1
      (Rendering|SetVisibility _frosthitcapsule (Variables|Default|GetDrawDebugCapsule) false))))

(fn ConstructionScript)