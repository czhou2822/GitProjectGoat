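; Actor component that tracks the health of its owner and destroys that actor when health runs out.
; BeginPlay fills Health from DefaultHealth, and DealDamage passes negated damage to ChangeHealth.
; ChangeHealth updates Health and HealthPercentage with a floor at zero but no upper cap, fires OnHealthChange, and calls Dead at zero.
; The EventGraph also holds an unconnected copy of the ChangeHealth logic that never runs.
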(event EventBeginPlay
  (Variables|Default|SetHealth (Variables|Default|GetDefaultHealth))
  (Variables|Default|SetHealthPercentage 1.0))

(event EventTick
  (params (DeltaSeconds :type Float%20%28single-precision%29)))

(fn Dead
  (if (Variables|Default|GetIsDead)
    (Actor|DestroyActor (Components|GetOwner))))

(fn DealDamage
  (params (AttackIn :type Float%20%28single-precision%29))
  (CallFunction|ChangeHealth (* -1 AttackIn)))

(fn ChangeHealth
  (params (InHealth :type Float%20%28single-precision%29))
  (if (<= (+ InHealth (Variables|Default|GetHealth)) 0.0)
    (Variables|Default|SetHealth 0.0)
    (Variables|Default|SetHealthPercentage 0.0)
    (Default|CallOnHealthChange)
    (Variables|Default|SetIsDead true)
    (CallFunction|Dead)
    (else
      (bind _output_get (Variables|Default|SetHealth (+ InHealth (Variables|Default|GetHealth))))
      (Variables|Default|SetHealthPercentage (/ _output_get (Variables|Default|GetDefaultHealth)))
      (Default|CallOnHealthChange))))