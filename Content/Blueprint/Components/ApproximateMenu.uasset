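; ApproximateMenu is a component that acts as a menu, judging by its name, hidden at BeginPlay and toggled through Enable and Disable.
; Enable unhides it, shows the first player's mouse cursor and ignores look input, and Disable hides it and reverses both.
; Logic to rotate it toward the player character's mesh while visible is present but disconnected, as Tick is empty.
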(event EventBeginPlay
  (Development|SetHiddeninGame true false))

(event EventTick
  (params (DeltaSeconds :type Float%20%28single-precision%29)))

(fn Enable
  (bind _returnvalue (Game|GetPlayerController 0))
  (Development|SetHiddeninGame false false)
  (Variables|/Script/Engine.PlayerController|SetbShowMouseCursor _returnvalue true)
  (Input|SetIgnoreLookInput _returnvalue true))

(fn Disable
  (bind _returnvalue (Game|GetPlayerController 0))
  (Development|SetHiddeninGame true false)
  (Variables|/Script/Engine.PlayerController|SetbShowMouseCursor _returnvalue false)
  (Input|SetIgnoreLookInput _returnvalue false))