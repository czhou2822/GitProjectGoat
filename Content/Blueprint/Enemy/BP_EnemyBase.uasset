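; BP_EnemyBase is a base enemy that drops a coin and destroys itself when its health component reports death.
; Health changes update a widget health bar, which rotates every tick to face the player.
; Construction replaces each mesh material with a dynamic frozen-material instance.
; Slow start plays a frozen timeline meant to drive that material's ice amount, and slow end stops it and resets the amount.
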(event OnHealthChange(HealthComponent)
  (bind _asumg_enemy_health (Utilities|Casting|CastToUMG_EnemyHealth (UserInterface|GetUserWidgetObject (Variables|Default|GetWidget))))
  (Progress|SetPercent (Variables|/Game/Blueprint/Enemy/UMG_EnemyHealth.UMG_EnemyHealth_C|GetPG_HealthBar _asumg_enemy_health) (Variables|/Game/Blueprint/Components/HealthComponent.HealthComponent_C|GetHealthPercentage (Variables|Default|GetHealthComponent))))

(event Custom|HandleOnCharacterDead
  (Game|SpawnActorfromClass "/Game/Blueprint/Misc/BP_Coin.BP_Coin_C" (Transformation|GetActorTransform) "Undefined" 0 0)
  (Actor|DestroyActor))

(event EventBeginPlay
  (EventDispatchers|AssignOnCharacterDead (Variables|Default|GetHealthComponent) (delegate Custom|HandleOnCharacterDead)))

(event EventTick
  (params (DeltaSeconds :type Float%20%28single-precision%29))
  (bind _returnvalue (Game|GetPlayerCharacter 0))
  (bind _widget (Variables|Default|GetWidget))
  (Utilities|IsValid _returnvalue
    (:Is%20Valid
      (Transformation|SetWorldRotation _widget (Math|Rotator|FindLookatRotation (Transformation|GetWorldLocation _widget) (Transformation|GetActorLocation _returnvalue)) false false))))

(event EventOnSlowStart
  (Components|Timeline|PlayfromStart (Variables|Default|GetTimeline_Frozen)))

(event EventOnSlowEnd
  (Audio|Components|Audio|Stop (Variables|Default|GetTimeline_Frozen))
  (Rendering|Material|SetScalarParameterValueonMaterials (Variables|Character|GetMesh) "amount" 0.0))

(fn ConstructionScript
  (bind _mesh (Variables|Character|GetMesh))
  ;[1 1 1] TODO, for alpha
  (for (_ _array_index) (Rendering|Material|GetMaterials _mesh)
    (Rendering|Material|CreateDynamicMaterialInstance _mesh _array_index "/Game/Material/Snow/FrozenGrassCharacter_Inst.FrozenGrassCharacter_Inst" "None" :!class /Script/Engine.PrimitiveComponent)
    (Rendering|Material|SetScalarParameterValueonMaterials _mesh "amount" 0.0)))