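; Base enemy Blueprint with health, a billboard health bar and a frost slow effect.
; Health component events update the bar widget and, on death, spawn a coin and destroy the enemy; Tick turns the widget toward the player.
; Capsule overlaps with BP_FrostCannon start and end the slow, whose events play or stop a frozen timeline meant to drive the mesh's SnowAmount material parameter.
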(event OnComponentBeginOverlap(CapsuleComponent)
  (params (OverlappedComponent :type Primitive%20Component%20Object%20Reference) (OtherActor :type Actor%20Object%20Reference) (OtherComp :type Primitive%20Component%20Object%20Reference) (OtherBodyIndex :type Integer) (bFromSweep :type Boolean) (SweepResult :type Hit%20Result%20Structure%20%28by%20ref%29))
  (Utilities|Casting|CastToBP_FrostCannon OtherActor)
  (Class|EnemyBase|StartSlow))

(event OnHealthChange(HealthComponent)
  (bind _asumg_enemy_health (Utilities|Casting|CastToUMG_EnemyHealth (UserInterface|GetUserWidgetObject (Variables|Default|GetWidget))))
  (Progress|SetPercent (Variables|/Game/Blueprint/Enemy/UMG_EnemyHealth.UMG_EnemyHealth_C|GetPG_HealthBar _asumg_enemy_health) (Variables|/Game/Blueprint/Components/HealthComponent.HealthComponent_C|GetHealthPercentage (Variables|Default|GetHealthComponent))))

(event OnComponentEndOverlap(CapsuleComponent)
  (params (OverlappedComponent :type Primitive%20Component%20Object%20Reference) (OtherActor :type Actor%20Object%20Reference) (OtherComp :type Primitive%20Component%20Object%20Reference) (OtherBodyIndex :type Integer))
  (Utilities|Casting|CastToBP_FrostCannon OtherActor)
  (Class|EnemyBase|EndSlow))

(event Custom|HandleOnCharacterDead
  (Game|SpawnActorfromClass "/Game/Blueprint/Misc/BP_Coin.BP_Coin_C" (Transformation|GetActorTransform) "Undefined" 0 0)
  (Actor|DestroyActor))

(event EventBeginPlay
  (EventDispatchers|AssignOnCharacterDead (Variables|Default|GetHealthComponent) (delegate Custom|HandleOnCharacterDead)))

(event EventTick
  (params (DeltaSeconds :type Float%20%28single-precision%29))
  (bind _returnvalue (Game|GetPlayerCharacter 0))
  (bind _widget (Variables|Default|GetWidget))
  (Utilities|IsValid _returnvalue
    (:Is%20Valid
      (Transformation|SetWorldRotation _widget (Math|Rotator|FindLookatRotation (Transformation|GetWorldLocation _widget) (Transformation|GetActorLocation _returnvalue)) false false))))

(event EventOnSlowStart
  (Components|Timeline|PlayfromStart (Variables|Default|GetTimeline_Frozen)))

(event EventOnSlowEnd
  (Audio|Components|Audio|Stop (Variables|Default|GetTimeline_Frozen))
  (Rendering|Material|SetScalarParameterValueonMaterials (Variables|Character|GetMesh) "SnowAmount" 0.0))

(fn ConstructionScript
  (Rendering|Material|SetScalarParameterValueonMaterials (Variables|Character|GetMesh) "SnowAmount" 0.0))

(fn SetDefaultHealth
  (params (InDefaultHealth :type Float%20%28single-precision%29))
  (bind _healthcomponent (Variables|Default|GetHealthComponent))
  (bind _output_get (Variables|/Game/Blueprint/Components/HealthComponent.HealthComponent_C|SetDefaultHealth _healthcomponent InDefaultHealth))
  (Variables|/Game/Blueprint/Components/HealthComponent.HealthComponent_C|SetHealth _healthcomponent _output_get))