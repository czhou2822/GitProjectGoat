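; Enemy base actor Blueprint, named as a backup, with a world-space health bar widget above a health component.
; Each tick, the widget rotates to face player character 0 when that character is valid.
; When the health component reports a change, the event casts the widget to UMG_EnemyHealth and sets its progress bar to the current health percentage.
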(event OnHealthChange(HealthComponent)
  (bind _asumg_enemy_health (Utilities|Casting|CastToUMG_EnemyHealth (UserInterface|GetUserWidgetObject (Variables|Default|GetWidget))))
  (Progress|SetPercent (Variables|/Game/Blueprint/Enemy/UMG_EnemyHealth.UMG_EnemyHealth_C|GetPG_HealthBar _asumg_enemy_health) (Variables|/Game/Blueprint/Components/HealthComponent.HealthComponent_C|GetHealthPercentage (Variables|Default|GetHealthComponent))))

(event EventBeginPlay)

(event EventTick
  (params (DeltaSeconds :type Float%20%28single-precision%29))
  (bind _returnvalue (Game|GetPlayerCharacter 0))
  (bind _widget (Variables|Default|GetWidget))
  (Utilities|IsValid _returnvalue
    (:Is%20Valid
      (Transformation|SetWorldRotation _widget (Math|Rotator|FindLookatRotation (Transformation|GetWorldLocation _widget) (Transformation|GetActorLocation _returnvalue)) false false))))

(fn ConstructionScript)