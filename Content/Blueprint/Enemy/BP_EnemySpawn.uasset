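; Enemy spawner actor that repeatedly spawns BP_EnemyBase at the world transform of its Arrow component.
; Tick compares game time against NextSpawn, then schedules the following spawn SpawnInterval seconds later, with no limit on enemy count.
; BeginPlay sets the first NextSpawn to SpawnInterval as an absolute game time, so a spawner that begins play after that time spawns on its first Tick.
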(event EventBeginPlay
  (Variables|Default|SetNextSpawn (Variables|Default|GetSpawnInterval)))

(event EventTick
  (params (DeltaSeconds :type Float%20%28single-precision%29))
  (if (> (Utilities|Time|GetGameTimeinSeconds) (Variables|Default|GetNextSpawn))
    (Game|SpawnActorfromClass "/Game/Blueprint/Enemy/BP_EnemyBase.BP_EnemyBase_C" (Transformation|GetWorldTransform (Variables|Default|GetArrow)) "Undefined" 0 0)
    (Variables|Default|SetNextSpawn (+ (Utilities|Time|GetGameTimeinSeconds) (Variables|Default|GetSpawnInterval)))))

(fn ConstructionScript)