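; Enemy spawner Blueprint that spawns waves of BP_EnemyBase actors at its Arrow component's location and rotation.
; SpawnWave clears EnemyArray, stores the requested count and starts a looping timer that calls SpawnSingleEnemy by name.
; SpawnSingleEnemy spawns a slightly scaled-down enemy while the count is non-negative, but never decrements it or fills the array.
; WaitForWaveToCompleteTick is an empty stub, and nothing here stops the timer.
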(fn ConstructionScript)

(fn SpawnSingleEnemy
  (bind _arrow (Variables|Default|GetArrow))
  (bind _returnvalue (Transformation|GetWorldTransform _arrow))
  (bind (_location _rotation) (Math|Transform|BreakTransform _returnvalue))
  (if (>= (Variables|Default|GetEnemyToBeSpawn) 0)
    (bind _returnvalue_2 (Game|SpawnActorfromClass "/Game/Blueprint/Enemy/BP_EnemyBase.BP_EnemyBase_C" (Math|Transform|MakeTransform _location _rotation "0.900000,0.900000,0.900000") "Undefined" 0 0))
    (return _returnvalue_2)))

(fn SpawnWave
  (params (SpawnInterval :type Float%20%28single-precision%29) (SpawnEnemyCount :type Integer))
  (Utilities|Set|Clear (Variables|Default|GetEnemyArray))
  (Variables|Default|SetEnemyToBeSpawn SpawnEnemyCount)
  (bind _returnvalue (Utilities|Time|SetTimerbyFunctionName 0 "SpawnSingleEnemy" SpawnInterval true))
  (Variables|Default|SetSpawnWaveTimer _returnvalue))

(fn WaitforWavetoCompleteTick)