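; Player character Blueprint for tower building, which also creates the HUD, opens the pause menu and draws snow-collection hits into a render target.
; Holding Build pulls out the camera via timeline and spawns a laser tower, which a looping timer moves to a screen-center trace hit.
; Releasing Build ends placement and resets the camera.
; Frost cannon, tower cycling and other tower spawns remain as unconnected prototype logic.
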(event OnComponentBeginOverlap(FrostCannon)
  (params (OverlappedComponent :type Primitive%20Component%20Object%20Reference) (OtherActor :type Actor%20Object%20Reference) (OtherComp :type Primitive%20Component%20Object%20Reference) (OtherBodyIndex :type Integer) (bFromSweep :type Boolean) (SweepResult :type Hit%20Result%20Structure%20%28by%20ref%29))
  ;[1 1 1] Frost Canon prototype
)

(event Custom|WhichTower
  ;[1 1 1] Spawn Different Towers
  (switch Utilities|FlowControl|Switch|SwitchonTower_Type (Variables|Default|GetTower)
    (:NewEnumerator1
      (bind _hitpoint (CallFunction|GetScreentoWorldLocation))
      (bind _returnvalue (Game|SpawnActorfromClass "/Game/Blueprint/Tower/BP_LaserTower.BP_LaserTower_C" (Math|Conversions|ToTransform(Vector) (.Location (Collision|BreakHitResult _hitpoint))) "AlwaysSpawn" 0 0))
      (Variables|Default|SetSpawnedTower _returnvalue))))

(event EventOnCollectSnow
  (params (location :type Vector :default "0, 0, 0"))
  (bind _hitsonwmaterial (Variables|Default|GetHitSonwMaterial))
  ;[1 1 1] collecting snow RTT
  (Rendering|Material|SetVectorParameterValue _hitsonwmaterial "HitLocationW" (Math|Conversions|ToLinearColor(Vector) location) :!class /Script/Engine.MaterialInstanceDynamic)
  (Rendering|DrawMaterialtoRenderTarget "/Game/Material/Snow/SnowDeformation/Snow_Scene_Capture_RTT2.Snow_Scene_Capture_RTT2" _hitsonwmaterial))

(event EventTick
  (params (DeltaSeconds :type Float%20%28single-precision%29))
  (Utilities|FlowControl|Sequence))

(event EventBeginPlay
  (Utilities|FlowControl|Sequence
    (:then_0
      ;[1 1 1] set up hit snow material
      (bind _returnvalue (Rendering|Material|CreateDynamicMaterialInstance "/Game/Material/Snow/SnowDeformation/HitOnSnow.HitOnSnow" "None" :!class /Script/Engine.KismetMaterialLibrary))
      (Variables|Default|SetHitSonwMaterial _returnvalue))
    (:then_1
      ;[1 1 1] Setup Variables
      (CallFunction|SetupVariables))
    (:then_2
      ;[1 1 1] Main Interface
      (bind _returnvalue_2 (UserInterface|CreateWidget "/Game/CC/widget/widget/UMG_PlayerHUD.UMG_PlayerHUD_C"))
      (UserInterface|Viewport|AddtoViewport _returnvalue_2 0))))

(event Input|ActionEvents|InputActionDestroyTower
  (params (Key :type Key%20Structure :default "None"))
  ;[1 1 1] Press Button
  (:Pressed
    (if (Variables|Default|GetIsCharacterPlacingTower)
      (Variables|Default|SetDestroyTowerMode true)
      (switch Utilities|FlowControl|Switch|SwitchonTower_Type (Variables|Default|GetTower)
        (:NewEnumerator0
          (Actor|DestroyActor (Variables|Default|GetBlue%20Tower)))
        (:NewEnumerator1
          (Actor|DestroyActor (Variables|Default|GetRed%20Tower)))
        (:NewEnumerator2
          (Actor|DestroyActor (Variables|Default|GetGreen%20Tower))))
      (Variables|Default|SetIsCharacterPlacingTower false)))
  (:Released
    (Variables|Default|SetDestroyTowerMode false)))

(event Input|ActionEvents|InputActionBuild
  (params (Key :type Key%20Structure :default "None"))
  ;[1 1 1] Press Button
  (:Pressed
    (|PulloutBuildingCamera)
    (CallFunction|WhichTower)
    (Variables|Default|SetIsCharacterPlacingTower true)
    (Default|CallOnCharacterStartPlacing true)
    (bind _returnvalue (Utilities|Time|SetTimerbyFunctionName 0 "AdjustTowerLocation" 0.016667 true))
    (Variables|Default|SetTowerAdjustTimer _returnvalue))
  (:Released
    (Variables|Default|SetIsCharacterPlacingTower false)
    (Default|CallOnTowerPlaced)
    (Default|CallOnCharacterStartPlacing false)
    (Utilities|Time|ClearandInvalidateTimerbyHandle (Variables|Default|GetTowerAdjustTimer))
    (|ResetBuildingCamera)))

(event Input|ActionEvents|InputActionBuild
  (params (Key :type Key%20Structure :default "None"))
  ;[1 1 1] TowerSeedThrowing
)

(event Input|ActionEvents|InputActionOpenMenu
  (params (Key :type Key%20Structure :default "None"))
  (bind _returnvalue (Game|GetPlayerController 0))
  ;[1 1 1] Press Button
  (:Pressed
    (Game|SetGamePaused true)
    (bind _returnvalue_2 (UserInterface|CreateWidget "/Game/CC/widget/widget/UMG_Pause.UMG_Pause_C" _returnvalue))
    (UserInterface|Viewport|AddtoViewport _returnvalue_2 0)
    (Input|SetInputModeUIOnly _returnvalue 0 "DoNotLock")
    (Variables|/Script/Engine.PlayerController|SetbShowMouseCursor _returnvalue true)))

(event Input|ActionEvents|InputActionSelectTower
  (params (Key :type Key%20Structure :default "None"))
  ;[1 1 1] Press Button
  (:Pressed
    (Variables|Default|SetIsSelecting true))
  (:Released
    (Variables|Default|SetIsSelecting false)))

(event Input|MouseEvents|LeftMouseButton
  (params (Key :type Key%20Structure :default "None"))
  ;[1 1 1] Frost Canon prototype
)

(fn ConstructionScript)

(fn GetScreentoWorldLocation
  (bind _returnvalue (Game|GetPlayerController 0))
  (bind _returnvalue_2 (Viewport|GetViewportSize))
  (bind _returnvalue_3 (/ _returnvalue_2 2.0))
  (bind (_worldposition _worlddirection) (Class|GameplayStatics|DeprojectScreentoWorld _returnvalue _returnvalue_3))
  (bind _outhit (Collision|LineTraceForObjects _worldposition (+ _worldposition (* _worlddirection 5000)) (Variables|Default|GetTowerTraceObjectArray) false 0 "None" true "(R=1.000000,G=0.000000,B=0.000000,A=1.000000)" "(R=0.000000,G=1.000000,B=0.000000,A=1.000000)" 0.2))
  (return _outhit))

(fn SetupVariables
  (Variables|Default|SetTower "NewEnumerator1")
  (Variables|Default|SetDefaultFOV (Variables|/Script/Engine.CameraComponent|GetFieldOfView (Variables|Default|GettpsCamera)))
  (Variables|Default|SetDefaultCamaraTransform (Transformation|GetRelativeTransform (Variables|Default|GettpsCamera))))

(fn AdjustTowerLocation
  (bind _spawnedtower (Variables|Default|GetSpawnedTower))
  (Utilities|IsValid _spawnedtower
    (:Is%20Valid
      (bind _hitpoint (CallFunction|GetScreentoWorldLocation))
      (Transformation|SetActorTransform _spawnedtower (Math|Conversions|ToTransform(Vector) (.Location (Collision|BreakHitResult _hitpoint)))))))