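; Prototype player character for tower placement, with snow-hit painting and HUD, cursor and pause input.
; Holding Build spawns the selected tower and Tick moves it ahead of the character until release places it or DestroyTower removes it.
; Snow collection draws hit locations into a render target through a dynamic material.
; Tower cycling and Frost Cannon activation are unwired, leaving Laser (Red) selected and the enemy slow-down inactive.
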(event OnComponentBeginOverlap(FrostCannon)
  (params (OverlappedComponent :type Primitive%20Component%20Object%20Reference) (OtherActor :type Actor%20Object%20Reference) (OtherComp :type Primitive%20Component%20Object%20Reference) (OtherBodyIndex :type Integer) (bFromSweep :type Boolean) (SweepResult :type Hit%20Result%20Structure%20%28by%20ref%29))
  ;[1 1 1] Frost Canon prototype
)

(event Custom|WhichTower
  (bind _returnvalue (|CollapseGraph_0_2))
  ;[1 1 1] Spawn Different Towers
  (switch Utilities|FlowControl|Switch|SwitchonTower_Type (Variables|Default|GetTower)
    (:NewEnumerator0
      (bind _returnvalue_2 (Game|SpawnActorfromClass "/Game/Blueprint/Tower/BP_GrenadeTower.BP_GrenadeTower_C" _returnvalue "AdjustIfPossibleButDontSpawnIfColliding" 0 0))
      (Variables|Default|SetBlue%20Tower _returnvalue_2))
    (:NewEnumerator1
      (bind _returnvalue_3 (Game|SpawnActorfromClass "/Game/Blueprint/Tower/BP_LaserTower.BP_LaserTower_C" _returnvalue "AdjustIfPossibleButDontSpawnIfColliding" 0 0))
      (Variables|Default|SetRed%20Tower _returnvalue_3))
    (:NewEnumerator2
      (bind _returnvalue_4 (Game|SpawnActorfromClass "/Game/Blueprint/Tower/TowerBase/BP_TowerBase.BP_TowerBase_C" _returnvalue "AdjustIfPossibleButDontSpawnIfColliding" 0 0))
      (Variables|Default|SetBaseTower _returnvalue_4))))

(event EventTick
  (params (DeltaSeconds :type Float%20%28single-precision%29))
  (bind _newtransform (|Move_Tower_2))
  (bind _frostcannon (Variables|Default|GetFrostCannon))
  (bind _blue_tower (Variables|Default|GetBlue%20Tower))
  (bind _frostedenemies (Variables|Default|GetFrostedEnemies))
  (bind _red_tower (Variables|Default|GetRed%20Tower))
  (bind _basetower (Variables|Default|GetBaseTower))
  (Utilities|FlowControl|Sequence
    (:then_0
      ;[1 1 1] Tick
      (if (Variables|Default|GetIsCharacterPlacingTower)
        (switch Utilities|FlowControl|Switch|SwitchonTower_Type (Variables|Default|GetTower)
          (:NewEnumerator0
            (Utilities|IsValid _blue_tower
              (:Is%20Valid
                (Transformation|SetActorTransform _blue_tower _newtransform))))
          (:NewEnumerator1
            (Utilities|IsValid _red_tower
              (:Is%20Valid
                (Transformation|SetActorTransform _red_tower _newtransform))))
          (:NewEnumerator2
            (Utilities|IsValid _basetower
              (:Is%20Valid
                (Transformation|SetActorTransform _basetower _newtransform)))))))
    (:then_1
      ;[1 1 1] Draw Frost Cannon debug
      (if (Variables|Default|GetIsFrostCannonOn)
        (Rendering|Debug|DrawDebugBox :Center (Transformation|GetWorldLocation _frostcannon) :Extent (Variables|/Script/Engine.BoxComponent|GetBoxExtent _frostcannon))
        (for _array_element _frostedenemies
          (Utilities|IsValid _array_element
            (:Is%20Valid
              (Class|EnemyBase|SlowDown _array_element))))
        (Utilities|Array|Clear _frostedenemies)))))

(event EventBeginPlay
  (Utilities|FlowControl|Sequence
    (:then_0
      ;[1 1 1] set up hit snow material
      (bind _returnvalue (Rendering|Material|CreateDynamicMaterialInstance "/Game/Material/Snow/SnowDeformation/HitOnSnow.HitOnSnow" "None" :!class /Script/Engine.KismetMaterialLibrary))
      (Variables|Default|SetHitSonwMaterial _returnvalue))
    (:then_1
      ;[1 1 1] Start And Listen
      (Variables|Default|SetTower "NewEnumerator1"))
    (:then_2
      ;[1 1 1] Main Interface
      (bind _returnvalue_2 (UserInterface|CreateWidget "/Game/CC/widget/widget/UMG_MainInterface.UMG_MainInterface_C"))
      (UserInterface|Viewport|AddtoViewport _returnvalue_2 0))))

(event EventOnCollectSnow
  (params (location :type Vector :default "0, 0, 0"))
  (bind _hitsonwmaterial (Variables|Default|GetHitSonwMaterial))
  ;[1 1 1] collecting snow RTT
  (Rendering|Material|SetVectorParameterValue _hitsonwmaterial "HitLocationW" (Math|Conversions|ToLinearColor(Vector) location) :!class /Script/Engine.MaterialInstanceDynamic)
  (Rendering|DrawMaterialtoRenderTarget "/Game/Material/Snow/SnowDeformation/Snow_Scene_Capture_RTT2.Snow_Scene_Capture_RTT2" _hitsonwmaterial))

(event Input|ActionEvents|InputActionDestroyTower
  (params (Key :type Key%20Structure))
  ;[1 1 1] Press Button
  (:Pressed
    (if (Variables|Default|GetIsCharacterPlacingTower)
      (Variables|Default|SetDestroyTowerMode true)
      (switch Utilities|FlowControl|Switch|SwitchonTower_Type (Variables|Default|GetTower)
        (:NewEnumerator0
          (Actor|DestroyActor (Variables|Default|GetBlue%20Tower)))
        (:NewEnumerator1
          (Actor|DestroyActor (Variables|Default|GetRed%20Tower)))
        (:NewEnumerator2
          (Actor|DestroyActor (Variables|Default|GetBaseTower))))
      (Variables|Default|SetDestroyTowerMode false)
      (Variables|Default|SetIsCharacterPlacingTower false))))

(event Input|ActionEvents|InputActionBuild
  (params (Key :type Key%20Structure))
  (:Pressed
    ;[1 1 1] Press Button
    (CallFunction|WhichTower)
    (Variables|Default|SetIsCharacterPlacingTower true)
    (Default|CallOnCharacterStartPlacing true))
  (:Released
    (Variables|Default|SetIsCharacterPlacingTower false)
    (Default|CallOnTowerPlaced)
    (Default|CallOnCharacterStartPlacing false)))

(event Input|ActionEvents|InputActionBuild
  (params (Key :type Key%20Structure))
  ;[1 1 1] TowerSeedThrowing
)

(event Input|KeyboardEvents|E
  (params (Key :type Key%20Structure))
  (bind _returnvalue (Game|GetPlayerController 0))
  ;[1 1 1] Press Button
  (:Pressed
    (bind _returnvalue_2 (UserInterface|CreateWidget "/Game/CC/widget/widget/UMG_Pause.UMG_Pause_C" _returnvalue))
    (UserInterface|Viewport|AddtoViewport _returnvalue_2 0)
    (Input|SetInputModeUIOnly _returnvalue 0 "DoNotLock")
    (Variables|/Script/Engine.PlayerController|SetbShowMouseCursor _returnvalue true)))

(event Input|KeyboardEvents|LeftShift
  (params (Key :type Key%20Structure))
  ;[1 1 1] Press Button
)

(event Input|MouseEvents|LeftMouseButton
  (params (Key :type Key%20Structure))
  ;[1 1 1] Frost Canon prototype
  (:Released
    (Collision|SetCollisionResponsetoChannel (Variables|Default|GetFrostCannon) "ECC_Pawn" "ECR_Ignore")
    (Variables|Default|SetIsFrostCannonOn false)))

(event Input|KeyboardEvents|Tab
  (params (Key :type Key%20Structure))
  (bind _returnvalue (Game|GetPlayerController 0))
  ;[1 1 1] Press Button
  (:Pressed
    (Utilities|FlowControl|FlipFlop
      (:A
        (Variables|/Script/Engine.PlayerController|SetbShowMouseCursor _returnvalue true))
      (:B
        (Variables|/Script/Engine.PlayerController|SetbShowMouseCursor _returnvalue false)))))

(fn ConstructionScript)