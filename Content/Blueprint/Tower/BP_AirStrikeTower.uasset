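; Air strike tower that launches a homing missile at a given enemy, then recharges before the next strike.
; AirStrike spawns the missile pitched upward at the FirePoint socket, assigns its target and starts a looping countdown timer.
; At zero the timer is cleared and readiness is broadcast, as also happens when construction completes.
; Tick runs terrain snapping, and an unused grenade-spawn branch remains.
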(event EventBeginPlay
  (|CallParentFunction)
  (Variables|Default|SetCooldownTickDefault (Math|Float|Truncate (/ (Variables|Default|GetCooldownInSecond) (Variables|Default|GetCooldownTickInterval)))))

(event EventOnConstructionCompleteEvent
  (CallFunction|AirStrikeReadyFunction self))

(event EventTick
  (params (DeltaSeconds :type Float%20%28single-precision%29))
  (CallFunction|TerrianSnapping))

(fn ConstructionScript
  (|CallParentFunction))

(fn AirStrikeReadyFunction
  (params (NewParam :type BP%20Air%20Strike%20Tower%20Object%20Reference))
  (Default|CallOnAirStrikeReady NewParam)
  (Utilities|Time|ClearandInvalidateTimerbyHandle (Variables|Default|GetAirStrikeTimer))
  (Development|PrintString "AirStrikeReady" false false))

(fn AirStrikeCooldownTick
  (if (== (Variables|Default|GetCooldownTick) 0)
    (CallFunction|AirStrikeReadyFunction self)
    (else
      (Math|Integer|DecrementInt (Variables|Default|GetCooldownTick)
        (:%20%20
          (return))))))

(fn AirStrike
  (params (Target :type BP%20Enemy%20Base%20Object%20Reference))
  (bind _skeletonmesh (Variables|Default|GetSkeletonMesh))
  (bind _returnvalue (Transformation|GetSocketTransform _skeletonmesh "FirePoint" "RTS_World"))
  (bind (_location _rotation _scale) (Math|Transform|BreakTransform _returnvalue))
  (bind (_roll _pitch _yaw) (Math|Rotator|BreakRotator _rotation))
  (Development|PrintString (Utilities|String|Append (Utilities|GetDisplayName self) " air strikes"))
  (LocalVariables|SetSingleEnemy Target)
  (bind _returnvalue_2 (Game|SpawnActorfromClass "/Game/John/Blueprints/BP_HomingMissile.BP_HomingMissile_C" (Math|Transform|MakeTransform _location (Math|Rotator|MakeRotator _roll 9e+01 _yaw) _scale) "Undefined" 0 0))
  (AddComponent|AddSceneComponent (LocalVariables|GetSingleEnemy) false)
  (Variables|/Game/John/Blueprints/BP_HomingMissile.BP_HomingMissile_C|SetTargetEnemy _returnvalue_2 (LocalVariables|GetSingleEnemy))
  (Variables|Default|SetCooldownTick (Variables|Default|GetCooldownTickDefault))
  ;[1 1 1] Reset Cooldown Timer
  (bind _returnvalue_3 (Utilities|Time|SetTimerbyFunctionName 0 "AirStrikeCooldownTick" (Variables|Default|GetCooldownTickInterval) true))
  (Variables|Default|SetAirStrikeTimer _returnvalue_3))