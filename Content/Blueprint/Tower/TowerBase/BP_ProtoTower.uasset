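; Prototype tower pawn for a tower-defense mechanic, covering placement, construction, targeting and firing, with debug drawing.
; While unplaced, a padding box tracks overlapping towers and toggles a material outline; the player's placed event destroys it on overlap or awaits AnimBP construction completion.
; Completion caches the AI controller, whose target Tick uses to lerp AnimBP yaw and call the fire dispatcher at intervals; its handler is empty.
; Tick also ground-snaps the base outside placement mode.
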(event OnComponentBeginOverlap(TowerPadding)
  (params (OverlappedComponent :type Primitive%20Component%20Object%20Reference) (OtherActor :type Actor%20Object%20Reference) (OtherComp :type Primitive%20Component%20Object%20Reference) (OtherBodyIndex :type Integer) (bFromSweep :type Boolean) (SweepResult :type Hit%20Result%20Structure%20%28by%20ref%29))
  ;[1 1 1] CheckNearDistance
  (if (not (Variables|Default|GetIsPlaced))
    (bind _asbp_tower_base (Utilities|Casting|CastToBP_TowerBase OtherActor))
    (CallFunction|SetRedOutLine true)
    (Development|PrintString (Utilities|String|Append (Utilities|GetDisplayName _asbp_tower_base) " overlapped！"))
    (Utilities|Set|Add (Variables|Default|GetOverlappedTower) _asbp_tower_base)))

(event OnComponentEndOverlap(TowerPadding)
  (params (OverlappedComponent :type Primitive%20Component%20Object%20Reference) (OtherActor :type Actor%20Object%20Reference) (OtherComp :type Primitive%20Component%20Object%20Reference) (OtherBodyIndex :type Integer))
  ;[1 1 1] CheckNearDistance
  (bind _asbp_tower_base (Utilities|Casting|CastToBP_TowerBase OtherActor))
  (CallFunction|SetRedOutLine false)
  (Utilities|Set|Remove (Variables|Default|GetOverlappedTower) _asbp_tower_base)
  (Development|PrintString (Utilities|String|Append (Utilities|GetDisplayName _asbp_tower_base) " removed！")))

(event Custom|FireEvent
  ;[1 1 1] HookupAI and initialize
  ;;[1 1 1] If not collide, initilize
)

(event Custom|HandleOnConstructionComplete
  ;[1 1 1] HookupAI and initialize
  ;;[1 1 1] If not collide, initilize
  (CallFunction|TowerInit)
  (EventDispatchers|BindEventtoTowerFire (delegate Custom|FireEvent))
  (bind _asbp_player_character (Utilities|Casting|CastToBP_PlayerCharacter (Game|GetPlayerCharacter 0)))
  (EventDispatchers|BindEventtoOnCharacterStartPlacing _asbp_player_character (delegate Custom|HandleOnCharacterStartPlacing)))

(event Custom|HandleTowerPlacedEvent
  ;[1 1 1] Begin Play
  (EventDispatchers|UnbindEventfromOnTowerPlaced (stale EventBeginPlay _asbp_char_proto) (delegate Custom|HandleTowerPlacedEvent))
  ;[1 1 1] HookupAI and initialize
  (if (== (Utilities|Set|Length (Variables|Default|GetOverlappedTower)) 0)
    ;;[1 1 1] If not collide, initilize
    (EventDispatchers|BindEventtoOnConstructionComplete (Variables|Default|GetAnimInstance) (delegate Custom|HandleOnConstructionComplete))
    (Development|PrintString "Tower Placed， constructing starting")
    (Variables|Default|SetIsPlaced true)
    (else
      ;;[1 1 1] else, destroy
      (Actor|DestroyActor)
      (bind _result (Utilities|Set|ToArray (Variables|Default|GetOverlappedTower)))
      (for _array_element _result
        (Development|PrintString (Utilities|String|Append "overlap with " (Utilities|GetDisplayName _array_element)))))))

(event Custom|HandleOnCharacterStartPlacing
  (params (EnterPlacingMode :type Boolean))
  ;[1 1 1] HookupAI and initialize
  (Variables|Default|SetShowRange EnterPlacingMode))

(event EventBeginPlay
  (CallFunction|SetRedOutLine false)
  ;[1 1 1] Begin Play
  (bind _asbp_char_proto (Utilities|Casting|CastToBP_CharProto (Game|GetPlayerCharacter 0)))
  (EventDispatchers|BindEventtoOnTowerPlaced _asbp_char_proto (delegate Custom|HandleTowerPlacedEvent))
  (bind _asabp_tower_base (Utilities|Casting|CastToABP_TowerBase (Components|SkeletalMesh|GetAnimInstance (Variables|Default|GetSkeletalMesh))))
  (Variables|Default|SetAnimInstance _asabp_tower_base))

(event EventTick
  (params (DeltaSeconds :type Float%20%28single-precision%29))
  (bind _returnvalue (Utilities|Time|GetGameTimeinSeconds))
  (bind _base (Variables|Default|GetBase))
  (bind _range (Variables|Default|GetRange))
  (bind _towerpadding (Variables|Default|GetTowerPadding))
  (bind _base_2 (Variables|Default|GetBase))
  (bind _returnvalue_2 (Transformation|GetWorldLocation _base_2))
  (bind _returnvalue_3 (Transformation|GetWorldLocation _base))
  (Utilities|FlowControl|Sequence
    (:then_0
      ;[1 1 1] Tick
      (CallFunction|SetTargetActor))
    (:then_1
      (if (> _returnvalue (Variables|Default|GetNextFire))
        (Utilities|IsValid (Variables|Default|GetTargetActor)
          (:Is%20Valid
            (Default|CallTowerFire)
            (Variables|Default|SetNextFire (+ (Variables|Default|GetFireInterval) _returnvalue))))))
    (:then_2
      (if (not (Variables|Default|GetIsPlaced))
        (Rendering|Debug|DrawDebugBox :Center (Transformation|GetWorldLocation _towerpadding) :Extent (Variables|/Script/Engine.BoxComponent|GetBoxExtent _towerpadding) :Thickness 2.0)))
    (:then_3
      (if (Variables|Default|GetShowRange)
        (Rendering|Debug|DrawDebugSphere (Transformation|GetWorldLocation _range) (Variables|/Script/Engine.SphereComponent|GetSphereRadius _range) 12 "(R=1.000000,G=1.000000,B=1.000000,A=1.000000)" 0.0)))
    (:then_4
      (bind _asbp_player_character (Utilities|Casting|CastToBP_PlayerCharacter (Game|GetPlayerCharacter 0)))
      (if (not (Variables|/Game/Blueprint/Character/BP_PlayerCharacter.BP_PlayerCharacter_C|GetIsCharacterPlacingTower _asbp_player_character))
        (bind _outhit (Collision|LineTraceByChannel _returnvalue_2 (+ _returnvalue_2 (* (Math|Vector|GetUpVector _base_2) -500)) "TraceTypeQuery1" false 0 "Persistent"))
        (Transformation|SetWorldLocation _base (Math|Vector|MakeVector (.x _returnvalue_3) (.y _returnvalue_3) (+ (.z (.Location (Collision|BreakHitResult _outhit))) 25.0)) false false)))
    (:then_5
      (CallFunction|Turnto DeltaSeconds)
      (Development|PrintString (Utilities|String|ToString(Rotator) (Transformation|GetSocketRotation (Variables|Default|GetSkeletalMesh) "FireSocket")) true true "(R=0.000000,G=0.660000,B=1.000000,A=1.000000)" 0.0))))

(fn ConstructionScript)

(fn SetTargetActor
  (bind _towerai (Variables|Default|GetTowerAI))
  (Utilities|IsValid _towerai
    (:Is%20Valid
      (Utilities|IsValid (Variables|/Game/Blueprint/Tower/TowerBase/AI_TowerBase.AI_TowerBase_C|GetTargetActor _towerai)
        (:Is%20Valid
          (bind _output_get (Variables|Default|SetTargetActor (Variables|/Game/Blueprint/Tower/TowerBase/AI_TowerBase.AI_TowerBase_C|GetTargetActor _towerai)))
          (Variables|Default|SetTargetLocation (Transformation|GetActorLocation _output_get)))))))

(fn Turnto
  (params (DeltaTime :type Float%20%28single-precision%29))
  (Utilities|IsValid (Variables|Default|GetTargetActor)
    (:Is%20Valid
      (Variables|/Game/Blueprint/Tower/TowerBase/ABP_TowerBase.ABP_TowerBase_C|SetDoomRotation (Variables|Default|GetAnimInstance) (Math|Rotator|Lerp(Rotator) (Variables|/Game/Blueprint/Tower/TowerBase/ABP_TowerBase.ABP_TowerBase_C|GetDoomRotation (Variables|Default|GetAnimInstance)) (Math|Rotator|MakeRotator 0.0 0.0 (.Yaw (Math|Rotator|BreakRotator (Math|Rotator|FindLookatRotation (Transformation|GetSocketLocation (Variables|Default|GetSkeletalMesh) "FireSocket") (Variables|Default|GetTargetLocation))))) (Variables|Default|GetTurnSpeed)))
      (Rendering|Debug|DrawDebugLine :LineStart (Transformation|GetSocketLocation (Variables|Default|GetSkeletalMesh) "FireSocket") :LineEnd (Variables|Default|GetTargetLocation)))
    (:Is%20Not%20Valid
      (Development|PrintString "no actor in range" true true "(R=0.000000,G=0.660000,B=1.000000,A=1.000000)" 0.0)
      (return))))

(fn SetRedOutLine
  (params (isOutline :type Boolean))
  (bind _returnvalue (Math|Conversions|ToFloat(Boolean) isOutline))
  (Rendering|Material|SetScalarParameterValueonMaterials (Variables|Default|GetRotatory) "isOutLine" _returnvalue)
  (Rendering|Material|SetScalarParameterValueonMaterials (Variables|Default|GetCone) "isOutLine" _returnvalue)
  (Rendering|Material|SetScalarParameterValueonMaterials (Variables|Default|GetBase) "isOutLine" _returnvalue))

(fn TowerInit
  (bind _asai_tower_base (Utilities|Casting|CastToAI_TowerBase (Pawn|GetController)))
  (Variables|Default|SetTowerAI _asai_tower_base))