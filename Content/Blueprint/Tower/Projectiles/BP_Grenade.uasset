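; BP_Grenade is a tower projectile that explodes when an enemy enters its TriggerRadius or three seconds after spawning.
; Its ExplosiveRange sphere adds overlapping BP_EnemyBase actors to Targets, which are never removed.
; Explode damages each valid target through its HealthComponent.
; Particle, sound and DestroyActor run inside that loop, repeating per target and never running without a valid one.
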(event OnComponentBeginOverlap(ExplosiveRange)
  (params (OverlappedComponent :type Primitive%20Component%20Object%20Reference) (OtherActor :type Actor%20Object%20Reference) (OtherComp :type Primitive%20Component%20Object%20Reference) (OtherBodyIndex :type Integer) (bFromSweep :type Boolean) (SweepResult :type Hit%20Result%20Structure%20%28by%20ref%29))
  (bind _asbp_enemy_base (Utilities|Casting|CastToBP_EnemyBase OtherActor))
  (Utilities|Array|Add (Variables|Default|GetTargets) _asbp_enemy_base))

(event OnComponentBeginOverlap(TriggerRadius)
  (params (OverlappedComponent :type Primitive%20Component%20Object%20Reference) (OtherActor :type Actor%20Object%20Reference) (OtherComp :type Primitive%20Component%20Object%20Reference) (OtherBodyIndex :type Integer) (bFromSweep :type Boolean) (SweepResult :type Hit%20Result%20Structure%20%28by%20ref%29))
  (Utilities|Casting|CastToBP_EnemyBase OtherActor)
  (CallFunction|Explode))

(event EventBeginPlay
  (|CallParentFunction)
  (Utilities|FlowControl|Delay 3.0)
  (CallFunction|Explode))

(event Collision|EventActorBeginOverlap
  (params (OtherActor :type Actor%20Object%20Reference))
  (|CallParentFunction OtherActor) ; This node is disabled and will not be called.\nDrag off pins to build functionality.
)

(event EventTick
  (params (DeltaSeconds :type Float%20%28single-precision%29))
  (|CallParentFunction DeltaSeconds))

(fn ConstructionScript
  (|CallParentFunction))

(fn Explode
  (bind _returnvalue (Transformation|GetActorLocation))
  (bind _targets (Variables|Default|GetTargets))
  (if (not (== (Utilities|Array|Length _targets) 0))
    (for _array_element _targets
      (Utilities|IsValid _array_element
        (:Is%20Valid
          (Default|DealDamage (Variables|/Game/Blueprint/Enemy/EnemyBase/BP_EnemyBase.BP_EnemyBase_C|GetHealthComponent _array_element) (Variables|Default|GetProjectileDamage))
          (Effects|SpawnEmitteratLocation (Variables|Default|GetParticle) _returnvalue)
          (Audio|PlaySoundatLocation (Variables|Default|GetExplosionSound) _returnvalue "0, 0, 0" 1.0 1.0 0.0 0 0 0)
          (Actor|DestroyActor))))))