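; Grenade-launching tower Blueprint that turns toward its target and fires BP_Grenade projectiles.
; Each tick it calls TurnTo while TargetActor is valid.
; Its fire event spawns a grenade at FirePoint, rotated toward TargetLocation, then passes TowerDamage to it as projectile damage.
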(event Custom|FireEvent_1
  (bind _firepoint (Variables|Default|GetFirePoint))
  (bind _returnvalue (Transformation|GetWorldLocation _firepoint))
  (bind _returnvalue_2 (Game|SpawnActorfromClass "/Game/Blueprint/Tower/Projectiles/BP_Grenade.BP_Grenade_C" (Math|Transform|MakeTransform _returnvalue (Math|Rotator|FindLookatRotation _returnvalue (Variables|Default|GetTargetLocation))) "Undefined" 0 0))
  (Variables|/Game/Blueprint/Tower/Projectiles/BP_ProjectileBase.BP_ProjectileBase_C|SetProjectileDamage _returnvalue_2 (Variables|Default|GetTowerDamage)))

(event EventBeginPlay
  (|CallParentFunction) ; This node is disabled and will not be called.\nDrag off pins to build functionality.
)

(event Collision|EventActorBeginOverlap
  (params (OtherActor :type Actor%20Object%20Reference))
  (|CallParentFunction OtherActor) ; This node is disabled and will not be called.\nDrag off pins to build functionality.
)

(event EventTick
  (params (DeltaSeconds :type Float%20%28single-precision%29))
  (|CallParentFunction DeltaSeconds)
  (Utilities|IsValid (Variables|Default|GetTargetActor)
    (:Is%20Valid
      (CallFunction|Turnto DeltaSeconds))))

(fn ConstructionScript
  (|CallParentFunction))