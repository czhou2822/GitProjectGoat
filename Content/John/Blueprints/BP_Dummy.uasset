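; BP_Dummy is a dummy actor that shuttles back and forth along world Y and stores its Target as HomingTarget.
; BeginPlay caches the start location and derives the end point from MoveOffset.
; Tick checks game time against TurnInterval and uses a FlipFlop to alternately play and reverse a timeline.
; The timeline lerps the root's world location between both points, without sweep.
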(event EventBeginPlay
  (bind _output_get (Variables|Default|SetStartingLocation (Transformation|GetActorLocation)))
  (Variables|Default|SetEndLocation (Math|Vector|MakeVector (.x _output_get) (+ (.y _output_get) (Variables|Default|GetMoveOffset)) (.z _output_get)))
  (Variables|Default|SetHomingTarget (Variables|Default|GetTarget)))

(event Collision|EventActorBeginOverlap
  (params (OtherActor :type Actor%20Object%20Reference)))

(event EventTick
  (params (DeltaSeconds :type Float%20%28single-precision%29))
  (bind _returnvalue (Utilities|Time|GetGameTimeinSeconds))
  (if (>= _returnvalue (Variables|Default|GetNextTurnTime))
    (Variables|Default|SetNextTurnTime (+ _returnvalue (Variables|Default|GetTurnInterval)))
    (Utilities|FlowControl|FlipFlop
      (:A
        (bind _newtrack_2 (Timeline|Timeline_0 PlayFromStart)
          (:Update
            (Transformation|SetWorldLocation (Variables|Default|GetDefaultSceneRoot) (Math|Vector|Lerp(Vector) (Variables|Default|GetStartingLocation) (Variables|Default|GetEndLocation) _newtrack_2) false false))))
      (:B
        (Timeline|Timeline_0 ReverseFromEnd)))))

(fn ConstructionScript)