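; BP_HomingMissile is a projectile that seeks a target actor and deals area damage to enemies.
; Tick watches the Cube's physics velocity and, as upward speed nears zero at the apex, enables strong ProjectileMovement homing and turns the Cube toward TargetActor.
; ExplosionRadius overlaps maintain the list of enemies in range.
; Touching an enemy or a lifetime timeout triggers Explode, which damages their HealthComponents, draws a debug sphere and destroys the missile.
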(event OnComponentBeginOverlap(TriggerSphere)
  (params (OverlappedComponent :type Primitive%20Component%20Object%20Reference) (OtherActor :type Actor%20Object%20Reference) (OtherComp :type Primitive%20Component%20Object%20Reference) (OtherBodyIndex :type Integer) (bFromSweep :type Boolean) (SweepResult :type Hit%20Result%20Structure%20%28by%20ref%29))
  (Utilities|Casting|CastToBP_EnemyBase OtherActor)
  (CallFunction|Explode))

(event OnComponentBeginOverlap(ExplosionRadius)
  (params (OverlappedComponent :type Primitive%20Component%20Object%20Reference) (OtherActor :type Actor%20Object%20Reference) (OtherComp :type Primitive%20Component%20Object%20Reference) (OtherBodyIndex :type Integer) (bFromSweep :type Boolean) (SweepResult :type Hit%20Result%20Structure%20%28by%20ref%29))
  (bind _asbp_enemy_base (Utilities|Casting|CastToBP_EnemyBase OtherActor))
  (Utilities|Set|Add (Variables|Default|GetOverlappedArray) _asbp_enemy_base))

(event OnComponentEndOverlap(ExplosionRadius)
  (params (OverlappedComponent :type Primitive%20Component%20Object%20Reference) (OtherActor :type Actor%20Object%20Reference) (OtherComp :type Primitive%20Component%20Object%20Reference) (OtherBodyIndex :type Integer))
  (bind _asbp_enemy_base (Utilities|Casting|CastToBP_EnemyBase OtherActor))
  (Utilities|Set|Remove (Variables|Default|GetOverlappedArray) _asbp_enemy_base))

(event EventBeginPlay
  (Utilities|FlowControl|Delay 5.0)
  (CallFunction|Explode))

(event EventTick
  (params (DeltaSeconds :type Float%20%28single-precision%29))
  (bind _projectilemovement (Variables|Default|GetProjectileMovement))
  (if (not (Variables|/Script/Engine.ProjectileMovementComponent|GetbIsHomingProjectile (Variables|Default|GetProjectileMovement)))
    (bind _returnvalue (Physics|GetPhysicsLinearVelocity (Variables|Default|GetCube) "None"))
    (if (and (<= (.z _returnvalue) 2e+01) (> (.z _returnvalue) 0.0))
      (Development|PrintString (Utilities|String|ToString(Float) (.z _returnvalue)))
      (Variables|/Script/Engine.ProjectileMovementComponent|SetHomingTargetComponent _projectilemovement (Actor|GetComponentbyClass (Variables|Default|GetTargetActor) "/Script/Engine.SceneComponent"))
      (Variables|/Script/Engine.ProjectileMovementComponent|SetbIsHomingProjectile _projectilemovement true)
      (Variables|/Script/Engine.ProjectileMovementComponent|SetHomingAccelerationMagnitude _projectilemovement 4e+04)
      (Transformation|SetWorldRotation (Variables|Default|GetCube) (Math|Rotator|FindLookatRotation (Transformation|GetWorldLocation (Variables|Default|GetCube)) (Transformation|GetWorldLocation (Variables|/Script/Engine.Actor|GetRootComponent (Variables|Default|GetTargetActor)))) false false))))

(fn ConstructionScript)

(fn Explode
  (bind _explosionradius (Variables|Default|GetExplosionRadius))
  (Rendering|Debug|DrawDebugSphere (Transformation|GetWorldLocation _explosionradius) (Variables|/Script/Engine.SphereComponent|GetSphereRadius _explosionradius) 12 "(R=1.000000,G=1.000000,B=1.000000,A=1.000000)" 3.0 3.0)
  (bind _result (Utilities|Set|ToArray (Variables|Default|GetOverlappedArray)))
  (for _array_element _result
    (Utilities|IsValid _array_element
      (:Is%20Valid
        (Default|DealDamage (Actor|GetComponentbyClass _array_element "/Game/Blueprint/Components/HealthComponent.HealthComponent_C") (Variables|Default|GetDamage)))))
  (Actor|DestroyActor))