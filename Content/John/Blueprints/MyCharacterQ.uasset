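; Player character Blueprint that lets the player pick and place one of three tower types in the level.
; Left Shift cycles the Tower selection through Blue, Red and Green, and F spawns the matching grenade, laser or turret tower into a per-color array.
; A collapsed graph computes the spawn point ahead of the player's capsule.
; F also sets hold and release flags that nothing here reads.
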(event Custom|WhichTower
  (bind _returnvalue (|CollapseGraph_0))
  (switch Utilities|FlowControl|Switch|SwitchonTower_Type (Variables|Default|GetTower)
    (:NewEnumerator0
      (bind _returnvalue_2 (Game|SpawnActorfromClass "/Game/Blueprint/Tower/BP_GrenadeTower.BP_GrenadeTower_C" _returnvalue "AdjustIfPossibleButDontSpawnIfColliding" 0 0))
      (Utilities|Array|Add (Variables|Default|GetBlue_Towerarray) _returnvalue_2)
      (Development|PrintString "blue"))
    (:NewEnumerator1
      (bind _returnvalue_3 (Game|SpawnActorfromClass "/Game/Blueprint/Tower/BP_LaserTower.BP_LaserTower_C" _returnvalue "AdjustIfPossibleButDontSpawnIfColliding" 0 0))
      (Utilities|Array|Add (Variables|Default|GetRed_TowerArray) _returnvalue_3)
      (Development|PrintString "red"))
    (:NewEnumerator2
      (bind _returnvalue_4 (Game|SpawnActorfromClass "/Game/Blueprint/Tower/BP_Turret.BP_Turret_C" _returnvalue "AdjustIfPossibleButDontSpawnIfColliding" 0 0))
      (Utilities|Array|Add (Variables|Default|GetGreen_Tower%20Array) _returnvalue_4)
      (Development|PrintString "Green"))))

(event EventBeginPlay
  (Variables|Default|SetTower "NewEnumerator0"))

(event Collision|EventActorBeginOverlap
  (params (OtherActor :type Actor%20Object%20Reference)))

(event Input|KeyboardEvents|LeftShift
  (params (Key :type Key%20Structure :default "None"))
  (:Pressed
    (switch Utilities|FlowControl|Switch|SwitchonTower_Type (Variables|Default|GetTower)
      (:NewEnumerator0
        (Variables|Default|SetTower "NewEnumerator1"))
      (:NewEnumerator1
        (Variables|Default|SetTower "NewEnumerator2"))
      (:NewEnumerator2
        (Variables|Default|SetTower "NewEnumerator0")))))

(event Input|KeyboardEvents|F
  (params (Key :type Key%20Structure :default "None"))
  (:Pressed
    (CallFunction|WhichTower)
    (Variables|Default|Setis%20hold true))
  (:Released
    (Variables|Default|SetNewVar_0 true)))

(fn ConstructionScript)